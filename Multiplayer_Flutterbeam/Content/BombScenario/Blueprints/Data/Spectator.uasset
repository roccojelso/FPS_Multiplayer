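; Spectator pawn for the bomb scenario that points its player's camera at a random living teammate.
; Shortly after BeginPlay and on each left click, a server update rebuilds both living-team lists from the game mode's players, using their BS_ControllerComponent state.
; It then blends the view to a random character on its own team, requesting another update when the picked entry is invalid or has no character.
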(event `self.ReceiveBeginPlay`
  (`KismetSystemLibrary.Delay` 0.5)
  (`self.SV_UpdatePlayer`))

(event `Key|LeftMouseButton`
  (params (Key :type "Key Structure"))
  (:`Pressed`
    (`self.SV_UpdatePlayer`)))

(event `SV_UpdatePlayer`
  (if (not (`self.Updating`))
    (`self.UpdateLivingPlayer`)))

(event `SpectateTeamate`
  (switch `/Game/BombScenario/Blueprints/Data/E_Team` (`self.Team`)
    (:`NewEnumerator0`
      (`self.GetTeamA`))
    (:`NewEnumerator1`
      (`self.GetTeamB`))))

(fn `GetTeamA`
  (bind _livingteama (`self.LivingTeamA`))
  (bind _outitem (`KismetArrayLibrary.Array_Random` _livingteama))
  (if (`KismetArrayLibrary.Array_IsValidIndex` _livingteama)
    (`/Engine/EditorBlueprintResources/StandardMacros.IsValid` _outitem
      (:`Is Valid`
        (bind _ascharacter (cast `Character` (`Controller.K2_GetPawn` _outitem))
          (:`then`
            (bind _asplayer_controller (cast `PlayerController` (`self.GetController`)))
            (`PlayerController.SetViewTargetWithBlend` _asplayer_controller _ascharacter 0.0 "VTBlend_Linear" 0.0 false))
          (:`CastFailed`
            (`self.SV_UpdatePlayer` :!label _label))))
      (:`Is Not Valid`
        (goto _label)))))

(fn `GetTeamB`
  (bind _livingteamb (`self.LivingTeamB`))
  (bind _outitem (`KismetArrayLibrary.Array_Random` _livingteamb))
  (if (`KismetArrayLibrary.Array_IsValidIndex` _livingteamb)
    (`/Engine/EditorBlueprintResources/StandardMacros.IsValid` _outitem
      (:`Is Valid`
        (bind _ascharacter (cast `Character` (`Controller.K2_GetPawn` _outitem))
          (:`then`
            (bind _asplayer_controller (cast `PlayerController` (`self.GetController`)))
            (`PlayerController.SetViewTargetWithBlend` _asplayer_controller _ascharacter 0.0 "VTBlend_Linear" 0.0 false))
          (:`CastFailed`
            (`self.SV_UpdatePlayer` :!label _label))))
      (:`Is Not Valid`
        (goto _label)))))

(fn `UpdateLivingPlayer`
  (set `self.Updating` true)
  (`KismetArrayLibrary.Array_Clear` (`self.LivingTeamA`))
  (`KismetArrayLibrary.Array_Clear` (`self.LivingTeamB`))
  (bind _asbp_bomb_scenario_gm (cast `/Game/BombScenario/Blueprints/Game/BP_BombScenario_GM` (`GameplayStatics.GetGameMode`)))
  (for _array_element (`/Game/BombScenario/Blueprints/Game/BP_BombScenario_GM.AllPlayers` _asbp_bomb_scenario_gm)
    (bind _returnvalue (`self.GetComponentByClass` _array_element "/Game/BombScenario/Blueprints/Data/BS_ControllerComponent.BS_ControllerComponent_C"))
    (`/Engine/EditorBlueprintResources/StandardMacros.IsValid` _returnvalue
      (:`Is Valid`
        (if (`/Game/BombScenario/Blueprints/Data/BS_ControllerComponent.IsPlaying` _returnvalue)
          (switch `/Game/BombScenario/Blueprints/Data/E_Team` (`/Game/BombScenario/Blueprints/Data/BS_ControllerComponent.Team` _returnvalue)
            (:`NewEnumerator0`
              (`KismetArrayLibrary.Array_AddUnique` (`self.LivingTeamA`) _array_element))
            (:`NewEnumerator1`
              (`KismetArrayLibrary.Array_AddUnique` (`self.LivingTeamB`) _array_element)))))))
  (`self.SpectateTeamate`)
  (set `self.Updating` false))

(fn `UserConstructionScript`)