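; Game State for the Bomb Scenario mode that runs the round cycle, team scores, half-time side swap and match win check.
; Settings load from DT_GameStateSettings; timers drive the pre-round countdown and round clock, with timeout awarding Team B.
; Each round start clears characters and interactables, respawns items and players, then enables movement.
; Planting the bomb stops the round clock, while spawning and end screens go through the Game Mode.
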(event `StartRoundTimer`
  ;[0.1176 0.1176 0.1176] Round Timer
  (bind _returnvalue (`KismetSystemLibrary.K2_SetTimerDelegate` (delegate `TimeOut`) (`self.RoundTime`)))
  (set `self.TH_RoundTimeLeft` _returnvalue)
  (`KismetSystemLibrary.K2_SetTimerDelegate` (delegate `UpdateRoundTime`) 0.5 true))

(event `SV_AddVictory`
  (params (VictoryTeam :type "/Game/BombScenario/Blueprints/Data/E_Team Enum" :default "NewEnumerator0"))
  ;[0.1176 0.1176 0.1176] Round over, add victory
  (`/Engine/EditorBlueprintResources/StandardMacros.IncrementInt` (`self.RoundsPlayed`)
    (:`  `
      (`self.SV_RoundOver` VictoryTeam)
      (switch `/Game/BombScenario/Blueprints/Data/E_Team` VictoryTeam
        (:`NewEnumerator0`
          (`self.AddPoint` :!label _label)
          (`self.ResetTeamArrays`)
          (`self.HalfTime?`)
          (`self.HasAnyoneWon?`))
        (:`NewEnumerator1`
          (goto _label :!via `TeamB`))))))

(event `HalfTime?`
  ;[0.1176 0.1176 0.1176] Has the half time been reached?
  (if (== (`self.RoundsPlayed`) (/ (`self.TotalRounds`) 2))
    (`self.SV_SwitchTeams`)))

(event `UpdateRoundTime`
  ;[0.1176 0.1176 0.1176] Round Timer
  (set `self.RoundTimeLeft` (`KismetSystemLibrary.K2_GetTimerRemainingTimeHandle` (`self.TH_RoundTimeLeft`)))
  (`self.ForceNetUpdate`))

(event `HasAnyoneWon?`
  ;[0.1176 0.1176 0.1176] Let's see if a team has won
  (if (== (`self.ScoreA`) (+ (/ (`self.TotalRounds`) 2) 1))
    ;[0.1176 0.1176 0.1176] Team A have won
    (`self.SV_GameOver` "NewEnumerator0")
    (`self.DestroyAllInteractable`)
    (elif (== (`self.ScoreB`) (+ (/ (`self.TotalRounds`) 2) 1))
      ;[0.1176 0.1176 0.1176] Team B have won
      (`self.SV_GameOver` "NewEnumerator1")
      (`self.DestroyAllInteractable`)
      (else
        ;[0.1176 0.1176 0.1176] No winner, next round
        (`KismetSystemLibrary.Delay` (`self.TimeBetweenRounds`))
        (`self.StartRound`)))))

(event `SV_SpawnedPlayer`
  (params (PlayerController :type "PlayerController Object Reference"))
  ;[0.1176 0.1176 0.1176] New joined Player
  (`/Engine/EditorBlueprintResources/ActorMacros.Switch Has Authority`
    (:`Authority`
      (`KismetArrayLibrary.Array_Add` (`self.SpawnedPlayer`) PlayerController))))

(event `SV_GameOver`
  (params (VictoryTeam :type "/Game/BombScenario/Blueprints/Data/E_Team Enum" :default "NewEnumerator0"))
  ;[0.1176 0.1176 0.1176] There is a winner, Game Over
  (set `self.GameOver` true)
  (`/Game/BombScenario/Blueprints/Game/BP_BombScenario_GM.SV_ShowGameOver` (`self.BS_GameMode_Ref`) VictoryTeam))

(event `SV_RoundOver`
  (params (VictoryTeam :type "/Game/BombScenario/Blueprints/Data/E_Team Enum" :default "NewEnumerator0"))
  ;[0.1176 0.1176 0.1176] Show everyone the Round Over screens
  (`/Game/BombScenario/Blueprints/Game/BP_BombScenario_GM.SV_ShowRoundOver` (`self.BS_GameMode_Ref`) VictoryTeam))

(event `TimeOut`
  ;[0.1176 0.1176 0.1176] When the round time is over, Team B wins
  (`self.SV_AddVictory` "NewEnumerator1"))

(event `self.ReceiveBeginPlay`
  ;[0.1176 0.1176 0.1176] The round starts and all items are spawned
  (bind _asbp_bomb_scenario_gm (cast `/Game/BombScenario/Blueprints/Game/BP_BombScenario_GM` (`GameplayStatics.GetGameMode`)))
  (set `self.BS_GameMode_Ref` _asbp_bomb_scenario_gm)
  (`/Engine/EditorBlueprintResources/ActorMacros.Switch Has Authority`
    (:`Authority`
      (if (not (`self.GameStarted`))
        (bind _returnvalue (`KismetSystemLibrary.K2_SetTimerDelegate` (delegate `SpawnPlayer`) 0.5 true))
        (set `self.TH_Spawn` _returnvalue)))))

(event `SV_BombPlanted`
  ;[0.1176 0.1176 0.1176] Show everyone that the bomb was planted
  (for _array_element (`/Game/BombScenario/Blueprints/Game/BP_BombScenario_GM.AllSpawnedPlayer` (`self.BS_GameMode_Ref`))
    (bind _ascharacter (cast `Character` _array_element))
    (bind _returnvalue (`self.GetComponentByClass` _ascharacter "/Game/BombScenario/Blueprints/Data/BS_CharacterComponent.BS_CharacterComponent_C"))
    (`/Engine/EditorBlueprintResources/StandardMacros.IsValid` _returnvalue
      (:`Is Valid`
        (`/Game/BombScenario/Blueprints/Data/BS_CharacterComponent.CL_ShowBombPlanted` _returnvalue)))))

(event `SpawnPlayer`
  ;[0.1176 0.1176 0.1176] The round starts and all items are spawned
  (`/Game/BombScenario/Blueprints/Game/BP_BombScenario_GM.SV_SpawnJoinedPlayer` (`self.BS_GameMode_Ref`)))

(event `SV_SwitchTeams`
  ;[0.1176 0.1176 0.1176] Change of the two teams and the scores
  (for _array_element (`/Game/BombScenario/Blueprints/Game/BP_BombScenario_GM.AllPlayers` (`self.BS_GameMode_Ref`))
    (bind _returnvalue (`self.GetComponentByClass` _array_element "/Game/BombScenario/Blueprints/Data/BS_ControllerComponent.BS_ControllerComponent_C"))
    (`/Engine/EditorBlueprintResources/StandardMacros.IsValid` _returnvalue
      (:`Is Valid`
        (switch `/Game/BombScenario/Blueprints/Data/E_Team` (`/Game/BombScenario/Blueprints/Data/BS_ControllerComponent.Team` _returnvalue)
          (:`NewEnumerator0`
            (`/Game/BombScenario/Blueprints/Data/BS_ControllerComponent.SV_SelectTeam` _returnvalue "NewEnumerator1"))
          (:`NewEnumerator1`
            (`/Game/BombScenario/Blueprints/Data/BS_ControllerComponent.SV_SelectTeam` _returnvalue "NewEnumerator0"))))))
  (set `self.TemporaryScoreA` (`self.ScoreB`))
  (set `self.TemporaryScoreB` (`self.ScoreA`))
  (set `self.ScoreA` (`self.TemporaryScoreA`))
  (set `self.ScoreB` (`self.TemporaryScoreB`)))

(event `StartRound`
  ;[0.1176 0.1176 0.1176] Start Round
  (set `self.RoundStarted` false)
  (`KismetSystemLibrary.K2_ClearAndInvalidateTimerHandle` (`self.TH_Spawn`))
  (`self.DestroyAllCharacter`
    (:`Completed`
      (`self.DestroyAllInteractable`
        (:`Completed`
          (`self.ResetRoundVariables`)
          (`self.SpawnAllItems`)
          (bind _returnvalue (`KismetSystemLibrary.K2_SetTimerDelegate` (delegate `NextRound`) (`self.StartTimer`)))
          (set `self.TH_StartTimer` _returnvalue)
          (`/Game/BombScenario/Blueprints/Game/BP_BombScenario_GM.SV_SpawnAllPlayer` (`self.BS_GameMode_Ref`))
          (bind _returnvalue_2 (`KismetSystemLibrary.K2_SetTimerDelegate` (delegate `UpdateStartTimer`) 0.5 true))
          (set `self.TH_UpdateStartTimer` _returnvalue_2)
          (`self.UpdateStartTimer`))))))

(event `UpdateStartTimer`
  ;[0.1176 0.1176 0.1176] Start Round
  (set `self.RoundStartsIn` (`KismetSystemLibrary.K2_GetTimerRemainingTimeHandle` (`self.TH_StartTimer`)))
  (`self.ForceNetUpdate`))

(event `NextRound`
  ;[0.1176 0.1176 0.1176] Start Round
  (`/Game/BombScenario/Blueprints/Game/BP_BombScenario_GM.SV_EnableMovement` (`self.BS_GameMode_Ref`))
  (`self.StartRoundTimer`)
  (`KismetSystemLibrary.K2_ClearAndInvalidateTimerHandle` (`self.TH_UpdateStartTimer`))
  (set `self.RoundStarted` true)
  (set `self.GameStarted` true))

(fn `Bomb Planted`
  (params (BombPlanted :type Boolean))
  (set `self.BombPlanted` BombPlanted)
  (`KismetSystemLibrary.K2_ClearAndInvalidateTimerHandle` (`self.TH_RoundTimeLeft`))
  (`self.SV_BombPlanted`))

(fn `BombExploded`
  (params (Exploded :type Boolean))
  (set `self.Exploded` Exploded))

(fn `Explosion Timer`
  (params (ExplosionTimeLeft :type "Float (double-precision)"))
  (set `self.ExplosionTimeLeft` ExplosionTimeLeft))

(fn `ResetRoundVariables`
  (set `self.BombPlanted` false)
  (set `self.Exploded` false))

(fn `ResetTeamArrays`
  (bind _bs_gamemode_ref (`self.BS_GameMode_Ref`))
  (`KismetArrayLibrary.Array_Clear` (`/Game/BombScenario/Blueprints/Game/BP_BombScenario_GM.AllLivingPlayers_TeamA` _bs_gamemode_ref))
  (`KismetArrayLibrary.Array_Clear` (`/Game/BombScenario/Blueprints/Game/BP_BombScenario_GM.AllLivingPlayers_TeamB` _bs_gamemode_ref)))

(fn `SpawnAllItems`
  (bind _outactors (`GameplayStatics.GetAllActorsOfClass` "/Game/BombScenario/Blueprints/BP_ItemSpawner.BP_ItemSpawner_C"))
  (for _array_element _outactors
    (`/Game/BombScenario/Blueprints/BP_ItemSpawner.SV_SpawnItem` _array_element)))

(fn `UserConstructionScript`
  ;[0.1176 0.1176 0.1176] Loads your settings from the DT_GameStateSettings
  (bind _returnvalue (`|GetDataTableRow` "/Game/BombScenario/Blueprints/DT_GameStateSettings.DT_GameStateSettings" "1")
    (:`then`
      (bind (_roundtime _totalrounds _roundstartsintime _timebetweenrounds) (break `/Game/BombScenario/Blueprints/Data/Structures/Struct_GameStateSettings` _returnvalue))
      (bind _output_get (set `self.RoundTime` _roundtime))
      (set `self.RoundTimeLeft` _output_get)
      (set `self.TotalRounds` _totalrounds)
      (set `self.StartTimer` _roundstartsintime)
      (set `self.TimeBetweenRounds` _timebetweenrounds))))