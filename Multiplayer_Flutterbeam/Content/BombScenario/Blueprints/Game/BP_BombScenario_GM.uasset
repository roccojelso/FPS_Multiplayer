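; Game mode for a two-team bomb scenario that runs the lobby, spawning, round flow and game over.
; Lobby events gather player infos, set whether the match can start and handle kicks.
; Characters spawn at random team starts, and a random Team A member gets the bomb.
; Deaths shrink living-team arrays, awarding victory via the GameState depending on bomb state, while controller and character components handle UI, movement and session teardown.
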(event `self.ReceiveBeginPlay`
  ;[0.1176 0.1176 0.1176] Begin Play
  (bind _asbp_bomb_scenario_gs (cast `/Game/BombScenario/Blueprints/Game/BP_BombScenario_GS` (`GameplayStatics.GetGameState`)))
  (set `self.BS_GameState_Ref` _asbp_bomb_scenario_gs))

(event `self.HandleStartingNewPlayer`
  (params (NewPlayer :type "PlayerController Object Reference"))
  (bind _returnvalue (`self.GetComponentByClass` (`self.NewPlayer`) "/Game/BombScenario/Blueprints/Data/BS_ControllerComponent.BS_ControllerComponent_C"))
  ;[0.1176 0.1176 0.1176] Add all new players to the Player in Game Array
  (bind _output_get (set `self.NewPlayer` NewPlayer))
  (`KismetArrayLibrary.Array_Add` (`self.AllPlayers`) _output_get)
  (`/Engine/EditorBlueprintResources/StandardMacros.IsValid` _returnvalue
    (:`Is Valid`
      (`/Game/BombScenario/Blueprints/Data/BS_ControllerComponent.CL_CreateLobby` _returnvalue))))

(event `SV_SpawnJoinedPlayer`
  (bind _spawnedplayer (`/Game/BombScenario/Blueprints/Game/BP_BombScenario_GS.SpawnedPlayer` (`self.BS_GameState_Ref`)))
  ;[0.1176 0.1176 0.1176] Spawn all new joined Player
  (for _array_element _spawnedplayer
    (`self.SV_SpawnCharacter` _array_element))
  (`KismetArrayLibrary.Array_Clear` _spawnedplayer))

(event `SV_SpawnCharacter`
  (params (PlayerController :type "PlayerController Object Reference"))
  ;[0.1176 0.1176 0.1176] Server Spawn Character
  (`self.SpawnCharacter` PlayerController))

(event `self.K2_OnLogout`
  (params (ExitingController :type "Controller Object Reference"))
  ;[0.1176 0.1176 0.1176] Remove Player on Logout
  (bind _asplayer_controller (cast `PlayerController` ExitingController))
  (`KismetArrayLibrary.Array_RemoveItem` (`self.AllPlayers`) _asplayer_controller))

(event `SV_SpawnAllPlayer`
  ;[0.1176 0.1176 0.1176] Spawn All Player
  (`KismetArrayLibrary.Array_Clear` (`self.AllSpawnedPlayer`))
  (`KismetArrayLibrary.Array_Clear` (`self.AllLivingPlayers_TeamA`))
  (`KismetArrayLibrary.Array_Clear` (`self.AllLivingPlayers_TeamB`))
  (for _array_element (`self.AllPlayers`)
    (`self.SV_SpawnCharacter` _array_element))
  (`self.SV_CreateHUD`)
  (`KismetSystemLibrary.Delay` 0.2)
  (`self.SV_SpawnBomb`))

(event `SV_AddDeath`
  (params (Team :type "/Game/BombScenario/Blueprints/Data/E_Team Enum" :default "NewEnumerator0") (Pawn :type "Pawn Object Reference"))
  (bind _alllivingplayers_teamb (`self.AllLivingPlayers_TeamB`))
  (bind _alllivingplayers_teama (`self.AllLivingPlayers_TeamA`))
  (bind _bs_gamestate_ref (`self.BS_GameState_Ref`))
  ;[0.1176 0.1176 0.1176] Removes the player from his team array and compares whether there are still living team members
  (`KismetArrayLibrary.Array_RemoveItem` (`self.AllSpawnedPlayer`) Pawn)
  (switch `/Game/BombScenario/Blueprints/Data/E_Team` Team
    (:`NewEnumerator0`
      (bind _returnvalue (`KismetArrayLibrary.Array_RemoveItem` _alllivingplayers_teama Pawn))
      (if _returnvalue
        (if (`KismetArrayLibrary.Array_IsValidIndex` _alllivingplayers_teama)
          _
          (elif (not (`/Game/BombScenario/Blueprints/Game/BP_BombScenario_GS.BombPlanted` _bs_gamestate_ref))
            (`/Game/BombScenario/Blueprints/Game/BP_BombScenario_GS.SV_AddVictory` _bs_gamestate_ref "NewEnumerator1")))))
    (:`NewEnumerator1`
      (bind _returnvalue_2 (`KismetArrayLibrary.Array_RemoveItem` _alllivingplayers_teamb Pawn))
      (if _returnvalue_2
        (if (`KismetArrayLibrary.Array_IsValidIndex` _alllivingplayers_teamb)
          _
          (elif (not (`/Game/BombScenario/Blueprints/Game/BP_BombScenario_GS.Exploded` _bs_gamestate_ref))
            (`/Game/BombScenario/Blueprints/Game/BP_BombScenario_GS.SV_AddVictory` _bs_gamestate_ref "NewEnumerator0")))))))

(event `SV_SpawnBomb`
  (bind _alllivingplayers_teama (`self.AllLivingPlayers_TeamA`))
  ;[0.1176 0.1176 0.1176] Give a random terrorist the bomb
  (if (`KismetArrayLibrary.Array_IsValidIndex` _alllivingplayers_teama)
    (bind _ascharacter (cast `Character` (`KismetArrayLibrary.Array_Random` _alllivingplayers_teama)))
    (bind _returnvalue (`self.GetComponentByClass` _ascharacter "/Game/BombScenario/Blueprints/Data/BS_CharacterComponent.BS_CharacterComponent_C"))
    (`/Engine/EditorBlueprintResources/StandardMacros.IsValid` _returnvalue
      (:`Is Valid`
        (`/Game/BombScenario/Blueprints/Data/BS_CharacterComponent.PickUpBomb` _returnvalue true)))))

(event `SV_EnableMovement`
  ;[0.1176 0.1176 0.1176] The round begins and the movement is activated
  (for _array_element (`self.AllSpawnedPlayer`)
    (bind _ascharacter (cast `Character` _array_element))
    (bind _returnvalue (`self.GetComponentByClass` _ascharacter "/Game/BombScenario/Blueprints/Data/BS_CharacterComponent.BS_CharacterComponent_C"))
    (`/Engine/EditorBlueprintResources/StandardMacros.IsValid` _returnvalue
      (:`Is Valid`
        (`/Game/BombScenario/Blueprints/Data/BS_CharacterComponent.SV_EnableMovement` _returnvalue)))))

(event `SV_ShowRoundOver`
  (params (VictoryTeam :type "/Game/BombScenario/Blueprints/Data/E_Team Enum" :default "NewEnumerator0"))
  ;[0.1176 0.1176 0.1176] Show Round Over Screen
  (for _array_element (`self.AllPlayers`)
    (bind _returnvalue (`self.GetComponentByClass` _array_element "/Game/BombScenario/Blueprints/Data/BS_ControllerComponent.BS_ControllerComponent_C"))
    (`/Engine/EditorBlueprintResources/StandardMacros.IsValid` _returnvalue
      (:`Is Valid`
        (`/Game/BombScenario/Blueprints/Data/BS_ControllerComponent.CL_ShowRoundOver` _returnvalue VictoryTeam)))))

(event `SV_CreateHUD`
  ;[0.1176 0.1176 0.1176] Create HUD and Disable Movement
  (for _array_element (`self.AllSpawnedPlayer`)
    (bind _ascharacter (cast `Character` _array_element))
    (bind _returnvalue (`self.GetComponentByClass` _ascharacter "/Game/BombScenario/Blueprints/Data/BS_CharacterComponent.BS_CharacterComponent_C"))
    (`/Engine/EditorBlueprintResources/StandardMacros.IsValid` _returnvalue
      (:`Is Valid`
        (`/Game/BombScenario/Blueprints/Data/BS_CharacterComponent.CL_CreateHUD` _returnvalue)
        (`/Game/BombScenario/Blueprints/Data/BS_CharacterComponent.SV_DisbaleMovement` _returnvalue)))))

(event `SV_ShowGameOver`
  (params (VictoryTeam :type "/Game/BombScenario/Blueprints/Data/E_Team Enum" :default "NewEnumerator0"))
  ;[0.1176 0.1176 0.1176] Show Game Over Screen
  (for _array_element (`self.AllPlayers`)
    (bind _returnvalue (`self.GetComponentByClass` _array_element "/Game/BombScenario/Blueprints/Data/BS_ControllerComponent.BS_ControllerComponent_C"))
    (`/Engine/EditorBlueprintResources/StandardMacros.IsValid` _returnvalue
      (:`Is Valid`
        (`/Game/BombScenario/Blueprints/Data/BS_ControllerComponent.CL_ShowGameOver` _returnvalue VictoryTeam))))
  (`self.SV_DestroySession`))

(event `SV_RemoveAllWidgets`
  ;[0.1176 0.1176 0.1176] Remove All Widgets
  (for _array_element (`self.AllSpawnedPlayer`)
    (bind _ascharacter (cast `Character` _array_element))
    (bind _returnvalue (`self.GetComponentByClass` _ascharacter "/Game/BombScenario/Blueprints/Data/BS_CharacterComponent.BS_CharacterComponent_C"))
    (`/Engine/EditorBlueprintResources/StandardMacros.IsValid` _returnvalue
      (:`Is Valid`
        (`/Game/BombScenario/Blueprints/Data/BS_CharacterComponent.CL_RemoveAllWidgets` _returnvalue)))))

(event `SV_DestroySession`
  ;[0.1176 0.1176 0.1176] Game over, Quit Game
  (`KismetSystemLibrary.Delay` 5.0)
  (for _array_element (`self.AllPlayers`)
    (bind _returnvalue (`self.GetComponentByClass` _array_element "/Game/BombScenario/Blueprints/Data/BS_ControllerComponent.BS_ControllerComponent_C"))
    (`/Engine/EditorBlueprintResources/StandardMacros.IsValid` _returnvalue
      (:`Is Valid`
        (`/Game/BombScenario/Blueprints/Data/BS_ControllerComponent.CL_DestroySession` _returnvalue)))))

(event `MC_UpdateAll`
  ;[0.1176 0.1176 0.1176] Multicast All Server Infos and Check Ready Status
  (`self.SV_RefreshList`)
  (for _array_element (`self.AllPlayers`)
    (bind _returnvalue (`self.GetComponentByClass` _array_element "/Game/BombScenario/Blueprints/Data/BS_ControllerComponent.BS_ControllerComponent_C"))
    (`/Engine/EditorBlueprintResources/StandardMacros.IsValid` _returnvalue
      (:`Is Valid`
        (`/Game/BombScenario/Blueprints/Data/BS_ControllerComponent.CL_AddPlayer` _returnvalue (`self.AllPlayerInfos`)))))
  (for _array_element_2 (`self.AllPlayerInfos`)
    (if (`|EnumEquality` (`.Ready_10_0D0847F04ABD3D8F47A4B1B29F3C54B5` (break `/Game/BombScenario/Blueprints/Data/Structures/Struct_LobbyPlayerInfos` _array_element_2)) "Checked")
      (`KismetArrayLibrary.Array_Add` (`self.ReadyPlayer`) (`.Ready_10_0D0847F04ABD3D8F47A4B1B29F3C54B5` (break `/Game/BombScenario/Blueprints/Data/Structures/Struct_LobbyPlayerInfos` _array_element_2)))))
  (if (== (`KismetArrayLibrary.Array_Length` (`self.ReadyPlayer`)) (`KismetArrayLibrary.Array_Length` (`self.AllPlayers`)))
    (set `self.MatchCanStart` true)
    (else
      (set `self.MatchCanStart` false))))

(event `SV_RefreshList`
  ;[0.1176 0.1176 0.1176] Server Refresh List
  (`KismetArrayLibrary.Array_Clear` (`self.AllPlayerInfos`))
  (`KismetArrayLibrary.Array_Clear` (`self.ReadyPlayer`))
  (for _array_element (`self.AllPlayers`)
    (bind _returnvalue (`self.GetComponentByClass` _array_element "/Game/BombScenario/Blueprints/Data/BS_ControllerComponent.BS_ControllerComponent_C"))
    (`/Engine/EditorBlueprintResources/StandardMacros.IsValid` _returnvalue
      (:`Is Valid`
        (`KismetArrayLibrary.Array_AddUnique` (`self.AllPlayerInfos`) (`/Game/BombScenario/Blueprints/Data/BS_ControllerComponent.PlayerInfo` _returnvalue))))))

(event `SV_StartRound`
  ;[0.1176 0.1176 0.1176] Start New Round
  (`self.SV_RemoveAllWidgets`)
  (`/Game/BombScenario/Blueprints/Game/BP_BombScenario_GS.StartRound` (`self.BS_GameState_Ref`)))

(event `SV_KickPlayer`
  (params (PlayerID :type Integer))
  (bind _returnvalue (`self.GetComponentByClass` (`|GetArrayItem` (`self.AllPlayers`) PlayerID) "/Game/BombScenario/Blueprints/Data/BS_ControllerComponent.BS_ControllerComponent_C"))
  ;[0.1176 0.1176 0.1176] Server Kick Player
  (`/Engine/EditorBlueprintResources/StandardMacros.IsValid` _returnvalue
    (:`Is Valid`
      (`/Game/BombScenario/Blueprints/Data/BS_ControllerComponent.CL_KickPlayer` _returnvalue))))

(fn `SelectPlayerStart_A`
  (returns (SpawnLocation :type "Transform Structure"))
  (bind _outactors (`GameplayStatics.GetAllActorsOfClass` "/Game/BombScenario/Blueprints/BP_PlayerStart_TeamA.BP_PlayerStart_TeamA_C"))
  (if (`KismetArrayLibrary.Array_IsValidIndex` _outactors)
    (return (`SceneComponent.K2_GetComponentToWorld` (`Actor.RootComponent` (`|GetArrayItem` _outactors (`KismetMathLibrary.RandomIntegerInRange` 0 (`KismetArrayLibrary.Array_LastIndex` _outactors))))))))

(fn `SelectPlayerStart_B`
  (returns (SpawnLocation :type "Transform Structure"))
  (bind _outactors (`GameplayStatics.GetAllActorsOfClass` "/Game/BombScenario/Blueprints/BP_PlayerStart_TeamB.BP_PlayerStart_TeamB_C"))
  (if (`KismetArrayLibrary.Array_IsValidIndex` _outactors)
    (return (`SceneComponent.K2_GetComponentToWorld` (`Actor.RootComponent` (`|GetArrayItem` _outactors (`KismetMathLibrary.RandomIntegerInRange` 0 (`KismetArrayLibrary.Array_LastIndex` _outactors))))))))

(fn `SpawnCharacter`
  (params (PlayerController :type "PlayerController Object Reference"))
  (locals (Team :type "/Game/BombScenario/Blueprints/Data/E_Team Enum"))
  (bind _returnvalue (`self.GetComponentByClass` PlayerController "/Game/BombScenario/Blueprints/Data/BS_ControllerComponent.BS_ControllerComponent_C"))
  ;[0.1176 0.1176 0.1176] Spawn Character based on his team selection
  (`/Engine/EditorBlueprintResources/StandardMacros.IsValid` _returnvalue
    (:`Is Valid`
      (`/Game/BombScenario/Blueprints/Data/BS_ControllerComponent.SV_SetIsPlaying` _returnvalue true)
      (bind _output_get (set `local.Team` (`/Game/BombScenario/Blueprints/Data/BS_ControllerComponent.Team` _returnvalue)))
      (switch `/Game/BombScenario/Blueprints/Data/E_Team` _output_get
        (:`NewEnumerator0`
          (bind _spawnlocation (`self.SelectPlayerStart_A`))
          (bind _returnvalue_2 (`|SpawnActorFromClass` "/Game/BombScenario/Blueprints/ThirdPersonCharacter.ThirdPersonCharacter_C" _spawnlocation "AlwaysSpawn" "OverrideRootScale" null null))
          (bind _returnvalue_3 (`self.GetComponentByClass` _returnvalue_2 "/Game/BombScenario/Blueprints/Data/BS_CharacterComponent.BS_CharacterComponent_C"))
          (`/Engine/EditorBlueprintResources/StandardMacros.IsValid` _returnvalue_3
            (:`Is Valid`
              (set `/Game/BombScenario/Blueprints/Data/BS_CharacterComponent.Team` (`local.Team`) _returnvalue_3)
              (`Controller.Possess` (`local.PlayerController`) _returnvalue_2)
              (`KismetArrayLibrary.Array_AddUnique` (`self.AllLivingPlayers_TeamA`) _returnvalue_2)
              (`KismetArrayLibrary.Array_AddUnique` (`self.AllSpawnedPlayer`) _returnvalue_2))))
        (:`NewEnumerator1`
          (bind _spawnlocation_2 (`self.SelectPlayerStart_B`))
          (bind _returnvalue_4 (`|SpawnActorFromClass` "/Game/BombScenario/Blueprints/ThirdPersonCharacter.ThirdPersonCharacter_C" _spawnlocation_2 "AlwaysSpawn" "OverrideRootScale" null null))
          (bind _returnvalue_5 (`self.GetComponentByClass` _returnvalue_4 "/Game/BombScenario/Blueprints/Data/BS_CharacterComponent.BS_CharacterComponent_C"))
          (`/Engine/EditorBlueprintResources/StandardMacros.IsValid` _returnvalue_5
            (:`Is Valid`
              (set `/Game/BombScenario/Blueprints/Data/BS_CharacterComponent.Team` (`local.Team`) _returnvalue_5)
              (`Controller.Possess` (`local.PlayerController`) _returnvalue_4)
              (`KismetArrayLibrary.Array_AddUnique` (`self.AllLivingPlayers_TeamB`) _returnvalue_4)
              (`KismetArrayLibrary.Array_AddUnique` (`self.AllSpawnedPlayer`) _returnvalue_4))))))))

(fn `UserConstructionScript`)