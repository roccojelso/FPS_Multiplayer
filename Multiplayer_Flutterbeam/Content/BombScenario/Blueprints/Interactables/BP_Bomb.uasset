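; Replicated bomb for a two-team bomb scenario: Team A picks it up and plants it, Team B defuses it.
; A DataTable row supplies its settings, and sphere overlaps offer pickup or defusal by team, with defuse kits halving interact time.
; Server-side timers drive the countdown and radial-damage explosion, while multicasts play effects.
; Explosion or defusal reports the winning team to the GameState, then destroys the actor.
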(event `SV_PlanBomb`
  (params (Instigator :type "Actor Object Reference"))
  ;[0.1176 0.1176 0.1176] Plan the Bomb
  (bind _ascharacter (cast `Character` Instigator))
  (bind _returnvalue (`self.GetComponentByClass` _ascharacter "/Game/BombScenario/Blueprints/Data/BS_CharacterComponent.BS_CharacterComponent_C"))
  (`/Engine/EditorBlueprintResources/StandardMacros.IsValid` _returnvalue
    (:`Is Valid`
      (`/Game/BombScenario/Blueprints/Data/BS_CharacterComponent.PickUpBomb` _returnvalue false)
      (set `self.BombPlanted?` true)
      (`self.ForceNetUpdate`)
      (bind _returnvalue_2 (`KismetSystemLibrary.K2_SetTimerDelegate` (delegate `Explosion`) (`self.TimeToExplosion`)))
      (set `self.TH_DetonationTime` _returnvalue_2)
      (bind _returnvalue_3 (`KismetSystemLibrary.K2_SetTimerDelegate` (delegate `UpdateExplosionTimer`) 0.2 true))
      (set `self.TH_UpdateExplosionTimer` _returnvalue_3)
      (`self.MC_PlantedEffects`))))

(event `Explosion`
  ;[0.1176 0.1176 0.1176] Plan the Bomb
  (`/Game/BombScenario/Blueprints/Game/BP_BombScenario_GS.BombExploded` (`self.BS_GameState_Ref`) true)
  (`self.Explode`))

(event `UpdateExplosionTimer`
  ;[0.1176 0.1176 0.1176] Plan the Bomb
  (bind _output_get (set `self.UpdateExplosionTime` (`KismetSystemLibrary.K2_GetTimerRemainingTimeHandle` (`self.TH_DetonationTime`))))
  (`/Game/BombScenario/Blueprints/Game/BP_BombScenario_GS.Explosion Timer` (`self.BS_GameState_Ref`) _output_get))

(event `PlanBomb`
  (params (Instigator :type "Actor Object Reference"))
  ;[0.1176 0.1176 0.1176] Plan the Bomb
  (`self.SV_PlanBomb` Instigator))

(event `MC_PlantedEffects`
  ;[0.1176 0.1176 0.1176] Multicast Bomb Planted Effects
  (bind _returnvalue (`KismetSystemLibrary.K2_SetTimerDelegate` (delegate `PlayPlantedEffects`) 0.5 true))
  (set `self.TH_PlantedEffects` _returnvalue))

(event `Explode`
  (bind (_returnvalue_x _returnvalue_y _returnvalue_z) (`KismetMathLibrary.BreakVector` (`self.K2_GetActorLocation`)))
  ;[0.1176 0.1176 0.1176] Explosion
  (`GameplayStatics.ApplyRadialDamage` :`BaseDamage` (`self.BombDamage`) :`Origin` (`KismetMathLibrary.MakeVector` _returnvalue_x _returnvalue_y (+ _returnvalue_z 45.0)) :`DamageRadius` (`self.BombRadius`) :`DamageCauser` null :`InstigatedByController` null)
  (`self.ClearTimerHandle`)
  (`self.MC_ExplosionEffect`)
  (`KismetSystemLibrary.Delay` 1.5)
  (`/Game/BombScenario/Blueprints/Game/BP_BombScenario_GS.SV_AddVictory` (`self.BS_GameState_Ref`) "NewEnumerator0")
  (`self.TearOff`)
  (`self.K2_DestroyActor`))

(event `PlayPlantedEffects`
  ;[0.1176 0.1176 0.1176] Multicast Bomb Planted Effects
  (`TextRenderComponent.K2_SetText` (`self.Timer`) (`KismetTextLibrary.Conv_DoubleToText` (`self.UpdateExplosionTime`) "HalfToEven" false true 1 324 0 0))
  (`SceneComponent.ToggleVisibility` (`self.PointLight`) false)
  (`GameplayStatics.PlaySoundAtLocation` "/Engine/VREditor/Sounds/UI/Selection_Changes.Selection_Changes" (`self.K2_GetActorLocation`) (struct) 1.0 1.0 0.0 null null null null))

(event `SV_DefuseBomb`
  (bind _bs_gamestate_ref (`self.BS_GameState_Ref`))
  ;[0.1176 0.1176 0.1176] Defuse the Bomb
  (set `self.BombDefused` true)
  (`self.ClearTimerHandle`)
  (`/Game/BombScenario/Blueprints/Game/BP_BombScenario_GS.SV_AddVictory` _bs_gamestate_ref "NewEnumerator1")
  (`KismetSystemLibrary.Delay` (`/Game/BombScenario/Blueprints/Game/BP_BombScenario_GS.TimeBetweenRounds` _bs_gamestate_ref))
  (`self.TearOff`)
  (`self.K2_DestroyActor`))

(event `/Game/BombScenario/Blueprints/Data/Interface/BPI_Interactable.Interact`
  (params (Instigator :type "Actor Object Reference"))
  ;[0.1176 0.1176 0.1176] Interact
  (if (not (`/Game/BombScenario/Blueprints/Game/BP_BombScenario_GS.Exploded` (`self.BS_GameState_Ref`)))
    (`self.SV_DefuseBomb`)))

(event `SV_PickupBomb`
  (params (BS_Component :type "/Game/BombScenario/Blueprints/Data/BS_CharacterComponent Object Reference"))
  ;[0.1176 0.1176 0.1176] Pick up the Bomb
  (`/Engine/EditorBlueprintResources/StandardMacros.IsValid` BS_Component
    (:`Is Valid`
      (`/Game/BombScenario/Blueprints/Data/BS_CharacterComponent.PickUpBomb` BS_Component true)
      (`self.TearOff`)
      (`self.K2_DestroyActor`))))

(event `MC_ExplosionEffect`
  (bind _returnvalue (`self.K2_GetActorLocation`))
  ;[0.1176 0.1176 0.1176] Multicast Explosion Effects
  (`GameplayStatics.SpawnEmitterAtLocation` (`self.ExplosionEmitter`) _returnvalue (struct) (`self.ExplosionEmitterScale`))
  (`GameplayStatics.PlaySoundAtLocation` (`self.ExplosionSound`) _returnvalue (struct) 1.0 1.0 0.0 null null null null))

(event `self.ReceiveBeginPlay`
  ;[0.1176 0.1176 0.1176] Set GameState Reference
  (bind _asbp_bomb_scenario_gs (cast `/Game/BombScenario/Blueprints/Game/BP_BombScenario_GS` (`GameplayStatics.GetGameState`)))
  (set `self.BS_GameState_Ref` _asbp_bomb_scenario_gs))

(event `self.Sphere.OnComponentEndOverlap`
  (params (OverlappedComponent :type "PrimitiveComponent Object Reference") (OtherActor :type "Actor Object Reference") (OtherComp :type "PrimitiveComponent Object Reference") (OtherBodyIndex :type Integer))
  ;[0.1176 0.1176 0.1176] On End Overlap Event
  (bind _ascharacter (cast `Character` OtherActor))
  (bind _returnvalue (`self.GetComponentByClass` _ascharacter "/Game/BombScenario/Blueprints/Data/BS_CharacterComponent.BS_CharacterComponent_C"))
  (`/Engine/EditorBlueprintResources/StandardMacros.IsValid` _returnvalue
    (:`Is Valid`
      (`/Game/BombScenario/Blueprints/Data/BS_CharacterComponent.SV_ShowInteractMessage` _returnvalue "Hidden")
      (set `self.InteractTime` (`self.DefaultInteractTime`)))))

(event `SetCollision`
  ;[0.1176 0.1176 0.1176] Set Collision
  (`PrimitiveComponent.SetCollisionResponseToAllChannels` (`self.Sphere`) "ECR_Overlap"))

(event `self.Sphere.OnComponentBeginOverlap`
  (params (OverlappedComponent :type "PrimitiveComponent Object Reference") (OtherActor :type "Actor Object Reference") (OtherComp :type "PrimitiveComponent Object Reference") (OtherBodyIndex :type Integer) (bFromSweep :type Boolean) (SweepResult :type "HitResult Structure (by ref)"))
  ;[0.1176 0.1176 0.1176] On Overlap Events
  (bind _ascharacter (cast `Character` OtherActor))
  (bind _returnvalue (`self.GetComponentByClass` _ascharacter "/Game/BombScenario/Blueprints/Data/BS_CharacterComponent.BS_CharacterComponent_C"))
  (`/Engine/EditorBlueprintResources/StandardMacros.IsValid` _returnvalue
    (:`Is Valid`
      (if (`self.BombPlanted?`)
        (`self.SelectTeam` _returnvalue
          (:`TeamB`
            (set `/Game/BombScenario/Blueprints/Data/BS_CharacterComponent.CanInteract` true _returnvalue)
            (`/Game/BombScenario/Blueprints/Data/BS_CharacterComponent.SV_ShowInteractMessage` _returnvalue "Visible")
            (set `/Game/BombScenario/Blueprints/Data/BS_CharacterComponent.Interactable` self _returnvalue)
            (`self.HasDefuseKit` _returnvalue)
            (set `/Game/BombScenario/Blueprints/Data/BS_CharacterComponent.InteractTime` (`self.InteractTime`) _returnvalue)))
        (else
          (`self.SelectTeam` _returnvalue
            (:`TeamA`
              (if (not (`/Game/BombScenario/Blueprints/Data/BS_CharacterComponent.CarriesTheBomb` _returnvalue))
                (`self.SV_PickupBomb` _returnvalue)))))))))

(fn `OnRep_BombPlanted?`
  (bind _asbp_bomb_scenario_gs (cast `/Game/BombScenario/Blueprints/Game/BP_BombScenario_GS` (`GameplayStatics.GetGameState`)))
  (`/Game/BombScenario/Blueprints/Game/BP_BombScenario_GS.Bomb Planted` _asbp_bomb_scenario_gs true)
  (`PrimitiveComponent.SetSimulatePhysics` (`self.ItemMesh`) true)
  (`PrimitiveComponent.SetCollisionResponseToAllChannels` (`self.Sphere`) "ECR_Overlap"))

(fn `UserConstructionScript`
  ;[0.1176 0.1176 0.1176] Loads all Bomb Settings from the DT_BombAndInteractSettings DataTable
  (bind _returnvalue (`|GetDataTableRow` "/Game/BombScenario/Blueprints/DT_BombAndInteractSettings.DT_BombAndInteractSettings" "C4")
    (:`then`
      (bind (_bombsettings _interactsettings) (break `/Game/BombScenario/Blueprints/Data/Structures/Struct_BombAndInteractSettings` _returnvalue))
      (`StaticMeshComponent.SetStaticMesh` (`self.ItemMesh`) (break `/Game/BombScenario/Blueprints/Data/Structures/Struct_BombSettings` _bombsettings))
      (set `self.TimeToExplosion` (`.TimetoExplosion_27_85239EE8445FF01C7BA631BD7AD5B8F3` (break `/Game/BombScenario/Blueprints/Data/Structures/Struct_BombSettings` _bombsettings)))
      (set `self.BombRadius` (`.ExplosionRadius_21_926C9DDB4D0ABA1B7C242E9F53C7FE99` (break `/Game/BombScenario/Blueprints/Data/Structures/Struct_BombSettings` _bombsettings)))
      (set `self.BombDamage` (`.ExplosionDamage_22_F06F8CFB40C33CCFD7C893B08B06EF3B` (break `/Game/BombScenario/Blueprints/Data/Structures/Struct_BombSettings` _bombsettings)))
      (set `self.ExplosionEmitter` (`.ExplosionEmitter_10_BD2F090148162D08AA28688E02053CA9` (break `/Game/BombScenario/Blueprints/Data/Structures/Struct_BombSettings` _bombsettings)))
      (set `self.ExplosionEmitterScale` (`.ExplosionEmitterScale_23_503D2473413A317849B41696F0765389` (break `/Game/BombScenario/Blueprints/Data/Structures/Struct_BombSettings` _bombsettings)))
      (set `self.ExplosionSound` (`.ExplosionSound_12_68041FAA4BCEEAA9B7AF8BA201FF2BE1` (break `/Game/BombScenario/Blueprints/Data/Structures/Struct_BombSettings` _bombsettings)))
      (set `self.DefaultInteractTime` (`.InteractTimeDefuseBomb_4_54773C10446459F05ACBE5A33F288F38` (break `/Game/BombScenario/Blueprints/Data/Structures/Struct_InteractSettings` _interactsettings)))
      (set `self.DefuseTime` (`.InteractTimeDefuseBomb_4_54773C10446459F05ACBE5A33F288F38` (break `/Game/BombScenario/Blueprints/Data/Structures/Struct_InteractSettings` _interactsettings))))))