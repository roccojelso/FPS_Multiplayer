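; Bomb zone interactable where a Team A bomb carrier can plant the bomb in the bomb scenario.
; Box overlaps set or clear the interact state, prompt, target and time on the character's BS_CharacterComponent.
; Interact spawns and plants BP_Bomb at the character's mesh and clears the carrier flag; SVDestroyActor is empty so the zone persists.
; The construction script loads plant time from a DataTable, then applies decal material and box extent.
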(event `self.BombZone.OnComponentBeginOverlap`
  (params (OverlappedComponent :type "PrimitiveComponent Object Reference") (OtherActor :type "Actor Object Reference") (OtherComp :type "PrimitiveComponent Object Reference") (OtherBodyIndex :type Integer) (bFromSweep :type Boolean) (SweepResult :type "HitResult Structure (by ref)"))
  ;[0.1176 0.1176 0.1176] Set Can Interact and Show Interact Message
  (bind _ascharacter (cast `Character` OtherActor))
  (bind _returnvalue (`self.GetComponentByClass` _ascharacter "/Game/BombScenario/Blueprints/Data/BS_CharacterComponent.BS_CharacterComponent_C"))
  (`/Engine/EditorBlueprintResources/StandardMacros.IsValid` _returnvalue
    (:`Is Valid`
      (`self.SelectTeam` _returnvalue
        (:`TeamA`
          (if (`/Game/BombScenario/Blueprints/Data/BS_CharacterComponent.CarriesTheBomb` _returnvalue)
            (set `/Game/BombScenario/Blueprints/Data/BS_CharacterComponent.CanInteract` true _returnvalue)
            (`/Game/BombScenario/Blueprints/Data/BS_CharacterComponent.SV_ShowInteractMessage` _returnvalue "Visible")
            (set `/Game/BombScenario/Blueprints/Data/BS_CharacterComponent.Interactable` self _returnvalue)
            (set `/Game/BombScenario/Blueprints/Data/BS_CharacterComponent.InteractTime` (`self.InteractTime`) _returnvalue)))))))

(event `self.BombZone.OnComponentEndOverlap`
  (params (OverlappedComponent :type "PrimitiveComponent Object Reference") (OtherActor :type "Actor Object Reference") (OtherComp :type "PrimitiveComponent Object Reference") (OtherBodyIndex :type Integer))
  ;[0.1176 0.1176 0.1176] Reset Can Interact and hide Interact Message
  (bind _ascharacter (cast `Character` OtherActor))
  (bind _returnvalue (`self.GetComponentByClass` _ascharacter "/Game/BombScenario/Blueprints/Data/BS_CharacterComponent.BS_CharacterComponent_C"))
  (`/Engine/EditorBlueprintResources/StandardMacros.IsValid` _returnvalue
    (:`Is Valid`
      (`self.SelectTeam` _returnvalue
        (:`TeamA`
          (set `/Game/BombScenario/Blueprints/Data/BS_CharacterComponent.CanInteract` false _returnvalue)
          (`/Game/BombScenario/Blueprints/Data/BS_CharacterComponent.SV_ShowInteractMessage` _returnvalue "Hidden")
          (set `/Game/BombScenario/Blueprints/Data/BS_CharacterComponent.Interactable` null _returnvalue))))))

(event `/Game/BombScenario/Blueprints/Data/Interface/BPI_Interactable.Interact`
  (params (Instigator :type "Actor Object Reference"))
  ;[0.1176 0.1176 0.1176] Event Interact
  (bind _ascharacter (cast `Character` Instigator))
  (bind _returnvalue (`|SpawnActorFromClass` "/Game/BombScenario/Blueprints/Interactables/BP_Bomb.BP_Bomb_C" (`SceneComponent.K2_GetComponentToWorld` (`Character.Mesh` _ascharacter)) "AlwaysSpawn" "OverrideRootScale" null null))
  (`/Game/BombScenario/Blueprints/Interactables/BP_Bomb.PlanBomb` _returnvalue Instigator)
  (`self.CarriesBomb` _ascharacter))

(event `CarriesBomb`
  (params (Character :type "Character Object Reference"))
  (bind _returnvalue (`self.GetComponentByClass` Character "/Game/BombScenario/Blueprints/Data/BS_CharacterComponent.BS_CharacterComponent_C"))
  ;[0.1176 0.1176 0.1176] Now he no longer wears the bomb
  (`/Engine/EditorBlueprintResources/StandardMacros.IsValid` _returnvalue
    (:`Is Valid`
      (set `/Game/BombScenario/Blueprints/Data/BS_CharacterComponent.CarriesTheBomb` false _returnvalue))))

(event `self.SV_DestroyActor`
  ;[0.1176 0.1176 0.1176] The Bomb Zone should not be destroyed
)

(fn `UserConstructionScript`
  ;[0.1176 0.1176 0.1176] Loads the time to place the bomb from the DT_BombAndInteractSettings DataTable
  (bind _returnvalue (`|GetDataTableRow` "/Game/BombScenario/Blueprints/DT_BombAndInteractSettings.DT_BombAndInteractSettings" "C4")
    (:`then`
      (bind (_interactsettings_pickupinteracttime _interactsettings_interacttimeplacebomb) (break `/Game/BombScenario/Blueprints/Data/Structures/Struct_InteractSettings` (break `/Game/BombScenario/Blueprints/Data/Structures/Struct_BombAndInteractSettings` _returnvalue)))
      (set `self.InteractTime` _interactsettings_interacttimeplacebomb)
      ;[0.1176 0.1176 0.1176] Set Bomb Zone Decal
      (`DecalComponent.SetDecalMaterial` (`self.Decal`) (`self.BombZoneDecal`))
      ;[0.1176 0.1176 0.1176] Set Bomb Zone Size
      (`BoxComponent.SetBoxExtent` (`self.BombZone`) (`self.BombZoneSize`) true))))