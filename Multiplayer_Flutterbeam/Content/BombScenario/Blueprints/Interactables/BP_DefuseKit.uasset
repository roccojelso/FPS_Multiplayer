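; BP_DefuseKit is a defuse kit pickup for the bomb scenario that only Team B characters can collect.
; Overlapping its sphere checks the character's BS_CharacterComponent for team and whether it already holds a kit.
; An SV-prefixed event then sets the kit on that component, tears off replication and destroys the actor.
; A separate event makes the sphere ignore all collision channels.
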(event `self.Sphere.OnComponentBeginOverlap`
  (params (OverlappedComponent :type "PrimitiveComponent Object Reference") (OtherActor :type "Actor Object Reference") (OtherComp :type "PrimitiveComponent Object Reference") (OtherBodyIndex :type Integer) (bFromSweep :type Boolean) (SweepResult :type "HitResult Structure (by ref)"))
  ;[0.1176 0.1176 0.1176] Pick up Defuse Kit on Overlap
  (bind _ascharacter (cast `Character` OtherActor))
  (bind _returnvalue (`self.GetComponentByClass` _ascharacter "/Game/BombScenario/Blueprints/Data/BS_CharacterComponent.BS_CharacterComponent_C"))
  (`/Engine/EditorBlueprintResources/StandardMacros.IsValid` _returnvalue
    (:`Is Valid`
      (`self.SelectTeam` _returnvalue
        (:`TeamB`
          (if (not (`/Game/BombScenario/Blueprints/Data/BS_CharacterComponent.DefuseKit` _returnvalue))
            (`self.SV_GetDefuseKit` _returnvalue)))))))

(event `SV_GetDefuseKit`
  (params (BS_Component :type "/Game/BombScenario/Blueprints/Data/BS_CharacterComponent Object Reference"))
  ;[0.1176 0.1176 0.1176] Add Defuse Kit to Character
  (`/Game/BombScenario/Blueprints/Data/BS_CharacterComponent.GetDefuseKit` BS_Component true)
  (`self.TearOff`)
  (`self.K2_DestroyActor`))

(event `SetCollision`
  ;[0.1176 0.1176 0.1176] Set Collision
  (`PrimitiveComponent.SetCollisionResponseToAllChannels` (`self.Sphere`) "ECR_Ignore"))

(fn `UserConstructionScript`
  (`parent.UserConstructionScript`))