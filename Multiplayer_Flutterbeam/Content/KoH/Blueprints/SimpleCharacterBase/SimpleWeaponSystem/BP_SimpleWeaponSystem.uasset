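; Weapon component for the owning character, driving firing, reloading, ammo and weapon UI from the current weapon actor's properties.
; The client fires on a looping fire-rate timer and traces from the camera; the server runs line-trace damage and spawns throttled trails, while multicasts play effects and sounds.
; Shooting and reload states reach the owner through interface messages.
; Crosshair and weapon-module widgets show ammo and hit/kill feedback; the camera shake event is empty.
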(event `SetCurrentWeapon`
  (params (CurrentWeapon :type "/Game/KoH/Blueprints/SimpleCharacterBase/SimpleWeaponSystem/Weapons/BP_BaseWeapon Object Reference"))
  ;[1 1 1] [SERVER] SET CURRENT WEAPON
  ;;[0.07371 1 0] WS Trigger form Owner. SetCurrentWeapon
  (set `self.CurrentWeapon` CurrentWeapon)
  (`KismetSystemLibrary.Delay` 0.2)
  ;;[1 1 1] [WEAPON SYSTEM UI] Update Weapon Module
  (`self.UpdateOnClientWeaponIcon`)
  (`self.UpdateOnClientAmmo`)
  (`self.UpdateOnClientWeaponName`))

(event `StartShooting`
  ;[1 1 1] [CLIENT] START SHOOTING
  ;;[0.07371 1 0] StartShooting
  ;;[1 1 1] Shooting Start Condition
  (if (not (`self.In Reload Weapon ?`))
    ;;[1 1 1] Check if ammo in clim == 0
    (if (== (`self.GetWeaponCurrentAmmoState`) 0)
      ;;[1 1 1] Logic if clip == 00 or pull == 0
      (if (not (== (`.CurrentAmmoPull` (`self.GetWeaponCurrentAmmoState`)) 0))
        ;;;[0 1 0.0568] Stop Shooting
        (`self.StopShooting`)
        ;;;[0 1 0.0568] Reload
        (`self.Reload`))
      (else
        ;;[1 1 1] Start Shooting Gate Logic
        (if (not (`self.In Shooting ?`))
          (`/Engine/EditorBlueprintResources/StandardMacros.DoOnce` false :!label _label
            (:`Completed`
              (set `self.In Shooting ?` true)
              ;;[1 0.9262 0] ServerStartShooting
              (`self.ServerStartShooting`)
              ;;[1 1 1] WS UI
              (`/Game/KoH/Blueprints/SimpleCharacterBase/SimpleWeaponSystem/UI/WBP_CrossHair.ShootingShakesON` (`self.CrossHair`) (`self.GetWeaponFireRate`))
              ;;[1 1 1] Start Timer of Create Shot Event (For Burst Type and AutoFire)
              (`self.CreateShot`)
              (`KismetSystemLibrary.K2_SetTimer` null "CreateShot" (`self.GetWeaponFireRate`) true))))))))

(event `ResetDoOnceShooting`
  ;[1 1 1] [CLIENT] START SHOOTING
  ;;[1 1 1] Start Shooting Gate Logic
  (goto _label :!via `Reset`))

(event `ServerStartShooting`
  ;[1 1 1] INTERFACE EVENTS TRIGGERS
  ;;[1 0.9262 0] ServerStartShooting
  ;;[0.2567 0 1] WS Interface. Shooting Start
  (message `/Game/KoH/Blueprints/SimpleCharacterBase/SimpleWeaponSystem/BP_SimpleWeaponSystemInterface.WSStartShooting` (`self.GetOwner`)))

(event `ServerMainReloadStart`
  ;[1 1 1] INTERFACE EVENTS TRIGGERS
  ;;[1 0.9262 0] ServerMainReloadStart
  ;;[0.2567 0 1] Comment
  (message `/Game/KoH/Blueprints/SimpleCharacterBase/SimpleWeaponSystem/BP_SimpleWeaponSystemInterface.WSMainReloadStart` (`self.GetOwner`)))

(event `ServerStopShooting`
  ;[1 1 1] INTERFACE EVENTS TRIGGERS
  ;;[1 0.9262 0] ServerStopShooting
  ;;[0.2567 0 1] WS Interface. Shooting Stop
  (message `/Game/KoH/Blueprints/SimpleCharacterBase/SimpleWeaponSystem/BP_SimpleWeaponSystemInterface.WSStopShooting` (`self.GetOwner`)))

(event `ServerMainReloadStop`
  ;[1 1 1] INTERFACE EVENTS TRIGGERS
  ;;[1 0.9262 0] ServerMainReloadStop
  ;;[0.2567 0 1] Comment
  (message `/Game/KoH/Blueprints/SimpleCharacterBase/SimpleWeaponSystem/BP_SimpleWeaponSystemInterface.WSMainReloadStop` (`self.GetOwner`)))

(event `StopShooting`
  ;[1 1 1] [CLIENT] STOP SHOOTING
  ;;[0.07371 1 0] StopShooting
  ;;[1 1 1] Stop Create Shot Event Timer
  (`KismetSystemLibrary.K2_ClearTimer` null "CreateShot")
  (set `self.In Shooting ?` false)
  ;;[1 1 1] Auto Logic
  (`self.ResetDoOnceShooting`)
  ;;[1 0.9262 0] ServerStopShooting
  (`self.ServerStopShooting`))

(event `CreateShot`
  ;[1 1 1] [CLIENT] CREATE SHOT
  ;;[1 1 1] Cheking Ammo Pull in Clip
  (if (and (>= (- (`self.GetWeaponCurrentAmmoState`) 1) 0) (not (`self.In Reload Weapon ?`)))
    (`|ExecutionSequence`
      (:`then_0`
        ;;[1 1 1] Recalculete current ammo in clip (per shoot)
        (`self.UpdateWeaponAmmoInClip` (- (`self.GetWeaponCurrentAmmoState`) 1))
        ;;[1 1 1] Create Trace
        (`self.CalculationShotOnClient`))
      (:`then_1`
        ;;[1 1 1] Create Camera Shake
        (`self.CreateCameraShake`)))
    (else
      ;;[1 1 1] If clip == 0 when shooting true
      ;;;[0 1 0.0568] StopShooting
      (`self.StopShooting`)
      ;;;[0 1 0.0568] Reload
      (`self.Reload`))))

(event `Reload`
  (bind _currentammoinclip (`self.GetWeaponCurrentAmmoState`))
  (bind _clipsize (`self.GetWeaponAmmoProperties`))
  ;[1 1 1] [CLIENT / SERVER] RELOAD
  ;;[0 1 0.0568] Reload
  ;;[1 1 1] Checking conditions for reload
  (if (and (> (`.CurrentAmmoPull` (`self.GetWeaponCurrentAmmoState`)) 0) (< _currentammoinclip _clipsize) (not (== _currentammoinclip _clipsize)))
    (set `self.In Reload Weapon ?` true)
    ;;[1 0.9262 0] ServerMainReloadStart
    (`self.ServerMainReloadStart`)
    ;;[1 1 1] Delay for reload time
    (`KismetSystemLibrary.Delay` (`self.GetWeaponReloadTime`))
    ;;[1 0.9262 0] ServerMainReloadStop
    (`self.ServerMainReloadStop`)
    ;;[1 1 1] Ammo calculation
    (bind (_new_current_ammo_in_clip _new_current_ammo_pull) (`self.ReloadAmmoCalculation`))
    ;;[1 1 1] [server] Ammo calculation
    (`self.UpdateWeaponAmmoInClip` _new_current_ammo_in_clip)
    (`self.UpdateWeaponAmmoPull` _new_current_ammo_pull)
    (set `self.In Reload Weapon ?` false)))

(event `UpdateWeaponAmmoInClip`
  (params (CurrentAmmoInClip :type Integer))
  ;[1 1 1] [CLIENT / SERVER] RELOAD
  ;;[1 1 1] [server] Update Ammo State
  (`self.SetWeaponCurrentAmmoInClip` CurrentAmmoInClip))

(event `UpdateWeaponAmmoPull`
  (params (CurrentAmmoPull :type Integer))
  ;[1 1 1] [CLIENT / SERVER] RELOAD
  ;;[1 1 1] [server] Update Ammo State
  (`self.SetWeaponCurrentAmmoPull` CurrentAmmoPull))

(event `CalculationShotOnClient`
  ;[1 1 1] [CLIENT] CALCULATION SHOT ON CLIENT
  (`|ExecutionSequence`
    (:`then_0`
      ;;[1 1 1] Trigger SFX Sound On Weapon
      (`self.TriggerSFXSoundOnWeapon`))
    (:`then_1`
      ;;[1 1 1] Calc Start & End Potin Trace
      (bind (_start_trace_point _end_trace_point) (`self.CalculateTrace`))
      ;;[1 1 1] Initilize Weapon trace description
      (bind _output_get (set `self.WeaponTraceDescription` (make `/Game/KoH/Blueprints/SimpleCharacterBase/SimpleWeaponSystem/SystemProperties/STR_WeaponTraceDescription` _start_trace_point _end_trace_point)))
      ;;[1 1 1] Create trace on server
      (`self.CreateSingleTraceOnServer` _output_get (`SceneComponent.GetSocketLocation` (`/Game/KoH/Blueprints/SimpleCharacterBase/SimpleWeaponSystem/Weapons/BP_BaseWeapon.SkeletalMesh` (`self.CurrentWeapon`)) "Muzzle")))))

(event `HideMainTrailIfScope`
  (params (CreatedTrail :type "/Game/KoH/Blueprints/SimpleCharacterBase/SimpleWeaponSystem/BP_BaseWeaponTrail Object Reference"))
  (`SceneComponent.SetHiddenInGame` (`/Game/KoH/Blueprints/SimpleCharacterBase/SimpleWeaponSystem/BP_BaseWeaponTrail.ParticleSystem` CreatedTrail) true true))

(event `CreateSingleTraceOnServer`
  (params (`Weapon Trace` :type "/Game/KoH/Blueprints/SimpleCharacterBase/SimpleWeaponSystem/SystemProperties/STR_WeaponTraceDescription Structure") (`Muzzle Location` :type "Vector Structure"))
  (bind (_linetracestartpoint _linetraceendpoint) (break `/Game/KoH/Blueprints/SimpleCharacterBase/SimpleWeaponSystem/SystemProperties/STR_WeaponTraceDescription` `Weapon Trace`))
  ;[1 1 1] [SERVER] CREATE SINGLE TRACE
  ;;[1 1 1] Create Trace
  (bind (_damage_from_line_trace _hitactor _blockinghit _hit_location _normal) (`self.ShootingLineTrace` _linetracestartpoint _linetraceendpoint (`self.GetWeaponDamageWeaponProperties`) (`self.GetOwner`)))
  ;;[1 1 1] Apply Damage on each single line trace
  (`self.ApplyDamage` _hitactor _damage_from_line_trace (`self.GetOwner`))
  ;;[1 1 1] Trigger Hitted sfx and sounds for All
  (`self.CreateSingleTraceOnAll` _hitactor _blockinghit _hit_location _normal)
  ;;[1 1 1] [SERVER] Trail
  (`/Engine/EditorBlueprintResources/StandardMacros.DoOnce` false :!label _label
    (:`Completed`
      (`self.CreateWeaponTrail` `Muzzle Location` _linetraceendpoint)
      (`KismetSystemLibrary.Delay` (* (`.Trail Frequency` (`self.GetWeaponSFXWeaponProperties`)) (`self.GetWeaponFireRate`)))
      (`self.ServerResetSingleTrailGate`))))

(event `CreateSingleTraceOnAll`
  (params (HitActor :type "Actor Object Reference") (BlockingHit :type Boolean) (`Hit Location` :type "Vector Structure") (Normal :type "Vector Structure") (`Hit Point Sound` :type "SoundBase Object Reference") (`Hit Point SFX` :type "ParticleSystem Object Reference"))
  ;[1 1 1] [MULTICAST] CREATE SINGLE TRACE. HIT POTIN SFX & SOUND
  (`self.LineTraceHit` HitActor BlockingHit `Hit Location` Normal `Hit Point Sound` `Hit Point SFX`))

(event `ServerResetSingleTrailGate`
  ;[1 1 1] [SERVER] CREATE SINGLE TRACE
  ;;[1 1 1] [SERVER] Trail
  (goto _label :!via `Reset`))

(event `TriggerSFXSoundOnWeapon`
  ;[1 1 1] [SERVER & MULTICAST] SOUNDS & SFX ON WEAPON
  ;;[1 1 1] [SERVER] Trigger SFX Sound On Weapon
  ;;;[1 1 1] Start sfx
  (`self.AllPlaySFXSoundOnWeapon`)
  ;;;[1 0.04677 0] Stop sfx logic
  (`KismetSystemLibrary.Delay` (`KismetMathLibrary.FClamp` (`self.GetWeaponFireRate`) 0.12 0.18))
  ;;;[1 1 1] Stop sfx
  (`self.AllStopSFXOnWeapon`))

(event `AllStopSFXOnWeapon`
  (bind _skeletalmesh (`/Game/KoH/Blueprints/SimpleCharacterBase/SimpleWeaponSystem/Weapons/BP_BaseWeapon.SkeletalMesh` (`self.CurrentWeapon`)))
  (bind _skeletalmesh_2 (`/Game/KoH/Blueprints/SimpleCharacterBase/SimpleWeaponSystem/Weapons/BP_BaseWeapon.SkeletalMesh` (`self.CurrentWeapon`)))
  ;[1 1 1] [SERVER & MULTICAST] SOUNDS & SFX ON WEAPON
  ;;[1 1 1] [MULTICAST] AllPlaySFXSoundOnWeapon & AllStopSFXOnWeapon
  (`|ExecutionSequence`
    (:`then_0`
      ;;;[1 1 1] Destroy Mazzle SFX (Main Logic for all)
      (`/Engine/EditorBlueprintResources/StandardMacros.IsValid` (stale `AllPlaySFXSoundOnWeapon` _returnvalue)
        (:`Is Valid`
          (`self.K2_DestroyComponent` (stale `AllPlaySFXSoundOnWeapon` _returnvalue)))))
    (:`then_1`
      (goto _label_2 :!via `Reset`))))

(event `AllPlaySFXSoundOnWeapon`
  (bind _skeletalmesh (`/Game/KoH/Blueprints/SimpleCharacterBase/SimpleWeaponSystem/Weapons/BP_BaseWeapon.SkeletalMesh` (`self.CurrentWeapon`)))
  (bind _skeletalmesh_2 (`/Game/KoH/Blueprints/SimpleCharacterBase/SimpleWeaponSystem/Weapons/BP_BaseWeapon.SkeletalMesh` (`self.CurrentWeapon`)))
  ;[1 1 1] [SERVER & MULTICAST] SOUNDS & SFX ON WEAPON
  ;;[1 1 1] [MULTICAST] AllPlaySFXSoundOnWeapon & AllStopSFXOnWeapon
  (`|ExecutionSequence`
    (:`then_0`
      ;;;[1 1 1] Create Muzzle SFX
      (`/Engine/EditorBlueprintResources/StandardMacros.DoOnce` false :!label _label_2
        (:`Completed`
          (bind _returnvalue (`GameplayStatics.SpawnEmitterAttached` (`self.GetWeaponSFXWeaponProperties`) _skeletalmesh "muzzle" (`SceneComponent.GetSocketLocation` _skeletalmesh "Muzzle") (`SceneComponent.GetSocketRotation` _skeletalmesh "Muzzle") (1.0 1.0 1.0) "KeepWorldPosition" false))
          ;;;[1 1 1] Create Shell SFX
          (`GameplayStatics.SpawnEmitterAttached` (`self.GetWeaponShellSFXWeaponProperties`) _skeletalmesh_2 "Shell" (`SceneComponent.GetSocketLocation` _skeletalmesh_2 "Shell") (`SceneComponent.GetSocketRotation` _skeletalmesh_2 "Shell") (1.0 1.0 1.0) "KeepWorldPosition"))))
    (:`then_1`
      ;;;[1 1 1] Create sound on weapon
      (`GameplayStatics.PlaySoundAtLocation` (`self.GetWeaponSoundWeaponProperties`) (`Actor.K2_GetActorLocation` (`self.CurrentWeapon`)) (struct) (`self.Weapon Sound Volume Multiplier`) 1.0 0.0 null null null))))

(event `self.ReceiveTick`
  (params (DeltaSeconds :type "Float (single-precision)"))
  ;[1 1 1] MISC
  ;;[1 1 1] EVENT TICK
  (`KismetSystemLibrary.Delay` DeltaSeconds)
  (`|ExecutionSequence`
    (:`then_0`
      ;;;[1 1 1] Update crosshair
      (`self.UpdateCrossHair`))
    (:`then_1`
      ;;;[1 1 1] Update Weapon Module (current ammo state)
      (`self.UpdateOnClientAmmo`))))

(event `CreateCameraShake`
  ;[1 1 1] MISC
  ;;[1 1 1] [CLIENT] CREATE CAMERA SHAKES
)

(event `UpdateCrossHair`
  ;[1 1 1] UI
  ;;[1 1 1] UPDATE CROSSHAIR MODULE & SOUNDS ON DAMAGED / KILLED OF TARGES
  ;;;[1 1 1] Update Spead value for crosshair elements
  (`/Engine/EditorBlueprintResources/StandardMacros.IsValid` (`self.CrossHair`)
    (:`Is Valid`
      (`/Game/KoH/Blueprints/SimpleCharacterBase/SimpleWeaponSystem/UI/WBP_CrossHair.UpdateCrossHair` (`self.CrossHair`) 0.0))))

(event `CreateWeaponSystemUI`
  ;[1 1 1] UI
  ;;[1 1 1] CREATE WEAPON SYSTEM UI MODULES
  ;;;[0.07371 1 0] WS Trigger form Owner. CreateWeaponSystemUI
  (`|ExecutionSequence`
    (:`then_0`
      ;;;[1 1 1] Create Crosshair
      (bind _returnvalue (`|CreateWidget` "/Game/KoH/Blueprints/SimpleCharacterBase/SimpleWeaponSystem/UI/WBP_CrossHair.WBP_CrossHair_C" (`GameplayStatics.GetPlayerController` 0)))
      (bind _output_get (set `self.CrossHair` _returnvalue))
      (`/Engine/EditorBlueprintResources/StandardMacros.IsValid` _output_get
        (:`Is Valid`
          (`KismetSystemLibrary.Delay` 0.3)
          (`UserWidget.AddToPlayerScreen` (`self.CrossHair`) 3))))
    (:`then_1`
      ;;;[1 1 1] Create weapon module
      (bind _returnvalue_2 (`|CreateWidget` "/Game/KoH/Blueprints/SimpleCharacterBase/SimpleWeaponSystem/UI/WBP_WeaponModule.WBP_WeaponModule_C" (`GameplayStatics.GetPlayerController` 0)))
      (bind _output_get_2 (set `self.WeaponModule` _returnvalue_2))
      (`/Engine/EditorBlueprintResources/StandardMacros.IsValid` _output_get_2
        (:`Is Valid`
          (`UserWidget.AddToPlayerScreen` (`self.WeaponModule`) 3))))))

(event `ValidTargetKilled`
  ;[1 1 1] UI
  ;;[1 1 1] UPDATE CROSSHAIR MODULE & SOUNDS ON DAMAGED / KILLED OF TARGES
  ;;;[1 1 1] Show killed markers
  (`/Game/KoH/Blueprints/SimpleCharacterBase/SimpleWeaponSystem/UI/WBP_CrossHair.KillerTarget` (`self.CrossHair`))
  ;;;;[1 1 1] Play killed sound
  (`GameplayStatics.PlaySound2D` null (`self.Weapon Sound Volume Multiplier`) 1.0 0.0 null null))

(event `RemoveUI`
  ;[1 1 1] UI
  ;;[1 1 1] CREATE WEAPON SYSTEM UI MODULES
  (`Widget.RemoveFromParent` (`self.CrossHair`))
  (`Widget.RemoveFromParent` (`self.WeaponModule`)))

(event `ValidTargetDamaged`
  ;[1 1 1] UI
  ;;[1 1 1] UPDATE CROSSHAIR MODULE & SOUNDS ON DAMAGED / KILLED OF TARGES
  ;;;[1 1 1] Show damaged markers
  (`/Game/KoH/Blueprints/SimpleCharacterBase/SimpleWeaponSystem/UI/WBP_CrossHair.HitValidTarget` (`self.CrossHair`))
  ;;;;[1 1 1] Play Damaged sound
  (`GameplayStatics.PlaySound2D` null (`self.Weapon Sound Volume Multiplier`) 1.0 0.0 null null))

(event `UpdateOnClientWeaponIcon`
  (bind _weaponmodule (`self.WeaponModule`))
  ;[1 1 1] UI
  ;;[1 1 1] UPDATE WEAPON MODULE
  ;;;[1 1 1] UpdateOnClientWeaponIcon (on set weapon)
  (`KismetSystemLibrary.Delay` 0.1)
  (`/Engine/EditorBlueprintResources/StandardMacros.IsValid` _weaponmodule
    (:`Is Valid`
      (`/Game/KoH/Blueprints/SimpleCharacterBase/SimpleWeaponSystem/UI/WBP_WeaponModule.UpdateWeaponIcon` _weaponmodule (`self.GetWeaponIcon`)))))

(event `UpdateOnClientAmmo`
  (bind (_currentammoinclip _currentammopull) (`self.GetWeaponCurrentAmmoState`))
  ;[1 1 1] UI
  ;;[1 1 1] UPDATE WEAPON MODULE
  ;;;[1 1 1] UpdateOnClientAmmo
  (`/Engine/EditorBlueprintResources/StandardMacros.IsValid` (`self.WeaponModule`)
    (:`Is Valid`
      (`/Game/KoH/Blueprints/SimpleCharacterBase/SimpleWeaponSystem/UI/WBP_WeaponModule.UpdateAmmo` (`self.WeaponModule`) _currentammoinclip _currentammopull))))

(event `GetHittedActorHealth`
  (params (`Current Health` :type "Float (double-precision)") (`Apply Damage` :type "Float (double-precision)"))
  ;[1 1 1] UI
  ;;[1 1 1] UPDATE CROSSHAIR MODULE & SOUNDS ON DAMAGED / KILLED OF TARGES
  ;;;[1 1 1] HITTED / DAMAGED
  ;;;;[0.07371 1 0] WS Trigger form Owner. GetHittedActorHealth
  (if (<= `Current Health` 0.0)
    (`self.ValidTargetKilled`)
    (else
      (`self.ValidTargetDamaged`))))

(event `UpdateOnClientWeaponName`
  (bind _weaponmodule (`self.WeaponModule`))
  ;[1 1 1] UI
  ;;[1 1 1] UPDATE WEAPON MODULE
  ;;;[1 1 1] UpdateOnClientWeaponName
  (`/Engine/EditorBlueprintResources/StandardMacros.IsValid` _weaponmodule
    (:`Is Valid`
      (`/Game/KoH/Blueprints/SimpleCharacterBase/SimpleWeaponSystem/UI/WBP_WeaponModule.UpdateName` _weaponmodule (`self.GetWeaponName`)))))

(fn `ApplyDamage`
  (params (`Hited Actor` :type "Actor Object Reference") (BaseDamage :type "Float (double-precision)") (DamageCauser :type "Actor Object Reference"))
  (locals (`loc damage` :type "Float (double-precision)" :default 0.0))
  (`/Engine/EditorBlueprintResources/StandardMacros.IsValid` `Hited Actor`
    (:`Is Valid`
      (if (`Actor.HasAuthority` `Hited Actor`)
        (if (`KismetArrayLibrary.Array_Contains` (`self.Can Damage Actors Classes`) (`GameplayStatics.GetObjectClass` `Hited Actor`))
          (`GameplayStatics.ApplyDamage` `Hited Actor` BaseDamage null DamageCauser))))))

(fn `CalculateTrace`
  (returns (`Start Trace Point` :type "Vector Structure") (`End Trace Point` :type "Vector Structure"))
  (locals (`Loc Start Point` :type "Vector Structure" :default (0.0 0.0 0.0)) (`Loc End Point` :type "Vector Structure" :default (0.0 0.0 0.0)) (`Loc CurrentSpreadAngle` :type "Float (double-precision)" :default 0.0))
  ;[1 1 1] Comment
  (if false
    (set `self.Rotator` (struct))
    (else
      (set `self.Rotator` (`PlayerCameraManager.GetCameraRotation` (`GameplayStatics.GetPlayerCameraManager` 0)))))
  ;[1 1 1] Initialize Start Point
  (set `local.Loc Start Point` (`PlayerCameraManager.GetCameraLocation` (`GameplayStatics.GetPlayerCameraManager` 0)))
  ;[1 1 1] Initialize End Point /// Output
  (set `local.Loc End Point` (+ (`local.Loc Start Point`) (* (`KismetMathLibrary.GetForwardVector` (`self.Rotator`)) (`self.GetWeaponShootingMaxDistance`))))
  (return (`local.Loc Start Point`) (`local.Loc End Point`)))

(fn `CreateWeaponTrail`
  (params (`Muzzle Loc` :type "Vector Structure") (`End Trace Loc` :type "Vector Structure (by ref)") (Condition :type Boolean :default false))
  (bind (_muzzle_sfx _trail_sfx _trail_speed) (`self.GetWeaponSFXWeaponProperties`))
  (`/Engine/EditorBlueprintResources/StandardMacros.IsValid` (`self.CurrentWeapon`)
    (:`Is Valid`
      (bind _returnvalue (`|SpawnActorFromClass` "/Game/KoH/Blueprints/SimpleCharacterBase/SimpleWeaponSystem/BP_BaseWeaponTrail.BP_BaseWeaponTrail_C" (`KismetMathLibrary.MakeTransform` `Muzzle Loc` (`KismetMathLibrary.FindLookAtRotation` `Muzzle Loc` `End Trace Loc`) (`.Trail Scale` (`self.GetWeaponSFXWeaponProperties`))) "AlwaysSpawn" "OverrideRootScale" null null))
      (`/Game/KoH/Blueprints/SimpleCharacterBase/SimpleWeaponSystem/BP_BaseWeaponTrail.SetSFXTemplate` _returnvalue _trail_sfx)
      (if Condition
        (`self.HideMainTrailIfScope` null)
        (else
          (`/Game/KoH/Blueprints/SimpleCharacterBase/SimpleWeaponSystem/BP_BaseWeaponTrail.SetTrailSpeed` _returnvalue _trail_speed))))))

(fn `GetFABBIKAnim`
  (returns (`1STPP FABBIKAnim` :type "Transform Structure") (`3RDPP FABBIKAnim` :type "Transform Structure"))
  (bind _currentweapon (`self.CurrentWeapon`))
  (bind _skeletalmesh (`/Game/KoH/Blueprints/SimpleCharacterBase/SimpleWeaponSystem/Weapons/BP_BaseWeapon.SkeletalMesh` _currentweapon))
  (`/Engine/EditorBlueprintResources/StandardMacros.IsValid` _currentweapon
    (:`Is Valid`
      (return (`SceneComponent.GetSocketTransform` _skeletalmesh "L_HandSocket_1stpp" "RTS_Actor") (`SceneComponent.GetSocketTransform` _skeletalmesh "L_HandSocket_3rdpp" "RTS_Actor")))))

(fn `GetOwnerMuzzlePoint`
  (returns (`Muzzle Point` :type "Vector Structure"))
  (bind _returnvalue (`GameplayStatics.GetPlayerCameraManager` 0))
  (return (`KismetMathLibrary.MakeVector` (.x (+ (`PlayerCameraManager.GetCameraLocation` _returnvalue) (* (`KismetMathLibrary.GetForwardVector` (`PlayerCameraManager.GetCameraRotation` _returnvalue)) 20.0))) (.y (+ (`PlayerCameraManager.GetCameraLocation` _returnvalue) (* (`KismetMathLibrary.GetForwardVector` (`PlayerCameraManager.GetCameraRotation` _returnvalue)) 20.0))) (- (.z (+ (`PlayerCameraManager.GetCameraLocation` _returnvalue) (* (`KismetMathLibrary.GetForwardVector` (`PlayerCameraManager.GetCameraRotation` _returnvalue)) 20.0))) 20.0))))

(fn `GetReloadCondition`
  (returns (`Can Reload ?` :type Boolean))
  (bind (_currentammoinclip _currentammopull) (`self.GetWeaponCurrentAmmoState`))
  (return (or (not (== (`self.GetWeaponAmmoProperties`) _currentammoinclip)) (== _currentammopull 0))))

(fn `GetShootingCondition`
  (returns (`Can Shoot?` :type Boolean))
  (return (not (`self.In Reload Weapon ?`))))

(fn `GetWeaponAimRate`
  (returns (AimRate :type "Float (double-precision)"))
  (bind _currentweapon (`self.CurrentWeapon`))
  (`/Engine/EditorBlueprintResources/StandardMacros.IsValid` _currentweapon
    (:`Is Valid`
      (return (`.AimRate_168_2F7162BF457843690FF4AFB07FACC296` (break `/Game/KoH/Blueprints/SimpleCharacterBase/SimpleWeaponSystem/WeaponProperties/STR_BasicWeaponProperties` (`/Game/KoH/Blueprints/SimpleCharacterBase/SimpleWeaponSystem/Weapons/BP_BaseWeapon.BasicWeaponProperties` _currentweapon)))))))

(fn `GetWeaponAmmoProperties`
  (returns (ClipSize :type Integer) (AmmoSize :type Integer))
  (bind (_firerate _clipsize _ammosize) (break `/Game/KoH/Blueprints/SimpleCharacterBase/SimpleWeaponSystem/WeaponProperties/STR_BasicWeaponProperties` (`/Game/KoH/Blueprints/SimpleCharacterBase/SimpleWeaponSystem/Weapons/BP_BaseWeapon.BasicWeaponProperties` (`self.CurrentWeapon`))))
  (return _clipsize _ammosize))

(fn `GetWeaponCameraShake`
  (returns (`Camera Shake Class` :type "CameraShake Class Reference"))
  (bind _currentweapon (`self.CurrentWeapon`))
  (`/Engine/EditorBlueprintResources/StandardMacros.IsValid` _currentweapon
    (:`Is Valid`
      (return (`.CameraShakeClass_171_7DE69FCE49DB5EDD88781F83331D0576` (break `/Game/KoH/Blueprints/SimpleCharacterBase/SimpleWeaponSystem/WeaponProperties/STR_MiscWeaponProperties` (`/Game/KoH/Blueprints/SimpleCharacterBase/SimpleWeaponSystem/Weapons/BP_BaseWeapon.MiscWeaponProperties` _currentweapon)))))))

(fn `GetWeaponCurrentAmmoState`
  (returns (CurrentAmmoInClip :type Integer) (CurrentAmmoPull :type Integer))
  (bind _currentweapon (`self.CurrentWeapon`))
  (bind (_currentammoinclip _currentammopull) (break `/Game/KoH/Blueprints/SimpleCharacterBase/SimpleWeaponSystem/WeaponProperties/STR_CurrentAmmoState` (`/Game/KoH/Blueprints/SimpleCharacterBase/SimpleWeaponSystem/Weapons/BP_BaseWeapon.CurrentAmmoState` _currentweapon)))
  (`/Engine/EditorBlueprintResources/StandardMacros.IsValid` _currentweapon
    (:`Is Valid`
      (return _currentammoinclip _currentammopull))))

(fn `GetWeaponDamageWeaponProperties`
  (returns (`Damage Amount` :type "Float (double-precision)"))
  (bind _currentweapon (`self.CurrentWeapon`))
  (`/Engine/EditorBlueprintResources/StandardMacros.IsValid` _currentweapon
    (:`Is Valid`
      (return (`.DamageAmount_70_4890118A42A2CCB1BF3A2285234ACA91` (break `/Game/KoH/Blueprints/SimpleCharacterBase/SimpleWeaponSystem/WeaponProperties/STR_DamageWeaponProperties` (`/Game/KoH/Blueprints/SimpleCharacterBase/SimpleWeaponSystem/Weapons/BP_BaseWeapon.DamageWeaponProperties` _currentweapon)))))))

(fn `GetWeaponFireRate`
  (returns (ShotDelay :type "Float (double-precision)") (FireRate :type Integer))
  (bind _firerate (break `/Game/KoH/Blueprints/SimpleCharacterBase/SimpleWeaponSystem/WeaponProperties/STR_BasicWeaponProperties` (`/Game/KoH/Blueprints/SimpleCharacterBase/SimpleWeaponSystem/Weapons/BP_BaseWeapon.BasicWeaponProperties` (`self.CurrentWeapon`))))
  (return (/ 1.0 (/ (`KismetMathLibrary.Conv_IntToDouble` _firerate) 60.0)) _firerate))

(fn `GetWeaponIcon`
  (returns (`Weapon Icon` :type "Texture2D Object Reference"))
  (bind _currentweapon (`self.CurrentWeapon`))
  (`/Engine/EditorBlueprintResources/StandardMacros.IsValid` _currentweapon
    (:`Is Valid`
      (return (`.WeaponIcon_199_AADA25684315C53A9F97A1B399B32924` (break `/Game/KoH/Blueprints/SimpleCharacterBase/SimpleWeaponSystem/WeaponProperties/STR_MiscWeaponProperties` (`/Game/KoH/Blueprints/SimpleCharacterBase/SimpleWeaponSystem/Weapons/BP_BaseWeapon.MiscWeaponProperties` _currentweapon)))))))

(fn `GetWeaponName`
  (returns (WeaponName :type Text))
  (bind _currentweapon (`self.CurrentWeapon`))
  (`/Engine/EditorBlueprintResources/StandardMacros.IsValid` _currentweapon
    (:`Is Valid`
      (return (`.WeaponName_204_7F56BF404EC5ABFCC01BA8AC29B18AD3` (break `/Game/KoH/Blueprints/SimpleCharacterBase/SimpleWeaponSystem/WeaponProperties/STR_MiscWeaponProperties` (`/Game/KoH/Blueprints/SimpleCharacterBase/SimpleWeaponSystem/Weapons/BP_BaseWeapon.MiscWeaponProperties` _currentweapon)))))))

(fn `GetWeaponReloadTime`
  (returns (ReloadTime :type "Float (double-precision)") (`Bolt Action Reload Time` :type "Float (double-precision)"))
  (return (`.ReloadTime_204_A1857EB24E39B8A56EDB3BAE3A7CF3FC` (break `/Game/KoH/Blueprints/SimpleCharacterBase/SimpleWeaponSystem/WeaponProperties/STR_BasicWeaponProperties` (`/Game/KoH/Blueprints/SimpleCharacterBase/SimpleWeaponSystem/Weapons/BP_BaseWeapon.BasicWeaponProperties` (`self.CurrentWeapon`)))) 0.0))

(fn `GetWeaponSFXWeaponProperties`
  (returns (`Muzzle SFX` :type "ParticleSystem Object Reference") (`Trail SFX` :type "ParticleSystem Object Reference") (`Trail Speed` :type "Float (double-precision)") (`Trail Frequency` :type Integer) (`Trail Scale` :type "Vector Structure"))
  (bind (_muzzlesfx _trailsfx _trailspeed _trailfrequency _trailscale) (break `/Game/KoH/Blueprints/SimpleCharacterBase/SimpleWeaponSystem/WeaponProperties/STR_SFXWeaponProperties` (`/Game/KoH/Blueprints/SimpleCharacterBase/SimpleWeaponSystem/Weapons/BP_BaseWeapon.SFXWeaponProperties` (`self.CurrentWeapon`))))
  (return _muzzlesfx _trailsfx _trailspeed _trailfrequency _trailscale))

(fn `GetWeaponShellSFXWeaponProperties`
  (returns (`Shell SFX` :type "ParticleSystem Object Reference"))
  (return (`.ShellSFX_196_9C8E921346C5ED0BDB4098B6D857B7EC` (break `/Game/KoH/Blueprints/SimpleCharacterBase/SimpleWeaponSystem/WeaponProperties/STR_SFXWeaponProperties` (`/Game/KoH/Blueprints/SimpleCharacterBase/SimpleWeaponSystem/Weapons/BP_BaseWeapon.SFXWeaponProperties` (`self.CurrentWeapon`))))))

(fn `GetWeaponShootingMaxDistance`
  (returns (ShootingMaxDistance :type "Float (double-precision)"))
  (bind _currentweapon (`self.CurrentWeapon`))
  (`/Engine/EditorBlueprintResources/StandardMacros.IsValid` _currentweapon
    (:`Is Valid`
      (return (`/Game/KoH/Blueprints/SimpleCharacterBase/SimpleWeaponSystem/Weapons/BP_BaseWeapon.ShootingMaxDistance` _currentweapon)))))

(fn `GetWeaponSoundWeaponProperties`
  (returns (WeaponShotSoundCue :type "SoundCue Object Reference") (`Main Reload Start Sound` :type "SoundCue Object Reference") (`Main Reload Stop Sound` :type "SoundCue Object Reference"))
  (bind (_weaponshotsoundcue _mainreloadstartsound _mainreloadstopsound) (break `/Game/KoH/Blueprints/SimpleCharacterBase/SimpleWeaponSystem/WeaponProperties/STR_SoundWeaponProperties` (`/Game/KoH/Blueprints/SimpleCharacterBase/SimpleWeaponSystem/Weapons/BP_BaseWeapon.SoundWeaponProperties` (`self.CurrentWeapon`))))
  (return _weaponshotsoundcue _mainreloadstartsound _mainreloadstopsound))

(fn `LineTraceHit`
  (params (HitActor :type "Actor Object Reference") (BlockingHit :type Boolean) (`Hit Location` :type "Vector Structure") (Normal :type "Vector Structure") (`Hit Point Sound` :type "SoundBase Object Reference") (`Hit Point SFX` :type "ParticleSystem Object Reference"))
  (locals (`loc line trace damage` :type "Float (double-precision)") (`loc hit actor` :type "Actor Object Reference") (`loc blocing hit` :type Boolean) (`loc hit location` :type "Vector Structure") (HitNormal :type "Vector Structure") (`loc Hit Point Decal` :type "MaterialInterface Object Reference") (`loc Hit Point Sound` :type "SoundBase Object Reference") (`loc Hit Point SFX` :type "ParticleSystem Object Reference") (`FindedValidActor?` :type Boolean))
  (`GameplayStatics.PlaySoundAtLocation` `Hit Point Sound` `Hit Location` (struct) (`self.Weapon Sound Volume Multiplier`) 1.0 0.0 null null null)
  (`GameplayStatics.SpawnEmitterAtLocation` `Hit Point SFX` `Hit Location` (`KismetMathLibrary.MakeRotFromX` Normal)))

(fn `PlayReloadSound`
  (params (`Start Sound?` :type Boolean))
  (locals (Sound :type "SoundBase Object Reference"))
  (bind (_weaponshotsoundcue _main_reload_start_sound _main_reload_stop_sound) (`self.GetWeaponSoundWeaponProperties`))
  (if `Start Sound?`
    (set `local.Sound` _main_reload_start_sound)
    (else
      (set `local.Sound` _main_reload_stop_sound)))
  (`GameplayStatics.PlaySoundAtLocation` (`local.Sound`) (`Actor.K2_GetActorLocation` (`self.CurrentWeapon`)) (struct) (`self.Weapon Sound Volume Multiplier`) 1.0 0.0 null null null))

(fn `ReloadAmmoCalculation`
  (returns (`New Current Ammo In Clip` :type Integer) (`New Current Ammo Pull` :type Integer))
  (locals (AddAmmo :type Integer) (`Local Current Ammo Pull` :type Integer) (`Local Current Ammo In Clip` :type Integer))
  (bind (_currentammoinclip _currentammopull) (`self.GetWeaponCurrentAmmoState`))
  (set `local.AddAmmo` (- (`self.GetWeaponAmmoProperties`) (`self.GetWeaponCurrentAmmoState`)))
  (if (> (`local.AddAmmo`) (`.CurrentAmmoPull` (`self.GetWeaponCurrentAmmoState`)))
    (set `local.Local Current Ammo Pull` 0)
    (set `local.Local Current Ammo In Clip` (+ _currentammopull _currentammoinclip))
    (else
      (set `local.Local Current Ammo Pull` (- (`.CurrentAmmoPull` (`self.GetWeaponCurrentAmmoState`)) (`local.AddAmmo`)))
      (set `local.Local Current Ammo In Clip` (+ (`local.AddAmmo`) (`self.GetWeaponCurrentAmmoState`)))))
  (return (`local.Local Current Ammo In Clip`) (`local.Local Current Ammo Pull`)))

(fn `SetWeaponCurrentAmmoInClip`
  (params (CurrentAmmoInClip :type Integer))
  (bind _currentweapon (`self.CurrentWeapon`))
  (set `/Game/KoH/Blueprints/SimpleCharacterBase/SimpleWeaponSystem/Weapons/BP_BaseWeapon.CurrentAmmoState` (make `/Game/KoH/Blueprints/SimpleCharacterBase/SimpleWeaponSystem/WeaponProperties/STR_CurrentAmmoState` CurrentAmmoInClip (`.CurrentAmmoPull_164_4A5B94374165F68CA0BCBA9FB036E4F2` (break `/Game/KoH/Blueprints/SimpleCharacterBase/SimpleWeaponSystem/WeaponProperties/STR_CurrentAmmoState` (`/Game/KoH/Blueprints/SimpleCharacterBase/SimpleWeaponSystem/Weapons/BP_BaseWeapon.CurrentAmmoState` _currentweapon)))) _currentweapon)
  (return))

(fn `SetWeaponCurrentAmmoPull`
  (params (CurrentAmmoPull :type Integer))
  (bind _currentweapon (`self.CurrentWeapon`))
  (set `/Game/KoH/Blueprints/SimpleCharacterBase/SimpleWeaponSystem/Weapons/BP_BaseWeapon.CurrentAmmoState` (make `/Game/KoH/Blueprints/SimpleCharacterBase/SimpleWeaponSystem/WeaponProperties/STR_CurrentAmmoState` (`.CurrentAmmoInClip_165_1F7C1C124ECBAA81902442A78D34BF2B` (break `/Game/KoH/Blueprints/SimpleCharacterBase/SimpleWeaponSystem/WeaponProperties/STR_CurrentAmmoState` (`/Game/KoH/Blueprints/SimpleCharacterBase/SimpleWeaponSystem/Weapons/BP_BaseWeapon.CurrentAmmoState` _currentweapon))) CurrentAmmoPull) _currentweapon)
  (return))

(fn `ShootingLineTrace`
  (params (`Line Trace Start Point` :type "Vector Structure") (`Line Trace End Point` :type "Vector Structure") (`Damage Amount` :type "Float (double-precision)") (`Ignore Character Actor` :type "Actor Object Reference"))
  (returns (`Damage From Line Trace` :type "Float (double-precision)") (HitActor :type "Actor Object Reference") (BlockingHit :type Boolean) (`Hit Location` :type "Vector Structure") (Normal :type "Vector Structure"))
  (bind _outhit (`KismetSystemLibrary.LineTraceSingleForObjects` `Line Trace Start Point` `Line Trace End Point` (`self.Object Types`) false (`|MakeArray` `Ignore Character Actor`) "None" true (struct :`R` 1.0 :`A` 1.0) (struct :`G` 1.0 :`A` 1.0) 3.0))
  (bind (_bblockinghit _binitialoverlap _time _distance _location _impactpoint _normal _impactnormal _physmat _hitactor) (`GameplayStatics.BreakHitResult` _outhit))
  (return `Damage Amount` _hitactor _bblockinghit _location _normal))