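; First-person shooter character Blueprint that spawns its weapon on possession and drives first-person camera changes for aiming and crouching.
; After a short BeginPlay delay, it attaches the weapon to the first-person mesh when locally controlled, otherwise to the body mesh.
; The authority registers the weapon with the weapon system and binds aim and crouch updates.
; These call Client-prefixed events whose timelines blend FOV, arms position and camera height.
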(event `SpawnWeapon`
  (params (`Weapon Class` :type "Actor Class Reference"))
  ;[1 1 1] EVENT POSSESSED
  ;;[1 1 1] Spawn Weapon
  (bind _returnvalue (`|SpawnActorFromClass` `Weapon Class` (`SceneComponent.GetRelativeTransform` (`self.MeshFP`)) "AlwaysSpawn" "OverrideRootScale" null null))
  (bind _asbp_base_weapon (cast `/Game/KoH/Blueprints/SimpleCharacterBase/SimpleWeaponSystem/Weapons/BP_BaseWeapon` _returnvalue))
  (set `self.CurrentWeapon` _asbp_base_weapon))

(event `self.ReceivePossessed`
  (params (NewController :type "Controller Object Reference"))
  ;[1 1 1] EVENT POSSESSED
  (`self.SpawnWeapon` (`self.WeaponClass`)))

(event `self.ReceiveBeginPlay`
  (bind _currentweapon (`self.CurrentWeapon`))
  ;[1 1 1] BEGIN PLAY
  ;;[1 1 1] Wait for create weapon
  (`KismetSystemLibrary.Delay` 0.2)
  (`parent.ReceiveBeginPlay`)
  ;;[1 1 1] Attach weapon. Set Weapon in WS
  (`/Engine/EditorBlueprintResources/StandardMacros.IsValid` _currentweapon
    (:`Is Valid`
      (`self.K2_AttachToComponent` _currentweapon (`self.GetMeshToAttach`) "GunSocket" "SnapToTarget" "KeepRelative" "KeepRelative" true)
      (`/Engine/EditorBlueprintResources/ActorMacros.Switch Has Authority`
        (:`Authority`
          ;;[1 1 1] WS Trigger form Owner. SetCurrentWeapon
          (`/Game/KoH/Blueprints/SimpleCharacterBase/SimpleWeaponSystem/BP_SimpleWeaponSystem.SetCurrentWeapon` (`self.BP_SimpleWeaponSystem`) (`self.CurrentWeapon`))
          ;;[1 1 1] Bind On Update Aim State
          (add `self.UpdatedAimState` self (delegate `HandleUpdateAimState`))
          ;;[1 1 1] Bind on Update Crouch State
          (add `self.UpdateCrouchState` self (delegate `HandleUpdateCrouchState`)))))))

(event `HandleUpdateAimState` :!signature `self.UpdatedAimState`
  (params (`In Aim?` :type Boolean))
  ;[1 1 1] BEGIN PLAY
  ;;[1 1 1] Bind On Update Aim State
  (`self.ClientUpdateCameraState` `In Aim?`))

(event `HandleUpdateCrouchState` :!signature `self.UpdateCrouchState`
  (params (`In Crouch?` :type Boolean))
  ;[1 1 1] BEGIN PLAY
  ;;[1 1 1] Bind on Update Crouch State
  (`self.ClientUpdateCameraPosition` `In Crouch?`))

(event `ClientUpdateCameraState`
  (params (`In Aim?` :type Boolean))
  (bind _camerafovminizoom (`self.CameraFOVMinizoom`))
  (bind _camerafovdefault (`self.CameraFOVDefault`))
  ;[1 1 1] Update Camera Values
  ;;[1 1 1] Update FOV and mesh position
  (bind (_direction _newtrack_3) (`Timeline|CameraStateChange` :!via `PlayFromStart`)
    (:`Update`
      (if `In Aim?`
        ;;;[1 1 1] Fov
        (set `CameraComponent.FieldOfView` (`|EaseFunction` "Linear" _newtrack_3 _camerafovdefault _camerafovminizoom) (`self.Camera`))
        ;;;[1 1 1] Position
        (`SceneComponent.K2_SetRelativeLocationAndRotation` (`self.MeshFP`) (`|EaseFunction` "Linear" _newtrack_3 (`self.NOAim_Position`) (`self.Aim_Position`)) (struct :`Yaw` -90.0) false false)
        (else
          ;;;[1 1 1] Fov
          (set `CameraComponent.FieldOfView` (`|EaseFunction` "Linear" _newtrack_3 _camerafovminizoom _camerafovdefault) (`self.Camera`))
          ;;;[1 1 1] Position
          (`SceneComponent.K2_SetRelativeLocationAndRotation` (`self.MeshFP`) (`|EaseFunction` "Linear" _newtrack_3 (`self.Aim_Position`) (`self.NOAim_Position`)) (struct :`Yaw` -90.0) false false))))))

(event `ClientUpdateCameraPosition`
  (params (`In Crouch?` :type Boolean))
  ;[1 1 1] Update Camera Values
  ;;[1 1 1] ClientUpdateCameraPosition
  (bind (_direction _newtrack_3) (`Timeline|crouchPosition` :!via `PlayFromStart`)
    (:`Update`
      (if `In Crouch?`
        (`self.UpdateCamPos` _newtrack_3 70.0 10.0)
        (else
          (`self.UpdateCamPos` _newtrack_3 10.0 70.0))))))

(fn `GetMeshToAttach`
  (returns (Mesh :type "SkeletalMeshComponent Object Reference"))
  (return (select `bool` (`self.IsLocallyControlled`) :`false` (`self.Mesh`) :`true` (`self.MeshFP`))))

(fn `UpdateCamPos`
  (params (Alpha :type "Float (double-precision)") (A :type "Float (double-precision)") (B :type "Float (double-precision)"))
  (`SceneComponent.K2_SetRelativeLocation` (`self.Camera`) (`KismetMathLibrary.MakeVector` 0.0 0.0 (`|EaseFunction` "Linear" Alpha A B)) false false))

(fn `UserConstructionScript`
  (`parent.UserConstructionScript`))