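; Networked base shooter character with health, aim, crouch, sprint, shooting and reload states.
; Server events change states and multicast them, while BPSimpleWeaponSystem handles weapon actions and reports back through interface events.
; Server tick interpolates aim-offset pitch and yaw from control rotation.
; Damage passes a game-mode team check and reports hits to the attacker; death or PlayerState termination removes UI and destroys pawn and weapon.
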(event `TellAllToReloadWeaponStart`
  ;[1 1 1] RELOAD
  ;;[1 1 1] TellAllToReloadWeaponStart
  (set `self.In Reload ?` true))

(event `/Game/KoH/Blueprints/SimpleCharacterBase/SimpleWeaponSystem/BP_SimpleWeaponSystemInterface.WSMainReloadStart`
  ;[1 1 1] RELOAD
  ;;[1 1 1] WS Interface.  Reload Start
  (`self.TellAllToReloadWeaponStart`)
  (`self.ServerAimOff`)
  (`self.ServerShootingOff`))

(event `ServerReloadOn`
  ;[1 1 1] RELOAD
  ;;[1 1 1] WS Trigger form Owner. Reload
  (`/Game/KoH/Blueprints/SimpleCharacterBase/SimpleWeaponSystem/BP_SimpleWeaponSystem.Reload` (`self.BP_SimpleWeaponSystem`)))

(event `TellAllToReloadWeaponStop`
  ;[1 1 1] RELOAD
  ;;[1 1 1] TellAllToReloadWeaponStop
  (set `self.In Reload ?` false))

(event `/Game/KoH/Blueprints/SimpleCharacterBase/SimpleWeaponSystem/BP_SimpleWeaponSystemInterface.WSMainReloadStop`
  ;[1 1 1] RELOAD
  ;;[1 1 1] WS Interface.  Reload Stop
  (`self.TellAllToReloadWeaponStop`))

(event `self.ReceiveBeginPlay`
  ;[1 1 1] EVENT BEGIN PLAY
  ;;[1 1 1] Set current health
  (set `self.Current Health` (`self.Max Heath`))
  (`|ExecutionSequence`
    (:`then_0`
      ;;[1 1 1] Create UI from WS
      (`/Engine/EditorBlueprintResources/ActorMacros.Switch Has Authority`
        (:`Authority`
          (`/Engine/EditorBlueprintResources/StandardMacros.IsValid` (`self.BP_SimpleWeaponSystem`)
            (:`Is Valid`
              ;;;[1 1 1] WS Trigger form Owner. CreateWeaponSystemUI
              (`/Game/KoH/Blueprints/SimpleCharacterBase/SimpleWeaponSystem/BP_SimpleWeaponSystem.CreateWeaponSystemUI` (`self.BP_SimpleWeaponSystem`)))))))
    (:`then_1`
      ;;[1 1 1] Bind on event -Terminate Pawn
      (`/Engine/EditorBlueprintResources/StandardMacros.IsValid` (`self.GetController`)
        (:`Is Valid`
          (`/Engine/EditorBlueprintResources/StandardMacros.IsValid` (`Controller.PlayerState` (`self.GetController`))
            (:`Is Valid`
              (bind _asbp_ps_base (cast `/Game/KoH/Blueprints/GameModeBase/BP_PS_Base` (`Controller.PlayerState` (`self.GetController`))))
              (add `/Game/KoH/Blueprints/GameModeBase/BP_PS_Base.TriggerTerminatePawn` _asbp_ps_base (delegate `HandleTriggerTerminatePawn`)))))))))

(event `ServerShootingOn`
  ;[1 1 1] SHOOTING
  (`/Engine/EditorBlueprintResources/StandardMacros.IsValid` (`self.BP_SimpleWeaponSystem`)
    (:`Is Valid`
      ;;[1 1 1] WS Trigger form Owner. Start Shooting
      (`/Game/KoH/Blueprints/SimpleCharacterBase/SimpleWeaponSystem/BP_SimpleWeaponSystem.StartShooting` (`self.BP_SimpleWeaponSystem`)))))

(event `MulticastShootingOn`
  ;[1 1 1] SHOOTING
  ;;[1 1 1] MulticastShootingOn
  (set `self.In Shooting ?` true))

(event `HandleTriggerTerminatePawn`
  ;[1 1 1] EVENT BEGIN PLAY
  ;;[1 1 1] Bind on event -Terminate Pawn
  (`self.ClientRemoveUI`)
  (`self.ServerDeadStateOn`)
  (`/Game/KoH/Blueprints/SimpleCharacterBase/SimpleWeaponSystem/BP_SimpleWeaponSystem.StopShooting` (`self.BP_SimpleWeaponSystem`)))

(event `/Game/KoH/Blueprints/SimpleCharacterBase/SimpleWeaponSystem/BP_SimpleWeaponSystemInterface.WSStartShooting`
  ;[1 1 1] SHOOTING
  ;;[1 1 1] WS Interface. ShootingStart
  (`self.MulticastShootingOn`))

(event `ServerShootingOff`
  ;[1 1 1] SHOOTING
  (`/Engine/EditorBlueprintResources/StandardMacros.IsValid` (`self.BP_SimpleWeaponSystem`)
    (:`Is Valid`
      ;;[1 1 1] WS Trigger form Owner. Stop Shooting
      (`/Game/KoH/Blueprints/SimpleCharacterBase/SimpleWeaponSystem/BP_SimpleWeaponSystem.StopShooting` (`self.BP_SimpleWeaponSystem`)))))

(event `/Game/KoH/Blueprints/SimpleCharacterBase/SimpleWeaponSystem/BP_SimpleWeaponSystemInterface.WSStopShooting`
  ;[1 1 1] SHOOTING
  ;;[1 1 1] WS Interface. ShootingStop
  (`self.MulticastShootingOff`))

(event `MulticastShootingOff`
  ;[1 1 1] SHOOTING
  ;;[1 1 1] MulticastShootingOff
  (set `self.In Shooting ?` false))

(event `self.ReceiveTick`
  (params (DeltaSeconds :type "Float (single-precision)"))
  (bind (_returnvalue_x _returnvalue_y _returnvalue_z) (`KismetMathLibrary.BreakVector` (`self.GetVelocity`)))
  ;[1 1 1] EVENT TICK
  (set `self.Delta Time` DeltaSeconds)
  (set `self.In Jump ?` (> _returnvalue_z 0.0))
  ;;[1 1 1] update from server
  (`/Engine/EditorBlueprintResources/ActorMacros.Switch Has Authority`
    (:`Authority`
      ;;[1 1 1] Set Aim Off Set
      (set `self.Aim Pitch` (`KismetMathLibrary.ClampAngle` (.pitch (`KismetMathLibrary.RInterpTo` (`KismetMathLibrary.MakeRotator` 0.0 (`self.Aim Pitch`) (`self.Aim Yaw`)) (`KismetMathLibrary.NormalizedDeltaRotator` (`self.GetControlRotation`) (`self.K2_GetActorRotation`)) (`self.Delta Time`) 15.0)) -90.0 90.0))
      (set `self.Aim Yaw` (`KismetMathLibrary.ClampAngle` (.yaw (`KismetMathLibrary.RInterpTo` (`KismetMathLibrary.MakeRotator` 0.0 (`self.Aim Pitch`) (`self.Aim Yaw`)) (`KismetMathLibrary.NormalizedDeltaRotator` (`self.GetControlRotation`) (`self.K2_GetActorRotation`)) (`self.Delta Time`) 15.0)) -90.0 90.0)))))

(event `MulticastAimOn`
  ;[1 1 1] AIM
  ;;[1 1 1] MulticastAimOn
  (set `self.In AIM ?` true))

(event `ServerAimOn`
  ;[1 1 1] AIM
  ;;[1 1 1] ServerAimOn
  (`self.MulticastAimOn`)
  (bind _output_get (set `self.In AIM ?` true))
  (`self.UpdatedAimState` _output_get))

(event `MulticastAimOff`
  ;[1 1 1] AIM
  ;;[1 1 1] MulticastAimOff
  (set `self.In AIM ?` false))

(event `ServerAimOff`
  ;[1 1 1] AIM
  ;;[1 1 1] ServerAimOff
  (`self.MulticastAimOff`)
  (bind _output_get (set `self.In AIM ?` false))
  (`self.UpdatedAimState` _output_get))

(event `MulticastCrouchOn`
  ;[1 1 1] CROUCH
  ;;[1 1 1] MulticastCrouchOn
  (set `self.In Crouch ?` true)
  ;;[1 1 1] Set Speed
  (set `CharacterMovementComponent.MaxWalkSpeed` 300.0 (`self.CharacterMovement`)))

(event `ServerCrouchOn`
  ;[1 1 1] CROUCH
  ;;[1 1 1] ServerCrouchOn
  (if (`self.In Sprint ?`)
    (`self.ServerSprintOff`))
  (`self.MulticastCrouchOn`)
  (bind _output_get (set `self.In Crouch ?` true))
  (`self.UpdateCrouchState` _output_get))

(event `ServerCrouchOff`
  ;[1 1 1] CROUCH
  ;;[1 1 1] ServerCrouchOff
  (`self.MulticastCrouchOff`)
  (bind _output_get (set `self.In Crouch ?` false))
  (`self.UpdateCrouchState` _output_get))

(event `MulticastCrouchOff`
  ;[1 1 1] CROUCH
  ;;[1 1 1] MulticastCrouchOff
  (set `self.In Crouch ?` false)
  ;;[1 1 1] Set Speed
  (set `CharacterMovementComponent.MaxWalkSpeed` 500.0 (`self.CharacterMovement`)))

(event `ServerSprintOn`
  ;[1 1 1] SPRINT
  ;;[1 1 1] ServerSprintOn
  (if (`self.In Crouch ?`)
    (`self.ServerCrouchOff`))
  (`self.MulticastSprintOn`)
  (set `self.In Sprint ?` true)
  (`self.ServerShootingOff`))

(event `MulticastSprintOn`
  ;[1 1 1] SPRINT
  ;;[1 1 1] MulticastSprintOn
  (set `self.In Sprint ?` true)
  ;;[1 1 1] Set Speed
  (set `CharacterMovementComponent.MaxWalkSpeed` 700.0 (`self.CharacterMovement`)))

(event `ServerSprintOff`
  ;[1 1 1] SPRINT
  ;;[1 1 1] ServerSprintOff
  (`self.MulticastSprintOff`)
  (set `self.In Sprint ?` false))

(event `MulticastSprintOff`
  ;[1 1 1] SPRINT
  ;;[1 1 1] MulticastSprintOff
  (set `self.In Sprint ?` false)
  ;;[1 1 1] Set Speed
  (set `CharacterMovementComponent.MaxWalkSpeed` 500.0 (`self.CharacterMovement`)))

(event `self.ReceiveAnyDamage`
  (params (Damage :type "Float (single-precision)") (DamageType :type "DamageType Object Reference") (InstigatedBy :type "Controller Object Reference") (DamageCauser :type "Actor Object Reference"))
  (bind _returnvalue (- (`self.Current Health`) (`self.Taked Damage`)))
  ;[1 1 1] DAMAGE
  ;;[1 1 1] Check Team Before Damage
  (bind _asbp_gm_base (cast `/Game/KoH/Blueprints/GameModeBase/BP_GM_Base` (`GameplayStatics.GetGameMode`)))
  (bind _can_damage (`/Game/KoH/Blueprints/GameModeBase/BP_GM_Base.CheckTeamBeforeDamage` _asbp_gm_base self DamageCauser))
  (if _can_damage
    ;;[1 1 1] Apply damage logic
    (set `self.Taked Damage` Damage)
    (if (`self.Dead?`)
      _
      (elif (<= _returnvalue 0.0)
        (set `self.Current Health` 0.0)
        (set `self.Dead?` false)
        ;;[1 1 1] WS Trigger form Owner. Stop Shooting
        (`/Game/KoH/Blueprints/SimpleCharacterBase/SimpleWeaponSystem/BP_SimpleWeaponSystem.StopShooting` (`self.BP_SimpleWeaponSystem`))
        ;;[1 1 1] Dead State Trigger and Delete UI
        (`/Engine/EditorBlueprintResources/StandardMacros.DoOnce` false
          (:`Completed`
            (`self.ClientRemoveUI`)
            (`self.ServerDeadStateOn`)
            ;;[1 1 1] GAME MODE LOGIC
            (bind _asbp_gm_base_2 (cast `/Game/KoH/Blueprints/GameModeBase/BP_GM_Base` (`GameplayStatics.GetGameMode`)))
            (`/Game/KoH/Blueprints/GameModeBase/BP_GM_Base.PlayerDead` _asbp_gm_base_2 self DamageCauser)))
        (else
          (set `self.Current Health` _returnvalue)
          ;;[1 1 1] Event to damage causer
          (bind _asbp_simple_common_character (cast `/Game/KoH/Blueprints/SimpleCharacterBase/BP_SimpleCommonCharacter` DamageCauser))
          ;;;[1 1 1] WS Trigger form Owner. Get Hitted Actor Health
          (`/Game/KoH/Blueprints/SimpleCharacterBase/SimpleWeaponSystem/BP_SimpleWeaponSystem.GetHittedActorHealth` (`/Game/KoH/Blueprints/SimpleCharacterBase/BP_SimpleCommonCharacter.BP_SimpleWeaponSystem` _asbp_simple_common_character) (`self.Current Health`) (`self.Taked Damage`)))))))

(event `ServerDeadStateOn`
  ;[1 1 1] DEAD STATE
  (set `self.Dead?` false)
  (`KismetSystemLibrary.Delay` 0.2)
  (`self.K2_DestroyActor`)
  (`self.K2_DestroyActor` (`self.CurrentWeapon`))
  (`self.MulticastDeadStateOn`))

(event `MulticastDeadStateOn`
  ;[1 1 1] DEAD STATE
  (`/Engine/EditorBlueprintResources/StandardMacros.IsValid` (`self.CurrentWeapon`)
    (:`Is Valid`
      (`self.K2_DestroyActor` (`self.CurrentWeapon`)))))

(event `ClientRemoveUI`
  ;[1 1 1] ClientRemoveUI
  (`/Game/KoH/Blueprints/SimpleCharacterBase/SimpleWeaponSystem/BP_SimpleWeaponSystem.RemoveUI` (`self.BP_SimpleWeaponSystem`)))

(fn `IsLocalController`
  (returns (IsLocalControlled :type Boolean))
  (return (`self.IsLocallyControlled`)))

(fn `UserConstructionScript`)