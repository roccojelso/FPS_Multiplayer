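; Third-person shooter character base that spawns a weapon on possession and drives an over-the-shoulder camera.
; BeginPlay waits briefly, attaches the weapon to the mesh socket and, on authority, registers it with the weapon system and binds aim and crouch updates.
; Those updates call client-named events whose timelines blend spring arm length, socket offset and FOV for aiming, and spring arm height for crouching.
; GetAutoAimRotator returns a zero rotation.
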(event `SpawnWeapon`
  (params (`Weapon Class` :type "Actor Class Reference"))
  ;[1 1 1] EVENT POSSESSED
  ;;[1 1 1] Spawn Weapon
  (bind _returnvalue (`|SpawnActorFromClass` `Weapon Class` (`SceneComponent.GetRelativeTransform` (`self.Mesh`)) "AlwaysSpawn" "OverrideRootScale" null null))
  (bind _asbp_base_weapon (cast `/Game/KoH/Blueprints/SimpleCharacterBase/SimpleWeaponSystem/Weapons/BP_BaseWeapon` _returnvalue))
  (set `self.CurrentWeapon` _asbp_base_weapon))

(event `self.ReceivePossessed`
  (params (NewController :type "Controller Object Reference"))
  ;[1 1 1] EVENT POSSESSED
  (`self.SpawnWeapon` (`self.WeaponClass`)))

(event `self.ReceiveBeginPlay`
  (bind _currentweapon (`self.CurrentWeapon`))
  ;[1 1 1] BEGIN PLAY
  ;;[1 1 1] Wait for create weapon
  (`KismetSystemLibrary.Delay` 0.2)
  (`parent.ReceiveBeginPlay`)
  ;;[1 1 1] Attach weapon. Set Weapon in WS
  (`/Engine/EditorBlueprintResources/StandardMacros.IsValid` _currentweapon
    (:`Is Valid`
      (`self.K2_AttachToComponent` _currentweapon (`self.Mesh`) "GunSocket" "SnapToTarget" "KeepRelative" "KeepRelative" true)
      (`/Engine/EditorBlueprintResources/ActorMacros.Switch Has Authority`
        (:`Authority`
          ;;[1 1 1] WS Trigger form Owner. SetCurrentWeapon
          (`/Game/KoH/Blueprints/SimpleCharacterBase/SimpleWeaponSystem/BP_SimpleWeaponSystem.SetCurrentWeapon` (`self.BP_SimpleWeaponSystem`) (`self.CurrentWeapon`))
          ;;[1 1 1] Bind On Update Aim State
          (add `self.UpdatedAimState` self (delegate `HandleUpdateAimState`))
          ;;[1 1 1] Bind on Update Crouch State
          (add `self.UpdateCrouchState` self (delegate `HandleUpdateCrouchState`)))))))

(event `HandleUpdateAimState` :!signature `self.UpdatedAimState`
  (params (`In Aim?` :type Boolean))
  ;[1 1 1] BEGIN PLAY
  ;;[1 1 1] Bind On Update Aim State
  (`self.ClientUpdateCameraState` `In Aim?`))

(event `HandleUpdateCrouchState` :!signature `self.UpdateCrouchState`
  (params (`In Crouch?` :type Boolean))
  ;[1 1 1] BEGIN PLAY
  ;;[1 1 1] Bind on Update Crouch State
  (`self.ClientUpdateCameraPosition` `In Crouch?`))

(event `ClientUpdateCameraState`
  (params (`In Aim?` :type Boolean))
  ;[1 1 1] Update Camera
  ;;[1 1 1] Fov / Springarm lenght / SocketOffSet
  (bind (_direction _newtrack_3) (`Timeline|CameraStateChange` :!via `PlayFromStart`)
    (:`Update`
      (if `In Aim?`
        (`self.CameraUpdate` _newtrack_3 (`self.CameraArmLenghtDefault`) (`self.CameraArmLenghtAIM`) (`self.CameraSocketOffsetDefault`) (`self.CameraSocketOffsetAIM`) (`self.CameraFOVDefault`) (`self.CameraFOVAIM`))
        (else
          (`self.CameraUpdate` _newtrack_3 (`self.CameraArmLenghtAIM`) (`self.CameraArmLenghtDefault`) (`self.CameraSocketOffsetAIM`) (`self.CameraSocketOffsetDefault`) (`self.CameraFOVAIM`) (`self.CameraFOVDefault`)))))))

(event `ClientUpdateCameraPosition`
  (params (`In Crouch?` :type Boolean))
  ;[1 1 1] Update Camera
  ;;[1 1 1] ClientUpdateCameraPosition
  (bind (_direction _newtrack_3) (`Timeline|CrouchTransition` :!via `PlayFromStart`)
    (:`Update`
      (if `In Crouch?`
        (`self.UpdateCamPos` _newtrack_3 40.0 -10.0)
        (else
          (`self.UpdateCamPos` _newtrack_3 -10.0 40.0))))))

(fn `CameraUpdate`
  (params (Alpha :type "Float (double-precision)") (`Arm A` :type "Float (double-precision)") (`Arm B` :type "Float (double-precision)") (`Socket A` :type "Vector Structure") (`Socket B` :type "Vector Structure") (`FOV A` :type "Float (double-precision)") (`FOV B` :type "Float (double-precision)"))
  (set `SpringArmComponent.TargetArmLength` (`|EaseFunction` "Linear" Alpha `Arm A` `Arm B`) (`self.SpringArm`))
  (set `SpringArmComponent.SocketOffset` (`|EaseFunction` "Linear" Alpha `Socket A` `Socket B`) (`self.SpringArm`))
  (set `CameraComponent.FieldOfView` (`|EaseFunction` "Linear" Alpha `FOV A` `FOV B`) (`self.Camera`)))

(fn `GetAutoAimRotator`
  (returns (AutoAimRotator :type "Rotator Structure"))
  (return))

(fn `UpdateCamPos`
  (params (Alpha :type "Float (double-precision)") (`Pos A` :type "Float (double-precision)") (`Pos B` :type "Float (double-precision)"))
  (`SceneComponent.K2_SetRelativeLocation` (`self.SpringArm`) (`KismetMathLibrary.MakeVector` 0.0 0.0 (`|EaseFunction` "Linear" Alpha `Pos A` `Pos B`)) false false))

(fn `UserConstructionScript`
  (`parent.UserConstructionScript`))