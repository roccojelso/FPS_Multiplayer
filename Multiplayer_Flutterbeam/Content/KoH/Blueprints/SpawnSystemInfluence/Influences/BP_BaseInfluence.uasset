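; Base influence component for the spawn system, weighting nearby spawn points by its owner's team and influence type.
; A looping timer gathers spawn points overlapping an attached cylinder actor, clears its influence from those left behind and applies weights scaled by an optional horizontal-distance curve.
; Stopping or owner destruction removes its influence.
; A gated, delay-throttled Tick multicasts debug cylinders and labels according to the GameMode spawn component's flags.
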(event `self.ReceiveTick`
  (params (DeltaSeconds :type "Float (single-precision)"))
  (bind _returnvalue (`Actor.GetComponentByClass` (`GameplayStatics.GetGameMode`) "/Game/KoH/Blueprints/SpawnSystemInfluence/BP_GMC_InfluenceSpawnSystem.BP_GMC_InfluenceSpawnSystem_C"))
  ;[1 1 1] EVENT TICK
  ;;[1 1 1] Unlock gate for server only
  (`/Engine/EditorBlueprintResources/StandardMacros.Gate` true :!label _label
    (:`Exit`
      ;;[1 1 1] Special delay for performance. Draw debug text has same value of life time in function
      (`KismetSystemLibrary.Delay` 1.2)
      ;;[1 1 1] Condition
      (`/Engine/EditorBlueprintResources/StandardMacros.IsValid` _returnvalue
        (:`Is Valid`
          (if (`/Game/KoH/Blueprints/SpawnSystemInfluence/BP_GMC_InfluenceSpawnSystem.Debug Draw Influences` _returnvalue)
            (switch `/Game/KoH/Blueprints/SpawnSystemInfluence/Data/E_InfluenceType` (`self.Influence Type`)
              (:`NewEnumerator0`
                (if (`/Game/KoH/Blueprints/SpawnSystemInfluence/BP_GMC_InfluenceSpawnSystem.Debug Draw Enemy Forbid Influences` _returnvalue)
                  ;;[1 1 1] MulticastDrawDebugCylinderInfluence
                  (switch `/Game/KoH/Blueprints/SpawnSystemInfluence/Data/E_InfluenceShape` (`self.InfluenceShapeType`) :!label _label_2
                    (:`NewEnumerator0`
                      (`self.MulticastDrawDebugCylinderInfluence` (`self.CylinderHeight`) (`self.CylinderRadius`) (`self.Influence Type`) (`self.Team Type`) (`self.BaseGameModeInfType`))))))
              (:`NewEnumerator1`
                (if (`/Game/KoH/Blueprints/SpawnSystemInfluence/BP_GMC_InfluenceSpawnSystem.Debug Draw Ally Bias Influences` _returnvalue)
                  (goto _label_2)))
              (:`NewEnumerator2`
                (if (`/Game/KoH/Blueprints/SpawnSystemInfluence/BP_GMC_InfluenceSpawnSystem.Debug Draw DeadTeammate Influences` _returnvalue)
                  (goto _label_2)))
              (:`NewEnumerator3`
                (if (`/Game/KoH/Blueprints/SpawnSystemInfluence/BP_GMC_InfluenceSpawnSystem.Debug Draw GameMode Influences` _returnvalue)
                  (goto _label_2))))))))))

(event `UnlockEventTick`
  ;[1 1 1] EVENT TICK
  ;;[1 1 1] Unlock gate for server only
  ;;;[1 1 1] UnlockEventTick
  (goto _label :!via `Open`))

(event `MulticastDrawDebugCylinderInfluence`
  (params (CylinderHeight :type "Float (double-precision)") (CylinderRadius :type "Float (double-precision)") (InfluenceType :type "/Game/KoH/Blueprints/SpawnSystemInfluence/Data/E_InfluenceType Enum" :default "NewEnumerator0") (`Team Type` :type "/Game/KoH/Blueprints/SpawnSystemInfluence/Data/E_InfTeamType Enum" :default "NewEnumerator0") (`Game Mode Inf Type` :type "/Game/KoH/Blueprints/SpawnSystemInfluence/Data/E_GameModeInfType Enum" :default "NewEnumerator0"))
  ;[1 1 1] EVENT TICK
  ;;[1 1 1] MulticastDrawDebugCylinderInfluence
  (`self.DebugDrawCylinderInfluence` CylinderHeight CylinderRadius InfluenceType)
  (`self.DebugDrawInfluenceName` InfluenceType `Team Type` `Game Mode Inf Type`))

(event `StartInfluence`
  (bind _returnvalue (`Actor.GetComponentByClass` (`self.GetOwner`) "/Game/KoH/Blueprints/SpawnSystemInfluence/BP_InfTeamID.BP_InfTeamID_C"))
  ;[1 1 1] StartInfluence
  ;;[1 1 1] Waiting Owner Initialize on creating
  (`KismetSystemLibrary.Delay` 0.2)
  (`|ExecutionSequence`
    (:`then_0`
      (`KismetSystemLibrary.Delay` (`self.DelayForStartDebug`))
      ;;[1 1 1] UnlockEventTick
      (`self.UnlockEventTick`))
    (:`then_1`
      ;;[1 1 1] Get team type from character team indentificator
      (`/Engine/EditorBlueprintResources/StandardMacros.IsValid` _returnvalue
        (:`Is Valid`
          (`self.SetTeamType` (`/Game/KoH/Blueprints/SpawnSystemInfluence/BP_InfTeamID.GetTeam` _returnvalue))
          ;;[1 1 1] Start UpdateInfluence
          (`KismetSystemLibrary.K2_SetTimer` null "UpdateInfluence" (`self.TraceUpdatePeriod`) true)
          ;;[1 1 1] Bind on Even Owner Destroyed
          (add `Actor.OnDestroyed` (`self.GetOwner`) (delegate `OnDestroyed`)))))))

(event `OnDestroyed`
  (params (DestroyedActor :type "Actor Object Reference"))
  ;[1 1 1] StartInfluence
  ;;[1 1 1] Bind on Even Owner Destroyed
  (`self.StopInfluence`))

(event `StopInfluence`
  ;[1 1 1] StopInfluence
  ;;[1 1 1] Clear Timer for UpdateInfluence
  (`KismetSystemLibrary.K2_ClearTimer` null "UpdateInfluence")
  ;;[1 1 1] Remove influence from affected points
  (for _array_element (`self.MainInfluencedSpawnPoints`)
    (`/Game/KoH/Blueprints/SpawnSystemInfluence/BP_InfSpawnPoint.RemoveInfluencesOnPoint` _array_element (`KismetStringLibrary.Concat_StrStr` (`KismetSystemLibrary.GetObjectName` (`self.GetOwner`)) (`|GetEnumeratorNameAsString` (`self.Influence Type`)) (`|GetEnumeratorNameAsString` (`self.BaseGameModeInfType`))))))

(event `ReStartInfluence`
  (bind _returnvalue (`Actor.GetComponentByClass` (`self.GetOwner`) "/Game/KoH/Blueprints/SpawnSystemInfluence/BP_InfTeamID.BP_InfTeamID_C"))
  ;[1 1 1] ReStartInfluence
  ;;[1 1 1] Get team type from character team indentificator
  (`/Engine/EditorBlueprintResources/StandardMacros.IsValid` _returnvalue
    (:`Is Valid`
      (`self.SetTeamType` (`/Game/KoH/Blueprints/SpawnSystemInfluence/BP_InfTeamID.GetTeam` _returnvalue))
      ;;[1 1 1] Start UpdateInfluence
      (`KismetSystemLibrary.K2_SetTimer` null "UpdateInfluence" (`self.TraceUpdatePeriod`) true))))

(fn `CommonFormingSpawnPointsArray`
  (params (NewInfluencedSpawnPoints :type "Array of /Game/KoH/Blueprints/SpawnSystemInfluence/BP_InfSpawnPoint Object Reference"))
  ;[1 1 1] Cleal new spawn point array each trace period
  (`KismetArrayLibrary.Array_Clear` (`self.NewInfluencedSpawnPoints`))
  ;[1 1 1] Set New Spawn Point Array on trace period
  (set `self.NewInfluencedSpawnPoints` NewInfluencedSpawnPoints)
  (for _array_element (`self.MainInfluencedSpawnPoints`)
    ;[1 1 1] Remove influence from spawn point that are not contain on new spawn point array
    (if (not (`KismetArrayLibrary.Array_Contains` (`self.NewInfluencedSpawnPoints`) _array_element))
      (`/Game/KoH/Blueprints/SpawnSystemInfluence/BP_InfSpawnPoint.RemoveInfluencesOnPoint` _array_element (`KismetStringLibrary.Concat_StrStr` (`KismetSystemLibrary.GetObjectName` (`self.GetOwner`)) (`|GetEnumeratorNameAsString` (`self.Influence Type`)) (`|GetEnumeratorNameAsString` (`self.BaseGameModeInfType`))))))
  ;[1 1 1] Clear and initilize main spawn poinr array based on new array form trace
  (`KismetArrayLibrary.Array_Clear` (`self.MainInfluencedSpawnPoints`))
  (set `self.MainInfluencedSpawnPoints` (`self.NewInfluencedSpawnPoints`)))

(fn `CreateCylinderShape`
  (params (Radius :type "Float (double-precision)") (Height :type "Float (double-precision)"))
  (bind _returnvalue (* (/ (`self.CylinderRadius`) 100.0) 2.0))
  ;[1 1 1] Initialize basic properties
  (set `self.CylinderRadius` Radius)
  (set `self.CylinderHeight` Height)
  (set `self.InfluenceShapeType` "NewEnumerator0")
  ;[1 1 1] Spawn Cylinder Shape Actor
  (bind _returnvalue_2 (`|SpawnActorFromClass` "/Game/KoH/Blueprints/SpawnSystemInfluence/InfluencesShapes/BP_InfCylinderShape.BP_InfCylinderShape_C" (`Actor.GetTransform` (`self.GetOwner`)) "AlwaysSpawn" "OverrideRootScale" null null))
  (bind _output_get (set `self.InfluenceShape` _returnvalue_2))
  ;[1 1 1] Attach to owner
  (`/Engine/EditorBlueprintResources/StandardMacros.IsValid` _output_get
    (:`Is Valid`
      (`Actor.K2_AttachToActor` (`self.InfluenceShape`) (`self.GetOwner`) "None" "SnapToTarget" "KeepRelative" "SnapToTarget" true)
      ;[1 1 1] Set scale for shape
      (`SceneComponent.SetRelativeScale3D` (`/Game/KoH/Blueprints/SpawnSystemInfluence/InfluencesShapes/BP_InfCylinderShape.Cylinder` (`self.InfluenceShape`)) (`KismetMathLibrary.MakeVector` _returnvalue _returnvalue (/ (`self.CylinderHeight`) 100.0))))))

(fn `CylinderCalculationInfluence`
  (locals (loc_step_spawn_point :type "/Game/KoH/Blueprints/SpawnSystemInfluence/BP_InfSpawnPoint Object Reference") (loc_step_distance :type "Float (double-precision)") (loc_step_location_calc_point :type "Vector Structure" :default (0.0 0.0 0.0)) (loc_step_added_weight :type "Float (double-precision)" :default 0.0))
  (for _array_element (`self.MainInfluencedSpawnPoints`)
    (set `local.loc_step_spawn_point` _array_element)
    ;[1 1 1] loc_step_location_calc_point
    (set `local.loc_step_location_calc_point` (`KismetMathLibrary.MakeVector` (.x (`Actor.K2_GetActorLocation` (`local.loc_step_spawn_point`))) (.y (`Actor.K2_GetActorLocation` (`local.loc_step_spawn_point`))) (.z (`self.GetOwnerLocRot`))))
    ;[1 1 1] loc_step_distance
    (set `local.loc_step_distance` (`KismetMathLibrary.Vector_Distance` (`self.GetOwnerLocRot`) (`local.loc_step_location_calc_point`)))
    ;[1 1 1] loc_step_added_weight
    (`/Engine/EditorBlueprintResources/StandardMacros.IsValid` (`self.Distance Curve`)
      (:`Is Valid`
        (set `local.loc_step_added_weight` (* (`self.Influence Weight`) (`CurveFloat.GetFloatValue` (`self.Distance Curve`) (/ (/ (`local.loc_step_distance`) (/ (`self.CylinderRadius`) 100.0)) 100.0)))))
      (:`Is Not Valid`
        (set `local.loc_step_added_weight` (* (`self.Influence Weight`) 1.0))))
    ;[1 1 1] Add Influence on spawn point
    (`/Game/KoH/Blueprints/SpawnSystemInfluence/BP_InfSpawnPoint.AddInfluencesOnPoint` (`local.loc_step_spawn_point`) (`KismetStringLibrary.Concat_StrStr` (`KismetSystemLibrary.GetObjectName` (`self.GetOwner`)) (`|GetEnumeratorNameAsString` (`self.Influence Type`)) (`|GetEnumeratorNameAsString` (`self.BaseGameModeInfType`))) (`self.Influence Type`) (`self.Team Type`) (`local.loc_step_added_weight`) (`self.BaseGameModeInfType`))))

(fn `CylinderCreateTrace`
  (returns (`Initial Spawn Points Array` :type "Array of /Game/KoH/Blueprints/SpawnSystemInfluence/BP_InfSpawnPoint Object Reference"))
  (locals (loc_spawn_points :type "Array of /Game/KoH/Blueprints/SpawnSystemInfluence/BP_InfSpawnPoint Object Reference"))
  (bind _actor_location (`self.GetOwnerLocRot`))
  ;[1 1 1] Clear initial spawn point array each trace period
  (`KismetArrayLibrary.Array_Clear` (`local.loc_spawn_points`))
  ;[1 1 1] Creating Trace
  (bind _outhits (`KismetSystemLibrary.SphereTraceMultiForObjects` _actor_location _actor_location (`self.CylinderRadius`) (`|MakeArray` "ObjectTypeQuery2" :!type "EObjectTypeQuery Enum") false (`|MakeArray` null :!type "Actor Object Reference") "ForDuration" true (struct :`R` 1.0 :`A` 1.0) (struct :`G` 1.0 :`A` 1.0) (`self.TraceUpdatePeriod`)))
  ;[1 1 1] Forming initial spawn points array
  (for _array_element _outhits
    (bind (_bblockinghit _binitialoverlap _time _distance _location _impactpoint _normal _impactnormal _physmat _hitactor) (`GameplayStatics.BreakHitResult` _array_element))
    (if (== (`GameplayStatics.GetObjectClass` _hitactor) "/Game/KoH/Blueprints/SpawnSystemInfluence/BP_InfSpawnPoint.BP_InfSpawnPoint_C")
      (bind _asbp_inf_spawn_point (cast `/Game/KoH/Blueprints/SpawnSystemInfluence/BP_InfSpawnPoint` _hitactor))
      (`KismetArrayLibrary.Array_Add` (`local.loc_spawn_points`) _asbp_inf_spawn_point)))
  ;[1 1 1] Output
  (return (`local.loc_spawn_points`)))

(fn `DebugDrawCylinderInfluence`
  (params (CylinderHeight :type "Float (double-precision)") (CylinderRadius :type "Float (double-precision)") (InfluenceType :type "/Game/KoH/Blueprints/SpawnSystemInfluence/Data/E_InfluenceType Enum" :default "NewEnumerator0"))
  (bind _actor_location (`self.GetOwnerLocRot`))
  (bind _returnvalue (`KismetMathLibrary.MakeVector` (.x _actor_location) (.y _actor_location) (- (.z _actor_location) (/ CylinderHeight 2.0))))
  (bind _returnvalue_2 (`KismetMathLibrary.MakeVector` (.x _actor_location) (.y _actor_location) (+ (.z _actor_location) (/ CylinderHeight 2.0))))
  (switch `/Game/KoH/Blueprints/SpawnSystemInfluence/Data/E_InfluenceType` InfluenceType
    (:`NewEnumerator0`
      (`KismetSystemLibrary.DrawDebugCylinder` _returnvalue _returnvalue_2 CylinderRadius 30 (struct :`G` 1.0 :`B` 0.838407 :`A` 1.0) 1.2))
    (:`NewEnumerator1`
      (`KismetSystemLibrary.DrawDebugCylinder` _returnvalue _returnvalue_2 CylinderRadius 30 (struct :`R` 0.164169 :`G` 1.0 :`A` 1.0) 1.2))
    (:`NewEnumerator2`
      (`KismetSystemLibrary.DrawDebugCylinder` _returnvalue _returnvalue_2 CylinderRadius 30 (struct :`R` 1.0 :`G` 0.297505 :`A` 1.0) 1.2))
    (:`NewEnumerator3`
      (`KismetSystemLibrary.DrawDebugCylinder` _returnvalue _returnvalue_2 CylinderRadius 30 (struct :`R` 0.045916 :`B` 1.0 :`A` 1.0) 1.2))))

(fn `DebugDrawInfluenceName`
  (params (`Influence Type` :type "/Game/KoH/Blueprints/SpawnSystemInfluence/Data/E_InfluenceType Enum" :default "NewEnumerator0") (`Team Type` :type "/Game/KoH/Blueprints/SpawnSystemInfluence/Data/E_InfTeamType Enum" :default "NewEnumerator0") (`Game Mode Inf Type` :type "/Game/KoH/Blueprints/SpawnSystemInfluence/Data/E_GameModeInfType Enum" :default "NewEnumerator0"))
  (locals (loc_pos_z :type "Float (double-precision)"))
  (bind _returnvalue (`KismetStringLibrary.Concat_StrStr` (`|GetEnumeratorNameAsString` `Influence Type`) " from " (`|GetEnumeratorNameAsString` `Team Type`)))
  (bind _returnvalue_2 (`KismetMathLibrary.MakeVector` (.x (`self.GetOwnerLocRot`)) (.y (`self.GetOwnerLocRot`)) (+ (.z (`self.GetOwnerLocRot`)) (`local.loc_pos_z`))))
  (switch `/Game/KoH/Blueprints/SpawnSystemInfluence/Data/E_InfluenceType` `Influence Type`
    (:`NewEnumerator0`
      (set `local.loc_pos_z` 20.0)
      (`KismetSystemLibrary.DrawDebugString` _returnvalue_2 _returnvalue null (struct :`G` 1.0 :`B` 0.838407 :`A` 1.0) 1.2))
    (:`NewEnumerator1`
      (set `local.loc_pos_z` 40.0)
      (`KismetSystemLibrary.DrawDebugString` _returnvalue_2 _returnvalue null (struct :`R` 0.164169 :`G` 1.0 :`A` 1.0) 1.2))
    (:`NewEnumerator2`
      (set `local.loc_pos_z` 60.0)
      (`KismetSystemLibrary.DrawDebugString` _returnvalue_2 _returnvalue null (struct :`R` 1.0 :`G` 0.297505 :`A` 1.0) 1.2))
    (:`NewEnumerator3`
      (switch `/Game/KoH/Blueprints/SpawnSystemInfluence/Data/E_GameModeInfType` `Game Mode Inf Type`
        (:`NewEnumerator0`
          (set `local.loc_pos_z` 80.0))
        (:`NewEnumerator1`
          (set `local.loc_pos_z` 100.0))
        (:`NewEnumerator2`
          (set `local.loc_pos_z` 120.0)))
      (`KismetSystemLibrary.DrawDebugString` _returnvalue_2 _returnvalue null (struct :`R` 0.045916 :`B` 1.0 :`A` 1.0) 1.2))))

(fn `GetDebugSettings`
  (returns (`Debug Draw All Influences` :type Boolean) (`Debug Draw All Spawn Points` :type Boolean))
  (bind _returnvalue (`Actor.GetComponentByClass` (`GameplayStatics.GetGameMode`) "/Game/KoH/Blueprints/SpawnSystemInfluence/BP_GMC_InfluenceSpawnSystem.BP_GMC_InfluenceSpawnSystem_C"))
  (`/Engine/EditorBlueprintResources/StandardMacros.IsValid` _returnvalue
    (:`Is Valid`
      (return (`/Game/KoH/Blueprints/SpawnSystemInfluence/BP_GMC_InfluenceSpawnSystem.Debug Draw Influences` _returnvalue) (`/Game/KoH/Blueprints/SpawnSystemInfluence/BP_GMC_InfluenceSpawnSystem.Debug Draw Spawn Points` _returnvalue)))))

(fn `GetOverlappingSpawnPoints`
  (returns (`Initial Spawn Points Array` :type "Array of /Game/KoH/Blueprints/SpawnSystemInfluence/BP_InfSpawnPoint Object Reference"))
  (locals (loc_spawn_points :type "Array of /Game/KoH/Blueprints/SpawnSystemInfluence/BP_InfSpawnPoint Object Reference"))
  (bind _influenceshape (`self.InfluenceShape`))
  (`/Engine/EditorBlueprintResources/StandardMacros.IsValid` _influenceshape
    (:`Is Valid`
      (for _array_element (`PrimitiveComponent.GetOverlappingActors` (`/Game/KoH/Blueprints/SpawnSystemInfluence/InfluencesShapes/BP_InfCylinderShape.Cylinder` _influenceshape) "/Game/KoH/Blueprints/SpawnSystemInfluence/BP_InfSpawnPoint.BP_InfSpawnPoint_C")
        (bind _asbp_inf_spawn_point (cast `/Game/KoH/Blueprints/SpawnSystemInfluence/BP_InfSpawnPoint` _array_element))
        (`KismetArrayLibrary.Array_Add` (`local.loc_spawn_points`) _asbp_inf_spawn_point))
      (return (`local.loc_spawn_points`)))))

(fn `GetOwnerLocRot`
  (returns (`Actor Location` :type "Vector Structure"))
  (return (`Actor.K2_GetActorLocation` (`self.GetOwner`))))

(fn `GetTeamType`
  (returns (`Team Type` :type "/Game/KoH/Blueprints/SpawnSystemInfluence/Data/E_InfTeamType Enum"))
  (return (`self.Team Type`)))

(fn `SetBaseGameModeInfType`
  (params (BaseGameModeInfType :type "/Game/KoH/Blueprints/SpawnSystemInfluence/Data/E_GameModeInfType Enum" :default "NewEnumerator0"))
  (set `self.BaseGameModeInfType` BaseGameModeInfType))

(fn `SetTeamType`
  (params (`Team Type` :type "/Game/KoH/Blueprints/SpawnSystemInfluence/Data/E_InfTeamType Enum" :default "NewEnumerator0"))
  (set `self.Team Type` `Team Type`))

(fn `UpdateInfluence`
  ;[1 1 1] Check inf shape type. This values is initialized in Set Shape Functions
  (switch `/Game/KoH/Blueprints/SpawnSystemInfluence/Data/E_InfluenceShape` (`self.InfluenceShapeType`)
    (:`NewEnumerator0`
      ;[1 1 1] Cylinder Logics
      (bind _initial_spawn_points_array (`self.GetOverlappingSpawnPoints`))
      (`self.CommonFormingSpawnPointsArray` _initial_spawn_points_array)
      (`self.CylinderCalculationInfluence`))))