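; Influence-driven spawn point that scores itself for Team 1, Team 2 and Any team in the spawn system.
; A server timer folds registered enemy-forbid, ally-bias, dead-teammate and game-mode influences into those weights, adding base weight and random offset.
; Spawning a character flags a start point as used, or locks a common point for a cooldown.
; When the game mode's spawn component enables debug, the server multicasts weight or start-point labels.
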(event `self.ReceiveTick`
  (params (DeltaSeconds :type "Float (single-precision)"))
  (bind _returnvalue (`self.GetComponentByClass` (`GameplayStatics.GetGameMode`) "/Game/KoH/Blueprints/SpawnSystemInfluence/BP_GMC_InfluenceSpawnSystem.BP_GMC_InfluenceSpawnSystem_C"))
  ;[1 1 1] EVENT TICK
  ;;[1 1 1] Gate Logic
  (`/Engine/EditorBlueprintResources/StandardMacros.Gate` true :!label _label
    (:`Exit`
      ;;[1 1 1] Check server side
      (if (`KismetSystemLibrary.IsStandalone`)
        ;;[1 1 1] Special delay for performance. Draw debug text has same value of life time in function
        (`KismetSystemLibrary.Delay` 1.2 :!label _label_2)
        ;;[1 1 1] Condition
        (`/Engine/EditorBlueprintResources/StandardMacros.IsValid` _returnvalue
          (:`Is Valid`
            (if (`/Game/KoH/Blueprints/SpawnSystemInfluence/BP_GMC_InfluenceSpawnSystem.Debug Draw Spawn Points` _returnvalue)
              ;;[1 1 1] MulticastDrawSpawnPointInfo
              (`self.MulticastDrawSpawnPointInfo` (`self.K2_GetActorLocation`) (`self.Team1Weight`) (`self.Team2Weight`) (`self.AnyWeight`) (`self.IsLockSpawn?`) (`self.IsUsedForStartSpawn?`)))))
        (elif (`KismetSystemLibrary.IsServer`)
          (goto _label_2))))))

(event `MulticastDrawSpawnPointInfo`
  (params (`Point Location` :type "Vector Structure") (`Team 1 Weight` :type "Float (double-precision)") (`Team 2 Weight` :type "Float (double-precision)") (`Any Weight` :type "Float (double-precision)") (`Is Locked For Spawn?` :type Boolean) (`Is Used For Start Spawn?` :type Boolean))
  ;[1 1 1] EVENT TICK
  ;;[1 1 1] MulticastDrawSpawnPointInfo
  (`self.SpawnPointDebugInfo` `Point Location` `Team 1 Weight` `Team 2 Weight` `Any Weight` `Is Locked For Spawn?` `Is Used For Start Spawn?`))

(event `OpenEventTickGate`
  ;[1 1 1] EVENT TICK
  ;;[1 1 1] Gate Logic
  (goto _label :!via `Open`))

(event `self.ReceiveBeginPlay`
  ;[1 1 1] EVENT BEGIN PLAY
  ;;[1 1 1] Start UpdatePointWeight on Server
  (if (`KismetSystemLibrary.IsStandalone`)
    (`/Engine/EditorBlueprintResources/StandardMacros.DoOnce` false :!label _label_3
      (:`Completed`
        (`KismetSystemLibrary.K2_SetTimer` null "UpdatePointWeight" (`self.PointWeightUpdatePeriod`) true)
        (`|ExecutionSequence`
          (:`then_0`
            (`KismetSystemLibrary.Delay` (`self.DelayForStartDebug`))
            ;;[1 1 1] OpenEventTickGate
            (`self.OpenEventTickGate`))
          (:`then_1`
            ;;[1 1 1] If Base Weight == 0 // set 10 value. Point MUSH have weigth not equal 0
            (if (== (`self.Base Weight`) 0)
              (set `self.Base Weight` 10))))))
    (elif (`KismetSystemLibrary.IsServer`)
      (goto _label_3))))

(event `ServerCharacterSpawned`
  ;[1 1 1] ServerCharacterSpawned
  ;;[1 1 1] Start Point Cond
  (if (`self.Start Point `)
    ;;[1 1 1] Lock start point before finish rounde or match. Event finish math / round
    (set `self.IsUsedForStartSpawn?` true)
    (else
      ;;[1 1 1] Lock point on Spawn cooldown when character spawns on this point (for common spawn points)
      (set `self.IsLockSpawn?` true)
      (`KismetSystemLibrary.Delay` (`self.Spawn cooldown`))
      (set `self.IsLockSpawn?` false))))

(fn `AddInfluencesOnPoint`
  (params (`Owner Name` :type String) (`Influence Type` :type "/Game/KoH/Blueprints/SpawnSystemInfluence/Data/E_InfluenceType Enum" :default "NewEnumerator0") (`Team Type` :type "/Game/KoH/Blueprints/SpawnSystemInfluence/Data/E_InfTeamType Enum" :default "NewEnumerator0") (`Calculated Weight` :type "Float (double-precision)") (`Gamemode Inf Type` :type "/Game/KoH/Blueprints/SpawnSystemInfluence/Data/E_GameModeInfType Enum" :default "NewEnumerator0"))
  (locals (loc_step_owner_name :type String) (loc_step_inf_type :type "/Game/KoH/Blueprints/SpawnSystemInfluence/Data/E_InfluenceType Enum" :default "NewEnumerator0") (loc_step_inf_weight :type "Float (double-precision)") (loc_step_team_type :type "/Game/KoH/Blueprints/SpawnSystemInfluence/Data/E_InfTeamType Enum" :default "NewEnumerator0") (loc_gamemode_inf_type :type "/Game/KoH/Blueprints/SpawnSystemInfluence/Data/E_GameModeInfType Enum" :default "NewEnumerator0"))
  ;[1 1 1] Initialize inf properties
  (set `local.loc_step_owner_name` `Owner Name`)
  (set `local.loc_step_inf_type` `Influence Type`)
  (set `local.loc_step_inf_weight` `Calculated Weight`)
  (set `local.loc_step_team_type` `Team Type`)
  (set `local.loc_gamemode_inf_type` `Gamemode Inf Type`)
  ;[1 1 1] Add / Update Influence
  (if (`BlueprintMapLibrary.Map_Contains` (`self.Influence List`) (`local.loc_step_owner_name`))
    (`BlueprintMapLibrary.Map_Remove` (`self.Influence List`) (`local.loc_step_owner_name`)))
  (`BlueprintMapLibrary.Map_Add` (`self.Influence List`) (`local.loc_step_owner_name`) (make `/Game/KoH/Blueprints/SpawnSystemInfluence/Data/STR_InfluenceOnPointDesc` (`local.loc_step_inf_type`) (`local.loc_step_team_type`) (`local.loc_step_inf_weight`) (`local.loc_gamemode_inf_type`))))

(fn `GetAnyWeight`
  (returns (AnyWeight :type "Float (double-precision)"))
  (return (`self.AnyWeight`)))

(fn `GetIsLockSpawn`
  (returns (`IsLockSpawn?` :type Boolean))
  (return (`self.IsLockSpawn?`)))

(fn `GetIsUsedForStartSpawn?`
  (returns (`IsUsedForStartSpawn?` :type Boolean))
  (return (`self.IsUsedForStartSpawn?`)))

(fn `GetTeam1Weight`
  (returns (Team1Weight :type "Float (double-precision)"))
  (return (`self.Team1Weight`)))

(fn `GetTeam2Weight`
  (returns (Team2Weight :type "Float (double-precision)"))
  (return (`self.Team2Weight`)))

(fn `RemoveInfluencesOnPoint`
  (params (OwnerName :type String))
  (locals (loc_step_owner_name :type String))
  (set `local.loc_step_owner_name` OwnerName)
  (`BlueprintMapLibrary.Map_Remove` (`self.Influence List`) (`local.loc_step_owner_name`)))

(fn `SetIsUsedForStartSpawn?`
  (params (`IsUsedForStartSpawn?` :type Boolean))
  (set `self.IsUsedForStartSpawn?` `IsUsedForStartSpawn?`))

(fn `SpawnPointDebugInfo`
  (params (`Point Location` :type "Vector Structure") (`Team 1 Weight` :type "Float (double-precision)") (`Team 2 Weight` :type "Float (double-precision)") (`Any Weight` :type "Float (double-precision)") (`Is Locked For Spawn?` :type Boolean) (`Is Used For Start Spawn?` :type Boolean))
  (locals (loc_point_location :type "Vector Structure") (loc_team1 :type "Float (double-precision)") (loc_team2 :type "Float (double-precision)") (loc_update_delay :type "Float (double-precision)") (loc_any :type "Float (double-precision)") (`loc_Is Locked For Spawn?` :type Boolean) (`loc_Is Used For Start Spawn?` :type Boolean))
  ;[1 1 1] Initialize
  (set `local.loc_point_location` `Point Location`)
  (set `local.loc_team1` `Team 1 Weight`)
  (set `local.loc_team2` `Team 2 Weight`)
  (set `local.loc_any` `Any Weight`)
  (set `local.loc_update_delay` 0.0)
  (set `local.loc_Is Locked For Spawn?` `Is Locked For Spawn?`)
  (set `local.loc_Is Used For Start Spawn?` `Is Used For Start Spawn?`)
  ;[1 1 1] Location Sphere
  (`KismetSystemLibrary.DrawDebugSphere` (`local.loc_point_location`) 16.0 12 (struct :`R` 1.0 :`G` 1.0 :`B` 1.0 :`A` 1.0) 1.2)
  (if (`self.Start Point `)
    (switch `/Game/KoH/Blueprints/SpawnSystemInfluence/Data/E_InfTeamType` (`self.Team`)
      (:`NewEnumerator0`
        ;[1 1 1] Any:
        (`KismetSystemLibrary.DrawDebugString` (`KismetMathLibrary.MakeVector` (.x (`local.loc_point_location`)) (.y (`local.loc_point_location`)) (+ (.z (`local.loc_point_location`)) 70.0)) "START POINT - ANY" null (struct :`R` 1.0 :`G` 1.0 :`B` 1.0 :`A` 1.0) 1.2))
      (:`NewEnumerator1`
        ;[1 1 1] Team 1:
        (`KismetSystemLibrary.DrawDebugString` (`KismetMathLibrary.MakeVector` (.x (`local.loc_point_location`)) (.y (`local.loc_point_location`)) (+ (.z (`local.loc_point_location`)) 40.0)) "START POINT - TEAM 1" null (struct :`R` 1.0 :`B` 0.012991 :`A` 1.0) 1.2))
      (:`NewEnumerator2`
        ;[1 1 1] Team 2:
        (`KismetSystemLibrary.DrawDebugString` (`KismetMathLibrary.MakeVector` (.x (`local.loc_point_location`)) (.y (`local.loc_point_location`)) (+ (.z (`local.loc_point_location`)) 10.0)) "START POINT - TEAM 2" null (struct :`G` 0.097639 :`B` 1.0 :`A` 1.0) 1.2)))
    (elif (not (`local.loc_Is Locked For Spawn?`))
      ;[1 1 1] Any:
      (`KismetSystemLibrary.DrawDebugString` (`KismetMathLibrary.MakeVector` (.x (`local.loc_point_location`)) (.y (`local.loc_point_location`)) (+ (.z (`local.loc_point_location`)) 70.0)) (`KismetStringLibrary.Concat_StrStr` "Any:" (`KismetStringLibrary.Conv_DoubleToString` (`local.loc_any`))) null (struct :`R` 1.0 :`G` 1.0 :`B` 1.0 :`A` 1.0) 1.2)
      ;[1 1 1] Team 1:
      (`KismetSystemLibrary.DrawDebugString` (`KismetMathLibrary.MakeVector` (.x (`local.loc_point_location`)) (.y (`local.loc_point_location`)) (+ (.z (`local.loc_point_location`)) 40.0)) (`KismetStringLibrary.Concat_StrStr` "Team 1:" (`KismetStringLibrary.Conv_DoubleToString` (`local.loc_team1`))) null (struct :`R` 1.0 :`B` 0.012991 :`A` 1.0) 1.2)
      ;[1 1 1] Team 2:
      (`KismetSystemLibrary.DrawDebugString` (`KismetMathLibrary.MakeVector` (.x (`local.loc_point_location`)) (.y (`local.loc_point_location`)) (+ (.z (`local.loc_point_location`)) 10.0)) (`KismetStringLibrary.Concat_StrStr` "Team 2:" (`KismetStringLibrary.Conv_DoubleToString` (`local.loc_team2`))) null (struct :`G` 0.097639 :`B` 1.0 :`A` 1.0) 1.2))))

(fn `UpdatePointWeight`
  (locals (loc_inf_type :type "/Game/KoH/Blueprints/SpawnSystemInfluence/Data/E_InfluenceType Enum") (loc_team_type :type "/Game/KoH/Blueprints/SpawnSystemInfluence/Data/E_InfTeamType Enum") (loc_inf_Weight :type "Float (double-precision)") (pre_enemy_fobid_team1 :type "Float (double-precision)") (pre_enemy_fobid_team2 :type "Float (double-precision)") (pre_enemy_fobid_any :type "Float (double-precision)") (pre_ally_bias_team1 :type "Float (double-precision)") (pre_ally_bias_team2 :type "Float (double-precision)") (pre_dead_teammate_team1 :type "Float (double-precision)") (pre_dead_teammate_team2 :type "Float (double-precision)") (pre_dead_teammate_any :type "Float (double-precision)") (loc_gamemode_inf_type :type "/Game/KoH/Blueprints/SpawnSystemInfluence/Data/E_GameModeInfType Enum") (pre_gamemode_team1 :type "Float (double-precision)") (pre_gamemode_team2 :type "Float (double-precision)"))
  (bind _random_offset (`self.Random offset`))
  (bind _random_offset_2 (`self.Random offset`))
  (bind _random_offset_3 (`self.Random offset`))
  (bind _values (`BlueprintMapLibrary.Map_Values` (`self.Influence List`)))
  (for _array_element _values
    (bind (_influencetype _teamtype _calculatedweight _gamemodeinfluencetype) (break `/Game/KoH/Blueprints/SpawnSystemInfluence/Data/STR_InfluenceOnPointDesc` _array_element))
    (set `local.loc_inf_type` _influencetype)
    (set `local.loc_team_type` _teamtype)
    (set `local.loc_inf_Weight` _calculatedweight)
    (set `local.loc_gamemode_inf_type` _gamemodeinfluencetype)
    (switch `/Game/KoH/Blueprints/SpawnSystemInfluence/Data/E_InfluenceType` (`local.loc_inf_type`)
      (:`NewEnumerator0`
        ;[1 1 1] ENEMY FORBID
        (switch `/Game/KoH/Blueprints/SpawnSystemInfluence/Data/E_InfTeamType` (`local.loc_team_type`)
          (:`NewEnumerator0`
            ;;[1 1 1] if any ===>> negative for any
            (if (or (> (`local.loc_inf_Weight`) (`local.pre_enemy_fobid_any`)) (< (`local.loc_inf_Weight`) (`local.pre_enemy_fobid_any`)))
              (set `local.pre_enemy_fobid_any` (`local.loc_inf_Weight`))
              (else
                (set `local.pre_enemy_fobid_any` (`local.pre_enemy_fobid_any`)))))
          (:`NewEnumerator1`
            ;;[1 1 1] if team 1 ===>> vers. team 2 negative
            (if (or (> (`local.loc_inf_Weight`) (`local.pre_enemy_fobid_team2`)) (< (`local.loc_inf_Weight`) (`local.pre_enemy_fobid_team2`)))
              (set `local.pre_enemy_fobid_team2` (`local.loc_inf_Weight`))
              (else
                (set `local.pre_enemy_fobid_team2` (`local.pre_enemy_fobid_team2`)))))
          (:`NewEnumerator2`
            ;;[1 1 1] if team 2 ===>> vers. team 1 negative
            (if (or (> (`local.loc_inf_Weight`) (`local.pre_enemy_fobid_team1`)) (< (`local.loc_inf_Weight`) (`local.pre_enemy_fobid_team1`)))
              (set `local.pre_enemy_fobid_team1` (`local.loc_inf_Weight`))
              (else
                (set `local.pre_enemy_fobid_team1` (`local.pre_enemy_fobid_team1`)))))))
      (:`NewEnumerator1`
        ;[1 1 1] ALLY BIAS
        (switch `/Game/KoH/Blueprints/SpawnSystemInfluence/Data/E_InfTeamType` (`local.loc_team_type`)
          (:`NewEnumerator1`
            ;;[1 1 1] if team 1 ===>> to team 1 positive
            (if (or (> (`local.loc_inf_Weight`) (`local.pre_ally_bias_team1`)) (< (`local.loc_inf_Weight`) (`local.pre_ally_bias_team1`)))
              (set `local.pre_ally_bias_team1` (`local.loc_inf_Weight`))
              (else
                (set `local.pre_ally_bias_team1` (`local.pre_ally_bias_team1`)))))
          (:`NewEnumerator2`
            ;;[1 1 1] if team 2 ===>> to team 2 positive
            (if (or (> (`local.loc_inf_Weight`) (`local.pre_ally_bias_team2`)) (< (`local.loc_inf_Weight`) (`local.pre_ally_bias_team2`)))
              (set `local.pre_ally_bias_team2` (`local.loc_inf_Weight`))
              (else
                (set `local.pre_ally_bias_team2` (`local.pre_ally_bias_team2`)))))))
      (:`NewEnumerator2`
        ;[1 1 1] DEAD TEAMMATE
        (switch `/Game/KoH/Blueprints/SpawnSystemInfluence/Data/E_InfTeamType` (`local.loc_team_type`)
          (:`NewEnumerator0`
            ;;[1 1 1] if any ===>> negative for any
            (if (or (> (`local.loc_inf_Weight`) (`local.pre_dead_teammate_any`)) (< (`local.loc_inf_Weight`) (`local.pre_dead_teammate_any`)))
              (set `local.pre_dead_teammate_any` (`local.loc_inf_Weight`))
              (else
                (set `local.pre_dead_teammate_any` (`local.pre_dead_teammate_any`)))))
          (:`NewEnumerator1`
            ;;[1 1 1] if team 1 ===>> negative for team 1
            (if (or (> (`local.loc_inf_Weight`) (`local.pre_dead_teammate_team1`)) (< (`local.loc_inf_Weight`) (`local.pre_dead_teammate_team1`)))
              (set `local.pre_dead_teammate_team1` (`local.loc_inf_Weight`))
              (else
                (set `local.pre_dead_teammate_team1` (`local.pre_dead_teammate_team1`)))))
          (:`NewEnumerator2`
            ;;[1 1 1] if team 2 ===>> negative for team 2
            (if (or (> (`local.loc_inf_Weight`) (`local.pre_dead_teammate_team2`)) (< (`local.loc_inf_Weight`) (`local.pre_dead_teammate_team2`)))
              (set `local.pre_dead_teammate_team2` (`local.loc_inf_Weight`))
              (else
                (set `local.pre_dead_teammate_team2` (`local.pre_dead_teammate_team2`)))))))
      (:`NewEnumerator3`
        ;[1 1 1] GAMEMODE
        (switch `/Game/KoH/Blueprints/SpawnSystemInfluence/Data/E_InfTeamType` (`local.loc_team_type`)
          (:`NewEnumerator1`
            (switch `/Game/KoH/Blueprints/SpawnSystemInfluence/Data/E_GameModeInfType` (`local.loc_gamemode_inf_type`)
              (:`NewEnumerator0`
                ;;[1 1 1] if team 1 ===>> to team 1 positive
                (if (or (> (`local.loc_inf_Weight`) (`local.pre_gamemode_team1`)) (< (`local.loc_inf_Weight`) (`local.pre_gamemode_team1`)))
                  (set `local.pre_gamemode_team1` (`local.loc_inf_Weight`))
                  (else
                    (set `local.pre_gamemode_team1` (`local.pre_gamemode_team1`)))))
              (:`NewEnumerator1`
                ;;[1 1 1] if team 1 ===>> vers. team 2 negative
                (if (or (> (`local.loc_inf_Weight`) (`local.pre_gamemode_team2`)) (< (`local.loc_inf_Weight`) (`local.pre_gamemode_team2`)))
                  (set `local.pre_gamemode_team2` (* (`local.loc_inf_Weight`) -1.0))
                  (else
                    (set `local.pre_gamemode_team2` (* (`local.pre_gamemode_team2`) -1.0)))))
              (:`NewEnumerator2`
                ;;[1 1 1] if team 1 ===>> to team 1 negative
                (if (or (> (`local.loc_inf_Weight`) (`local.pre_gamemode_team1`)) (< (`local.loc_inf_Weight`) (`local.pre_gamemode_team1`))) :!label _label
                  (set `local.pre_gamemode_team1` (* (`local.loc_inf_Weight`) -1.0))
                  ;;[1 1 1] if team 1 ===>> vers. team 2 negative
                  (if (or (> (`local.loc_inf_Weight`) (`local.pre_gamemode_team2`)) (< (`local.loc_inf_Weight`) (`local.pre_gamemode_team2`)))
                    (set `local.pre_gamemode_team2` (* (`local.loc_inf_Weight`) -1.0))
                    (else
                      (set `local.pre_gamemode_team2` (* (`local.pre_gamemode_team2`) -1.0))))
                  (else
                    (set `local.pre_gamemode_team1` (* (`local.pre_gamemode_team1`) -1.0)))))))
          (:`NewEnumerator2`
            (switch `/Game/KoH/Blueprints/SpawnSystemInfluence/Data/E_GameModeInfType` (`local.loc_gamemode_inf_type`)
              (:`NewEnumerator0`
                ;;[1 1 1] if team 2 ===>> to team 2 positive
                (if (or (> (`local.loc_inf_Weight`) (`local.pre_gamemode_team2`)) (< (`local.loc_inf_Weight`) (`local.pre_gamemode_team2`)))
                  (set `local.pre_gamemode_team2` (`local.loc_inf_Weight`))
                  (else
                    (set `local.pre_gamemode_team2` (`local.pre_gamemode_team2`)))))
              (:`NewEnumerator1`
                ;;[1 1 1] if team 2 ===>> to team 1 negative
                (if (or (> (`local.loc_inf_Weight`) (`local.pre_gamemode_team1`)) (< (`local.loc_inf_Weight`) (`local.pre_gamemode_team1`)))
                  (set `local.pre_gamemode_team1` (* (`local.loc_inf_Weight`) -1.0))
                  (else
                    (set `local.pre_gamemode_team1` (* (`local.pre_gamemode_team1`) -1.0)))))
              (:`NewEnumerator2`
                (goto _label))))))))
  (`|ExecutionSequence`
    (:`then_0`
      ;[1 1 1] Team1Weight
      (set `self.Team1Weight` (+ (* (`local.pre_enemy_fobid_team1`) -1.0) (`local.pre_ally_bias_team1`) (`KismetMathLibrary.Conv_IntToDouble` (`self.Base Weight`)) (`KismetMathLibrary.RandomFloatInRange` (`KismetMathLibrary.Conv_IntToDouble` (`.Value` (break `Int32RangeBound` (break `Int32Range` _random_offset)))) (`KismetMathLibrary.Conv_IntToDouble` (`.Value` (break `Int32RangeBound` (`.UpperBound` (break `Int32Range` _random_offset)))))) (* (`local.pre_dead_teammate_team1`) -1.0) (`local.pre_gamemode_team1`))))
    (:`then_1`
      ;[1 1 1] Team2Weight
      (set `self.Team2Weight` (+ (* (`local.pre_enemy_fobid_team2`) -1.0) (`local.pre_ally_bias_team2`) (`KismetMathLibrary.Conv_IntToDouble` (`self.Base Weight`)) (`KismetMathLibrary.RandomFloatInRange` (`KismetMathLibrary.Conv_IntToDouble` (`.Value` (break `Int32RangeBound` (break `Int32Range` _random_offset_3)))) (`KismetMathLibrary.Conv_IntToDouble` (`.Value` (break `Int32RangeBound` (`.UpperBound` (break `Int32Range` _random_offset_3)))))) (* (`local.pre_dead_teammate_team2`) -1.0) (`local.pre_gamemode_team2`))))
    (:`then_2`
      ;[1 1 1] AnyWeight
      (set `self.AnyWeight` (+ (* (`local.pre_enemy_fobid_any`) -1.0) (`KismetMathLibrary.Conv_IntToDouble` (`self.Base Weight`)) (`KismetMathLibrary.RandomFloatInRange` (`KismetMathLibrary.Conv_IntToDouble` (`.Value` (break `Int32RangeBound` (break `Int32Range` _random_offset_2)))) (`KismetMathLibrary.Conv_IntToDouble` (`.Value` (break `Int32RangeBound` (`.UpperBound` (break `Int32Range` _random_offset_2)))))) (* (`local.pre_dead_teammate_any`) -1.0))))))

(fn `UserConstructionScript`)