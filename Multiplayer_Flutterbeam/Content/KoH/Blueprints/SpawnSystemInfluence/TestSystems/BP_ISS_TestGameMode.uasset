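; Test game mode for the Influence Spawn System (ISS) that spawns, possesses and assigns teams to test characters.
; After a startup delay it gives each PlayerArray controller a start spawn point, alternating two teams via FlipFlop or using one deathmatch team.
; Team IDs are set on both character and controller.
; CharacterRespawn waits RespawnTime, then on authority spawns at the system's best common point for the controller's stored team.
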(event `self.ReceiveBeginPlay`
  ;[1 1 1] EVENT BEGIN PLAY
  ;;[1 1 1] Special Waiting for initialize other logics
  (`KismetSystemLibrary.Delay` 4.0)
  ;;[1 1 1] Initial Spawn Characters
  (`self.InitialSpawn`))

(event `InitialSpawn`
  ;[1 1 1] Initial Spawn
  ;;[1 1 1] Get Player Array from Game State and get from player item player contrroller for possesing on spawn
  (for _array_element (`GameStateBase.PlayerArray` (`GameplayStatics.GetGameState`))
    (bind _asplayer_controller (cast `PlayerController` (`self.GetOwner` _array_element)))
    (set `self.PlayerController` _asplayer_controller)
    ;;[1 1 1] Team Base Option Checking
    (if (`self.TestTeamBaseMode?`)
      ;;[1 1 1] TEAM BASED
      ;;;[1 1 1] Divide into two teams
      (`/Engine/EditorBlueprintResources/StandardMacros.FlipFlop`
        (:`A`
          ;;;[1 1 1] ISS - Get Start Spawn Point Transform
          (bind _sp_transform (`/Game/KoH/Blueprints/SpawnSystemInfluence/BP_GMC_InfluenceSpawnSystem.GetStartSpawnPointTransform ` (`self.BP_InfluenceSpawnSystem`) "NewEnumerator1"))
          ;;;[1 1 1] Spawn & Posses
          (bind _returnvalue (`|SpawnActorFromClass` "/Game/KoH/Blueprints/SpawnSystemInfluence/TestSystems/BP_ISS_TestCharacter.BP_ISS_TestCharacter_C" _sp_transform "AlwaysSpawn" "OverrideRootScale" null null))
          (`/Engine/EditorBlueprintResources/StandardMacros.IsValid` _returnvalue
            (:`Is Valid`
              (`Controller.Possess` (`self.PlayerController`) _returnvalue)
              ;;;[1 1 1] ISS - Server Initialise Team on Character
              (`/Game/KoH/Blueprints/SpawnSystemInfluence/BP_InfTeamID.ServerInitializeTeam` (`/Game/KoH/Blueprints/SpawnSystemInfluence/TestSystems/BP_ISS_TestCharacter.BP_ISS_TeamID` _returnvalue) "NewEnumerator1")
              ;;;[1 1 1] ISS - Server Initialize Team on Player Controller
              (`/Game/KoH/Blueprints/SpawnSystemInfluence/BP_InfTeamID.ServerInitializeTeam` (`self.GetComponentByClass` (`self.PlayerController`) "/Game/KoH/Blueprints/SpawnSystemInfluence/BP_InfTeamID.BP_InfTeamID_C") "NewEnumerator1"))))
        (:`B`
          ;;;[1 1 1] ISS - Get Start Spawn Point Transform
          (bind _sp_transform_2 (`/Game/KoH/Blueprints/SpawnSystemInfluence/BP_GMC_InfluenceSpawnSystem.GetStartSpawnPointTransform ` (`self.BP_InfluenceSpawnSystem`) "NewEnumerator2"))
          ;;;[1 1 1] Spawn & Posses
          (bind _returnvalue_2 (`|SpawnActorFromClass` "/Game/KoH/Blueprints/SpawnSystemInfluence/TestSystems/BP_ISS_TestCharacter.BP_ISS_TestCharacter_C" _sp_transform_2 "AlwaysSpawn" "OverrideRootScale" null null))
          (`/Engine/EditorBlueprintResources/StandardMacros.IsValid` _returnvalue_2
            (:`Is Valid`
              (`Controller.Possess` (`self.PlayerController`) _returnvalue_2)
              ;;;[1 1 1] ISS - Server Initialise Team on Character
              (`/Game/KoH/Blueprints/SpawnSystemInfluence/BP_InfTeamID.ServerInitializeTeam` (`/Game/KoH/Blueprints/SpawnSystemInfluence/TestSystems/BP_ISS_TestCharacter.BP_ISS_TeamID` _returnvalue_2) "NewEnumerator2")
              ;;;[1 1 1] ISS - Server Initialize Team on Player Controller
              (`/Game/KoH/Blueprints/SpawnSystemInfluence/BP_InfTeamID.ServerInitializeTeam` (`self.GetComponentByClass` (`self.PlayerController`) "/Game/KoH/Blueprints/SpawnSystemInfluence/BP_InfTeamID.BP_InfTeamID_C") "NewEnumerator2")))))
      (else
        ;;[1 1 1] DM
        ;;;[1 1 1] ISS - Get Start Spawn Point Transform
        (bind _sp_transform_3 (`/Game/KoH/Blueprints/SpawnSystemInfluence/BP_GMC_InfluenceSpawnSystem.GetStartSpawnPointTransform ` (`self.BP_InfluenceSpawnSystem`) "NewEnumerator0"))
        ;;;[1 1 1] Spawn & Posses
        (bind _returnvalue_3 (`|SpawnActorFromClass` "/Game/KoH/Blueprints/SpawnSystemInfluence/TestSystems/BP_ISS_TestCharacter.BP_ISS_TestCharacter_C" _sp_transform_3 "AlwaysSpawn" "OverrideRootScale" null null))
        (`/Engine/EditorBlueprintResources/StandardMacros.IsValid` _returnvalue_3
          (:`Is Valid`
            (`Controller.Possess` (`self.PlayerController`) _returnvalue_3)
            ;;;[1 1 1] ISS - Server Initialise Team on Character
            (`/Game/KoH/Blueprints/SpawnSystemInfluence/BP_InfTeamID.ServerInitializeTeam` (`/Game/KoH/Blueprints/SpawnSystemInfluence/TestSystems/BP_ISS_TestCharacter.BP_ISS_TeamID` _returnvalue_3) "NewEnumerator0")
            ;;;[1 1 1] ISS - Server Initialize Team on Player Controller
            (`/Game/KoH/Blueprints/SpawnSystemInfluence/BP_InfTeamID.ServerInitializeTeam` (`self.GetComponentByClass` (`self.PlayerController`) "/Game/KoH/Blueprints/SpawnSystemInfluence/BP_InfTeamID.BP_InfTeamID_C") "NewEnumerator0")))))))

(event `CharacterRespawn`
  (params (`Player Controller` :type "PlayerController Object Reference") (ControllerOnRespawn :type "Controller Object Reference"))
  ;[1 1 1] RESPAWN
  ;;[1 1 1] Initialize & Validation & Respawn Delay & Authority Side
  (set `self.PlayerControllerOnRespawn` `Player Controller`)
  (set `self.ControllerOnRespawn` ControllerOnRespawn)
  (`/Engine/EditorBlueprintResources/StandardMacros.IsValid` (`self.PlayerControllerOnRespawn`)
    (:`Is Valid`
      (`KismetSystemLibrary.Delay` (`self.RespawnTime`))
      (`/Engine/EditorBlueprintResources/ActorMacros.Switch Has Authority`
        (:`Authority`
          ;;[1 1 1] ISS - Get The Best Common Spawn point for respawn
          (bind _best_point_transform (`/Game/KoH/Blueprints/SpawnSystemInfluence/BP_GMC_InfluenceSpawnSystem.GetBestCommonSpawnPointTransform` (`self.BP_InfluenceSpawnSystem`) (`/Game/KoH/Blueprints/SpawnSystemInfluence/BP_InfTeamID.GetTeam` (`self.GetComponentByClass` (`self.ControllerOnRespawn`) "/Game/KoH/Blueprints/SpawnSystemInfluence/BP_InfTeamID.BP_InfTeamID_C"))))
          ;;[1 1 1] Spawn
          (bind _returnvalue (`|SpawnActorFromClass` "/Game/KoH/Blueprints/SpawnSystemInfluence/TestSystems/BP_ISS_TestCharacter.BP_ISS_TestCharacter_C" _best_point_transform "AlwaysSpawn" "OverrideRootScale" null null))
          (`/Engine/EditorBlueprintResources/StandardMacros.IsValid` _returnvalue
            (:`Is Valid`
              (`Controller.Possess` (`self.ControllerOnRespawn`) _returnvalue)
              ;;[1 1 1] ISS - Server Initialise Team on Character
              (`/Game/KoH/Blueprints/SpawnSystemInfluence/BP_InfTeamID.ServerInitializeTeam` (`/Game/KoH/Blueprints/SpawnSystemInfluence/TestSystems/BP_ISS_TestCharacter.BP_ISS_TeamID` _returnvalue) (`/Game/KoH/Blueprints/SpawnSystemInfluence/BP_InfTeamID.GetTeam` (`self.GetComponentByClass` (`self.ControllerOnRespawn`) "/Game/KoH/Blueprints/SpawnSystemInfluence/BP_InfTeamID.BP_InfTeamID_C"))))))))))

(fn `UserConstructionScript`)