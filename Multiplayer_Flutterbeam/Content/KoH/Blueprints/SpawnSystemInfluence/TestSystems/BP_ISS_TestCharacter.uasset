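; BP_ISS_TestCharacter is a test character for the influence spawn system that simulates player death and respawn.
; ServerTestDeath has the dead-teammate spawner place an influence actor at the character's transform, then asks BP_ISS_TestPlayerController to respawn the player.
; After a short delay it calls MulticastTestDeath to destroy the character, a step skipped if either controller cast fails.
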(event `ServerTestDeath`
  (bind _returnvalue (`self.GetController` self))
  ;[1 1 1] TEST DEATH LOGIC
  ;;[1 1 1] ServerTestDeath
  ;;;[1 1 1] Spawm Dead Teammate Influence from spawner
  (`/Game/KoH/Blueprints/SpawnSystemInfluence/Influences/BP_DeamTeammateSpawner.SpawnDeadTeammateInfActor` (`self.BP_ISS_DeamTeammateSpawner`) (`self.GetTransform`))
  ;;;[1 1 1] Controller Logic
  (bind _asplayer_controller (cast `PlayerController` _returnvalue))
  (bind _asbp_iss_test_player_controller (cast `/Game/KoH/Blueprints/SpawnSystemInfluence/TestSystems/BP_ISS_TestPlayerController` _asplayer_controller))
  (`/Game/KoH/Blueprints/SpawnSystemInfluence/TestSystems/BP_ISS_TestPlayerController.RespawnPlayerCharacter` _asbp_iss_test_player_controller _asplayer_controller _returnvalue)
  ;;;[1 1 1] MulticastTestDeath after delay
  (`KismetSystemLibrary.Delay` 0.2)
  (`self.MulticastTestDeath`))

(event `MulticastTestDeath`
  ;[1 1 1] TEST DEATH LOGIC
  ;;[1 1 1] MulticastTestDeath
  (`self.K2_DestroyActor`))

(fn `UserConstructionScript`)