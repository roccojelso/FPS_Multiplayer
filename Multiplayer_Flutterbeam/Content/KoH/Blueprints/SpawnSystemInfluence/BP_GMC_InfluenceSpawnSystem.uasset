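; Influence-based spawn system (GMC) that picks player spawn transforms per team from the level's BP_InfSpawnPoint actors.
; On standalone or server BeginPlay it sorts them into per-team start arrays and one common array.
; Start spawns take the first unused team point; finding none triggers a delayed reset of used points for the next round.
; Common spawns take the highest team-weighted unlocked point, notify it, and optionally log candidate weights.
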(event `self.ReceiveBeginPlay`
  ;[1 1 1] EVENT BEGIN PLAY
  ;;[1 1 1] Check server side (didec or listen)
  (if (`KismetSystemLibrary.IsStandalone`)
    ;;[1 1 1] Initialize Spawn Points Arrays
    (bind _outactors (`GameplayStatics.GetAllActorsOfClass` "/Game/KoH/Blueprints/SpawnSystemInfluence/BP_InfSpawnPoint.BP_InfSpawnPoint_C" :!label _label))
    (set `self.AllSpawnPoints` _outactors)
    (`self.InitializeSpawnPointsArrays`)
    (elif (`KismetSystemLibrary.IsServer`)
      (goto _label))))

(event `ResetUsedStartPointforNextRound`
  ;[1 1 1] ResetUsedStartPointforNextRound
  ;;[1 1 1] Wait 10 second and clear used start spawn points array for initial spawn in a next round if it will be
  (`KismetSystemLibrary.Delay` 20.0)
  ;;[1 1 1] Update private additional state
  (for _array_element (`self.UsedStartPoints`)
    (`/Game/KoH/Blueprints/SpawnSystemInfluence/BP_InfSpawnPoint.SetIsUsedForStartSpawn?` _array_element false)
    ;;[1 1 1] Clear Used Start Points
    (`KismetArrayLibrary.Array_Clear` (`self.UsedStartPoints`))))

(fn `DebugSpawnLog`
  (params (`For Team Type` :type "/Game/KoH/Blueprints/SpawnSystemInfluence/Data/E_InfTeamType Enum" :default "NewEnumerator0") (`Difined Point` :type "/Game/KoH/Blueprints/SpawnSystemInfluence/BP_InfSpawnPoint Object Reference"))
  (locals (loc_team :type "/Game/KoH/Blueprints/SpawnSystemInfluence/Data/E_InfTeamType Enum" :default "NewEnumerator0") (loc_difined_point :type "/Game/KoH/Blueprints/SpawnSystemInfluence/BP_InfSpawnPoint Object Reference") (loc_point_weight :type "Float (double-precision)" :default 0.0) (other_points_string :type String :default "OTHER POINTS // "))
  (bind _loc_difined_point (`local.loc_difined_point`))
  ;[1 1 1] Condition
  (if (`self.Debug Spawn Log`)
    ;[1 1 1] Initialize
    (set `local.loc_team` `For Team Type`)
    (set `local.loc_difined_point` `Difined Point`)
    (switch `/Game/KoH/Blueprints/SpawnSystemInfluence/Data/E_InfTeamType` (`local.loc_team`)
      (:`NewEnumerator0`
        (set `local.loc_point_weight` (`/Game/KoH/Blueprints/SpawnSystemInfluence/BP_InfSpawnPoint.GetAnyWeight` _loc_difined_point)))
      (:`NewEnumerator1`
        (set `local.loc_point_weight` (`/Game/KoH/Blueprints/SpawnSystemInfluence/BP_InfSpawnPoint.GetTeam1Weight` _loc_difined_point)))
      (:`NewEnumerator2`
        (set `local.loc_point_weight` (`/Game/KoH/Blueprints/SpawnSystemInfluence/BP_InfSpawnPoint.GetTeam2Weight` _loc_difined_point))))
    ;[1 1 1] Log - Print String 1. Defined Point
    (`KismetSystemLibrary.PrintString` (`KismetStringLibrary.Concat_StrStr` (`KismetStringLibrary.Concat_StrStr` "SPAWN " (`|GetEnumeratorNameAsString` (`local.loc_team`))) " // " (`KismetStringLibrary.Concat_StrStr` (`KismetStringLibrary.Concat_StrStr` "SP " (`KismetStringLibrary.Conv_IntToString` (`KismetArrayLibrary.Array_Find` (`self.CommonSpawnPoints`) (`local.loc_difined_point`))) " WEIGHT: ") (`KismetStringLibrary.Conv_DoubleToString` (`local.loc_point_weight`)))) false true (struct :`R` 1.0 :`G` 0.11794 :`A` 1.0))
    ;[1 1 1] Reset String for other spawn point
    (set `local.other_points_string` "")
    ;[1 1 1] Other points string
    (for (_array_element _array_index) (`self.CommonSpawnPoints`)
      (if (not (`/Game/KoH/Blueprints/SpawnSystemInfluence/BP_InfSpawnPoint.GetIsLockSpawn` _array_element))
        (switch `/Game/KoH/Blueprints/SpawnSystemInfluence/Data/E_InfTeamType` (`local.loc_team`)
          (:`NewEnumerator0`
            (set `local.loc_point_weight` (`/Game/KoH/Blueprints/SpawnSystemInfluence/BP_InfSpawnPoint.GetAnyWeight` _array_element)))
          (:`NewEnumerator1`
            (set `local.loc_point_weight` (`/Game/KoH/Blueprints/SpawnSystemInfluence/BP_InfSpawnPoint.GetTeam1Weight` _array_element)))
          (:`NewEnumerator2`
            (set `local.loc_point_weight` (`/Game/KoH/Blueprints/SpawnSystemInfluence/BP_InfSpawnPoint.GetTeam2Weight` _array_element))))
        (set `local.other_points_string` (`KismetStringLibrary.BuildString_Name` (`local.other_points_string`) "SP " (`KismetStringLibrary.Conv_StringToName` (`KismetStringLibrary.Conv_IntToString` _array_index)) (`KismetStringLibrary.Concat_StrStr` " WEIGHT: " (`KismetStringLibrary.Conv_DoubleToString` (`local.loc_point_weight`)) " // ")))))
    (`KismetSystemLibrary.PrintString` (`local.other_points_string`) false true (struct :`R` 1.0 :`G` 0.11794 :`A` 1.0))))

(fn `GetBestCommonSpawnPointTransform`
  (params (`Team Type` :type "/Game/KoH/Blueprints/SpawnSystemInfluence/Data/E_InfTeamType Enum" :default "NewEnumerator0"))
  (returns (`Best Point Transform` :type "Transform Structure (by ref)"))
  (locals (loc_pre_final_wigth :type "Float (double-precision)") (loc_pre_final_point :type "/Game/KoH/Blueprints/SpawnSystemInfluence/BP_InfSpawnPoint Object Reference") (loc_team_type :type "/Game/KoH/Blueprints/SpawnSystemInfluence/Data/E_InfTeamType Enum" :default "NewEnumerator0"))
  (set `local.loc_team_type` `Team Type`)
  ;[1 1 1] Get point for team
  (switch `/Game/KoH/Blueprints/SpawnSystemInfluence/Data/E_InfTeamType` (`local.loc_team_type`)
    (:`NewEnumerator0`
      ;[1 1 1] For any
      (for _array_element (`self.CommonSpawnPoints`)
        (`/Engine/EditorBlueprintResources/StandardMacros.IsValid` _array_element
          (:`Is Valid`
            (bind _anyweight (`/Game/KoH/Blueprints/SpawnSystemInfluence/BP_InfSpawnPoint.GetAnyWeight` _array_element))
            (if (and (> _anyweight (`local.loc_pre_final_wigth`)) (not (`/Game/KoH/Blueprints/SpawnSystemInfluence/BP_InfSpawnPoint.GetIsLockSpawn` _array_element)))
              (set `local.loc_pre_final_point` _array_element)
              (set `local.loc_pre_final_wigth` _anyweight))))))
    (:`NewEnumerator1`
      ;[1 1 1] For team 1
      (for _array_element_2 (`self.CommonSpawnPoints`)
        (`/Engine/EditorBlueprintResources/StandardMacros.IsValid` _array_element_2
          (:`Is Valid`
            (bind _team1weight (`/Game/KoH/Blueprints/SpawnSystemInfluence/BP_InfSpawnPoint.GetTeam1Weight` _array_element_2))
            (if (and (> _team1weight (`local.loc_pre_final_wigth`)) (not (`/Game/KoH/Blueprints/SpawnSystemInfluence/BP_InfSpawnPoint.GetIsLockSpawn` _array_element_2)))
              (set `local.loc_pre_final_point` _array_element_2)
              (set `local.loc_pre_final_wigth` _team1weight))))))
    (:`NewEnumerator2`
      ;[1 1 1] For team 2
      (for _array_element_3 (`self.CommonSpawnPoints`)
        (`/Engine/EditorBlueprintResources/StandardMacros.IsValid` _array_element_3
          (:`Is Valid`
            (bind _team2weight (`/Game/KoH/Blueprints/SpawnSystemInfluence/BP_InfSpawnPoint.GetTeam2Weight` _array_element_3))
            (if (and (> _team2weight (`local.loc_pre_final_wigth`)) (not (`/Game/KoH/Blueprints/SpawnSystemInfluence/BP_InfSpawnPoint.GetIsLockSpawn` _array_element_3)))
              (set `local.loc_pre_final_point` _array_element_3)
              (set `local.loc_pre_final_wigth` _team2weight)))))))
  ;[1 1 1] Server Character Spawned in point
  (`/Game/KoH/Blueprints/SpawnSystemInfluence/BP_InfSpawnPoint.ServerCharacterSpawned` (`local.loc_pre_final_point`))
  ;[1 1 1] Debug Spawn Log
  (`self.DebugSpawnLog` (`local.loc_team_type`) (`local.loc_pre_final_point`))
  ;[1 1 1] Output
  (`/Engine/EditorBlueprintResources/StandardMacros.IsValid` (`local.loc_pre_final_point`)
    (:`Is Valid`
      (return (`Actor.GetTransform` (`local.loc_pre_final_point`))))))

(fn `GetStartSpawnPointTransform `
  (params (`For Team` :type "/Game/KoH/Blueprints/SpawnSystemInfluence/Data/E_InfTeamType Enum" :default "NewEnumerator0"))
  (returns (`SP Transform` :type "Transform Structure"))
  (locals (loc_step_spawn_point :type "/Game/KoH/Blueprints/SpawnSystemInfluence/BP_InfSpawnPoint Object Reference") (loc_start_point_array :type "Array of /Game/KoH/Blueprints/SpawnSystemInfluence/BP_InfSpawnPoint Object Reference"))
  ;[1 1 1] Input
  ;[1 1 1] Initialize loc array of spawn point base on team type
  (switch `/Game/KoH/Blueprints/SpawnSystemInfluence/Data/E_InfTeamType` `For Team`
    (:`NewEnumerator0`
      (set `local.loc_start_point_array` (`self.AnyTeamStartPoints`)))
    (:`NewEnumerator1`
      (set `local.loc_start_point_array` (`self.Team1StartPoints`)))
    (:`NewEnumerator2`
      (set `local.loc_start_point_array` (`self.Team2StartPoints`))))
  ;[1 1 1] For each step with conditions
  (for _array_element (`local.loc_start_point_array`)
    (bind _output_get (set `local.loc_step_spawn_point` _array_element))
    (if (and (`/Game/KoH/Blueprints/SpawnSystemInfluence/BP_InfSpawnPoint.Start Point ` _output_get) (not (`/Game/KoH/Blueprints/SpawnSystemInfluence/BP_InfSpawnPoint.GetIsUsedForStartSpawn?` _output_get)))
      (if (not (`KismetArrayLibrary.Array_Contains` (`self.UsedStartPoints`) (`local.loc_step_spawn_point`)))
        ;[1 1 1] If point is used, it add in used points array
        (`KismetArrayLibrary.Array_Add` (`self.UsedStartPoints`) (`local.loc_step_spawn_point`))
        ;[1 1 1] Update private additional state
        (`/Game/KoH/Blueprints/SpawnSystemInfluence/BP_InfSpawnPoint.ServerCharacterSpawned` (`local.loc_step_spawn_point`))
        ;[1 1 1] Output
        (return (`Actor.GetTransform` (`local.loc_step_spawn_point`))))))
  ;[1 1 1] ResetUsedStartPointforNextRound
  (`self.ResetUsedStartPointforNextRound`))

(fn `InitializeSpawnPointsArrays`
  (locals (loc_step_start_sp :type "/Game/KoH/Blueprints/SpawnSystemInfluence/BP_InfSpawnPoint Object Reference"))
  (for _array_element (`self.AllSpawnPoints`)
    (bind _output_get (set `local.loc_step_start_sp` _array_element))
    (if (`/Game/KoH/Blueprints/SpawnSystemInfluence/BP_InfSpawnPoint.Start Point ` _output_get)
      ;[1 1 1] Start Points
      (switch `/Game/KoH/Blueprints/SpawnSystemInfluence/Data/E_InfTeamType` (`/Game/KoH/Blueprints/SpawnSystemInfluence/BP_InfSpawnPoint.Team` (`local.loc_step_start_sp`))
        (:`NewEnumerator0`
          (`KismetArrayLibrary.Array_Add` (`self.AnyTeamStartPoints`) (`local.loc_step_start_sp`)))
        (:`NewEnumerator1`
          (`KismetArrayLibrary.Array_Add` (`self.Team1StartPoints`) (`local.loc_step_start_sp`)))
        (:`NewEnumerator2`
          (`KismetArrayLibrary.Array_Add` (`self.Team2StartPoints`) (`local.loc_step_start_sp`))))
      (else
        ;[1 1 1] Common Points
        (`KismetArrayLibrary.Array_Add` (`self.CommonSpawnPoints`) (`local.loc_step_start_sp`))))))