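; Player state Blueprint for the Circulatory game mode base that shows and hides the respawn screen.
; On BeginPlay it binds handlers to the client open and close respawn screen triggers.
; Opening creates the respawn widget for player controller 0 and adds it to the viewport, but only while the game state reports Round Started.
; Closing removes the stored widget from its parent if it is valid.
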(event `self.ReceiveBeginPlay`
  (`parent.ReceiveBeginPlay`)
  ;[1 1 1] Open Respawn Screen
  (add `self.TriggerClientOpenRespawnScreen` (delegate `HandleTriggerClientOpenRespawnScreen`))
  ;[1 1 1] Close Respawn Screen
  (add `self.TriggerClientCloseRespawnScreen` (delegate `HandleTriggerClientCloseRespawnScreen`)))

(event `HandleTriggerClientCloseRespawnScreen`
  ;[1 1 1] Close Respawn Screen
  (`/Engine/EditorBlueprintResources/StandardMacros.IsValid` (`self.RespawnScreen`)
    (:`Is Valid`
      (`Widget.RemoveFromParent` (`self.RespawnScreen`)))))

(event `HandleTriggerClientOpenRespawnScreen`
  ;[1 1 1] Open Respawn Screen
  (bind _asbp_gs_base (cast `/Game/KoH/Blueprints/GameModeBase/BP_GS_Base` (`GameplayStatics.GetGameState`)))
  (switch `/Game/KoH/Blueprints/GameModeBase/Data/E_MatchState` (`/Game/KoH/Blueprints/GameModeBase/BP_GS_Base.GetMatchState` _asbp_gs_base)
    (:`NewEnumerator2`
      (bind _returnvalue (`|CreateWidget` "/Game/KoH/Blueprints/UIBase/WBP_RespawnScreen.WBP_RespawnScreen_C" (`GameplayStatics.GetPlayerController` 0)))
      (bind _output_get (set `self.RespawnScreen` _returnvalue))
      (`/Engine/EditorBlueprintResources/StandardMacros.IsValid` (`self.RespawnScreen`)
        (:`Is Valid`
          (`UserWidget.AddToViewport` _output_get 0))))))

(fn `UserConstructionScript`
  (`parent.UserConstructionScript`))