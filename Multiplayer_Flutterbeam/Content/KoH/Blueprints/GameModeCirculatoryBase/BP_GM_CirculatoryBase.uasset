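; Base game mode for the Circulatory mode that handles team-based spawning of players.
; InitialPlayersSpawn places each player in the PlayerArray at a team start point, while the server common-spawn trigger uses the team's best common point, both from InfluenceSpawnSystem.
; Both paths multicast control rotation, spawn and possess a character, then set its BP_InfTeamID team, via ServerInitializeTeam initially and SetTeam for common spawns.
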(event `self.ReceiveBeginPlay`
  (`parent.ReceiveBeginPlay`)
  ;[1 1 1] Common Spawn
  (add `self.TriggerServerCommonSpawn` (delegate `HandleTriggerServerCommonSpawn`)))

(event `HandleTriggerServerCommonSpawn` :!signature `self.TriggerServerCommonSpawn`
  (params (CommonPS :type "/Game/KoH/Blueprints/GameModeBase/BP_PS_Base Object Reference"))
  ;[1 1 1] Common Spawn
  (`self.CirculatoryCommonPlayersSpawn` CommonPS))

(event `self.InitialPlayersSpawn`
  ;[1 1 1] Initial Players Spawn
  (for _array_element (`GameStateBase.PlayerArray` (`self.GetBaseGS`))
    (`/Engine/EditorBlueprintResources/StandardMacros.IsValid` _array_element
      (:`Is Valid`
        (`self.CirculatoryInitialPlayersSpawn` _array_element)))))

(fn `CirculatoryCommonPlayersSpawn`
  (params (`Player State` :type "PlayerState Object Reference"))
  (locals (loc_player_controller :type "PlayerController Object Reference") (loc_player_state :type "/Game/KoH/Blueprints/GameModeBase/BP_PS_Base Object Reference"))
  (bind _returnvalue (`self.GetOwner` `Player State`))
  (bind _asbp_ps_base (cast `/Game/KoH/Blueprints/GameModeBase/BP_PS_Base` `Player State`))
  (set `local.loc_player_state` _asbp_ps_base)
  (`/Engine/EditorBlueprintResources/StandardMacros.IsValid` _returnvalue
    (:`Is Valid`
      (bind _asplayer_controller (cast `PlayerController` _returnvalue))
      (set `local.loc_player_controller` _asplayer_controller)
      (bind _asbp_ps_base_2 (cast `/Game/KoH/Blueprints/GameModeBase/BP_PS_Base` `Player State`))
      (switch `/Game/KoH/Blueprints/GameModeBase/Data/E_ModeTeamType` (`/Game/KoH/Blueprints/GameModeBase/BP_PS_Base.GetTeam` _asbp_ps_base_2)
        (:`NewEnumerator1`
          (bind _best_point_transform (`/Game/KoH/Blueprints/SpawnSystemInfluence/BP_GMC_InfluenceSpawnSystem.GetBestCommonSpawnPointTransform` (`self.InfluenceSpawnSystem`) "NewEnumerator1"))
          (`/Game/KoH/Blueprints/GameModeBase/BP_PCC_Base.MulticastSetControlRotationOnSpawn` (`self.GetComponentByClass` (`local.loc_player_controller`) "/Game/KoH/Blueprints/GameModeBase/BP_PCC_Base.BP_PCC_Base_C") (.rotation _best_point_transform))
          (bind _returnvalue_2 (`|SpawnActorFromClass` (`self.CharacterClass`) _best_point_transform "AlwaysSpawn" "OverrideRootScale" null null))
          (`/Engine/EditorBlueprintResources/StandardMacros.IsValid` _returnvalue_2
            (:`Is Valid`
              (bind _aspawn (cast `Pawn` _returnvalue_2))
              (`Controller.Possess` (`local.loc_player_controller`) _aspawn)
              (switch `/Game/KoH/Blueprints/GameModeBase/Data/E_ModeTeamType` (`/Game/KoH/Blueprints/GameModeBase/BP_PS_Base.GetTeam` (`local.loc_player_state`))
                (:`NewEnumerator1`
                  (bind _returnvalue_3 (`self.GetComponentByClass` _aspawn "/Game/KoH/Blueprints/SpawnSystemInfluence/BP_InfTeamID.BP_InfTeamID_C"))
                  (`/Game/KoH/Blueprints/SpawnSystemInfluence/BP_InfTeamID.SetTeam` _returnvalue_3 "NewEnumerator1"))
                (:`NewEnumerator2`
                  (`/Game/KoH/Blueprints/SpawnSystemInfluence/BP_InfTeamID.SetTeam` _returnvalue_3 "NewEnumerator2"))))))
        (:`NewEnumerator2`
          (bind _best_point_transform_2 (`/Game/KoH/Blueprints/SpawnSystemInfluence/BP_GMC_InfluenceSpawnSystem.GetBestCommonSpawnPointTransform` (`self.InfluenceSpawnSystem`) "NewEnumerator2"))
          (`/Game/KoH/Blueprints/GameModeBase/BP_PCC_Base.MulticastSetControlRotationOnSpawn` (`self.GetComponentByClass` (`local.loc_player_controller`) "/Game/KoH/Blueprints/GameModeBase/BP_PCC_Base.BP_PCC_Base_C") (.rotation _best_point_transform_2))
          (bind _returnvalue_4 (`|SpawnActorFromClass` (`self.CharacterClass`) _best_point_transform_2 "AlwaysSpawn" "OverrideRootScale" null null))
          (`/Engine/EditorBlueprintResources/StandardMacros.IsValid` _returnvalue_4
            (:`Is Valid`
              (bind _aspawn_2 (cast `Pawn` _returnvalue_4))
              (`Controller.Possess` (`local.loc_player_controller`) _aspawn_2)
              (switch `/Game/KoH/Blueprints/GameModeBase/Data/E_ModeTeamType` (`/Game/KoH/Blueprints/GameModeBase/BP_PS_Base.GetTeam` (`local.loc_player_state`))
                (:`NewEnumerator1`
                  (bind _returnvalue_5 (`self.GetComponentByClass` _aspawn_2 "/Game/KoH/Blueprints/SpawnSystemInfluence/BP_InfTeamID.BP_InfTeamID_C"))
                  (`/Game/KoH/Blueprints/SpawnSystemInfluence/BP_InfTeamID.SetTeam` _returnvalue_5 "NewEnumerator1"))
                (:`NewEnumerator2`
                  (`/Game/KoH/Blueprints/SpawnSystemInfluence/BP_InfTeamID.SetTeam` _returnvalue_5 "NewEnumerator2"))))))))))

(fn `CirculatoryInitialPlayersSpawn`
  (params (`Player State` :type "PlayerState Object Reference"))
  (locals (loc_player_controller :type "PlayerController Object Reference") (loc_player_state :type "/Game/KoH/Blueprints/GameModeBase/BP_PS_Base Object Reference"))
  (bind _returnvalue (`self.GetOwner` `Player State`))
  (bind _characterclass (`self.CharacterClass`))
  (`/Engine/EditorBlueprintResources/StandardMacros.IsValid` _returnvalue
    (:`Is Valid`
      (bind _asplayer_controller (cast `PlayerController` _returnvalue))
      (set `local.loc_player_controller` _asplayer_controller)
      (bind _asbp_ps_base (cast `/Game/KoH/Blueprints/GameModeBase/BP_PS_Base` `Player State`))
      (bind _output_get (set `local.loc_player_state` _asbp_ps_base))
      (switch `/Game/KoH/Blueprints/GameModeBase/Data/E_ModeTeamType` (`/Game/KoH/Blueprints/GameModeBase/BP_PS_Base.GetTeam` _output_get)
        (:`NewEnumerator1`
          (bind _sp_transform (`/Game/KoH/Blueprints/SpawnSystemInfluence/BP_GMC_InfluenceSpawnSystem.GetStartSpawnPointTransform ` (`self.InfluenceSpawnSystem`) "NewEnumerator1"))
          (`/Game/KoH/Blueprints/GameModeBase/BP_PCC_Base.MulticastSetControlRotationOnSpawn` (`self.GetComponentByClass` (`local.loc_player_controller`) "/Game/KoH/Blueprints/GameModeBase/BP_PCC_Base.BP_PCC_Base_C") (.rotation _sp_transform))
          (bind _returnvalue_2 (`|SpawnActorFromClass` _characterclass _sp_transform "AlwaysSpawn" "OverrideRootScale" null null))
          (`/Engine/EditorBlueprintResources/StandardMacros.IsValid` _returnvalue_2
            (:`Is Valid`
              (bind _aspawn (cast `Pawn` _returnvalue_2))
              (`Controller.Possess` (`local.loc_player_controller`) _aspawn)
              (switch `/Game/KoH/Blueprints/GameModeBase/Data/E_ModeTeamType` (`/Game/KoH/Blueprints/GameModeBase/BP_PS_Base.GetTeam` (`local.loc_player_state`))
                (:`NewEnumerator1`
                  (bind _returnvalue_3 (`self.GetComponentByClass` _aspawn "/Game/KoH/Blueprints/SpawnSystemInfluence/BP_InfTeamID.BP_InfTeamID_C"))
                  (`/Game/KoH/Blueprints/SpawnSystemInfluence/BP_InfTeamID.ServerInitializeTeam` _returnvalue_3 "NewEnumerator1"))
                (:`NewEnumerator2`
                  (`/Game/KoH/Blueprints/SpawnSystemInfluence/BP_InfTeamID.ServerInitializeTeam` _returnvalue_3 "NewEnumerator2"))))))
        (:`NewEnumerator2`
          (bind _sp_transform_2 (`/Game/KoH/Blueprints/SpawnSystemInfluence/BP_GMC_InfluenceSpawnSystem.GetStartSpawnPointTransform ` (`self.InfluenceSpawnSystem`) "NewEnumerator2"))
          (`/Game/KoH/Blueprints/GameModeBase/BP_PCC_Base.MulticastSetControlRotationOnSpawn` (`self.GetComponentByClass` (`local.loc_player_controller`) "/Game/KoH/Blueprints/GameModeBase/BP_PCC_Base.BP_PCC_Base_C") (.rotation _sp_transform_2))
          (bind _returnvalue_4 (`|SpawnActorFromClass` _characterclass _sp_transform_2 "AlwaysSpawn" "OverrideRootScale" null null))
          (`/Engine/EditorBlueprintResources/StandardMacros.IsValid` _returnvalue_4
            (:`Is Valid`
              (bind _aspawn_2 (cast `Pawn` _returnvalue_4))
              (`Controller.Possess` (`local.loc_player_controller`) _aspawn_2)
              (switch `/Game/KoH/Blueprints/GameModeBase/Data/E_ModeTeamType` (`/Game/KoH/Blueprints/GameModeBase/BP_PS_Base.GetTeam` (`local.loc_player_state`))
                (:`NewEnumerator1`
                  (bind _returnvalue_5 (`self.GetComponentByClass` _aspawn_2 "/Game/KoH/Blueprints/SpawnSystemInfluence/BP_InfTeamID.BP_InfTeamID_C"))
                  (`/Game/KoH/Blueprints/SpawnSystemInfluence/BP_InfTeamID.ServerInitializeTeam` _returnvalue_5 "NewEnumerator1"))
                (:`NewEnumerator2`
                  (`/Game/KoH/Blueprints/SpawnSystemInfluence/BP_InfTeamID.ServerInitializeTeam` _returnvalue_5 "NewEnumerator2"))))))))))

(fn `UserConstructionScript`
  (`parent.UserConstructionScript`))