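; Base visual indicator for a capture point's form, using a static mesh to show a Neutral, Red or Blue state.
; A server event passes X and Y scale to a multicast event, which resizes the mesh while keeping Z at 1.
; A separate client event swaps the mesh's first material to grey, red or blue test materials to match the given color.
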(event `MulticastInitializeScale`
  (params (`Scale X` :type "Float (double-precision)") (`Scale Y` :type "Float (double-precision)"))
  ;[1 1 1] InitializeScale
  (`SceneComponent.SetRelativeScale3D` (`self.StaticMesh`) (`KismetMathLibrary.MakeVector` `Scale X` `Scale Y` 1.0)))

(event `ServerInitializeScale`
  (params (`Scale X` :type "Float (double-precision)") (`Scale Y` :type "Float (double-precision)"))
  ;[1 1 1] InitializeScale
  (`self.MulticastInitializeScale` `Scale X` `Scale Y`))

(event `ClientChangeFormIndicationColor`
  (params (Color :type "/Game/KoH/Blueprints/CapturePointBase/Data/E_FormIndicationColor Enum" :default "NewEnumerator0"))
  ;[1 1 1] ChangeFormIndicationColor
  (switch `/Game/KoH/Blueprints/CapturePointBase/Data/E_FormIndicationColor` Color
    (:`NewEnumerator0`
      (`PrimitiveComponent.SetMaterial` (`self.StaticMesh`) 0 "/Game/KoH/Materials/Common/M_TestGameObjGrey.M_TestGameObjGrey"))
    (:`NewEnumerator1`
      (`PrimitiveComponent.SetMaterial` (`self.StaticMesh`) 0 "/Game/KoH/Materials/Common/M_TestGameObjRed.M_TestGameObjRed"))
    (:`NewEnumerator2`
      (`PrimitiveComponent.SetMaterial` (`self.StaticMesh`) 0 "/Game/KoH/Materials/Common/M_TestGameObjBlue.M_TestGameObjBlue"))))

(fn `UserConstructionScript`)