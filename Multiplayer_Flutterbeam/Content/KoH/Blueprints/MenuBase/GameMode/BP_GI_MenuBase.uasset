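; Base menu GameInstance that manages LAN sessions and holds local player and game descriptors for the menus.
; Creating a session flags the local player as host and opens the lobby as a listen server, while joining flags them as client.
; Destroying resets the player descriptor before its IsHost check, which gates clearing the GameMode's player list, then opens the main menu.
; Getters, setters and toggleable debug logging support these flows.
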(event `InitializeGameModeComponent`
  ;[1 1 1] INITIALIZE GAME MODE COMPONENT
)

(event `CreateSession`
  ;[1 1 1] CREATE SESSION
  (`CreateSessionCallbackProxy.CreateSession` (`GameplayStatics.GetPlayerController` 0) 100 true
    (:`OnSuccess`
      (`self.DrawDebugLog` "SESSION CREATED")
      (`self.SetLocalClientAsHost`)
      (`GameplayStatics.OpenLevel` (`self.LobbyLevelName`) true "listen"))
    (:`OnFailure`
      (`self.DrawDebugLog` "FAIL SESSION CREATED"))))

(event `JoinSession`
  (params (SearchResult :type "BlueprintSessionResult Structure (by ref)"))
  ;[1 1 1] JOIN TO SESSION
  (`JoinSessionCallbackProxy.JoinSession` (`GameplayStatics.GetPlayerController` 0) SearchResult
    (:`OnSuccess`
      (`self.DrawDebugLog` "JOINED")
      (`self.SetLocalClientAsClient`))
    (:`OnFailure`
      (`self.DrawDebugLog` "FAIL JOINED"))))

(event `DestroySession`
  ;[1 1 1] DESTROY SESSION
  (`DestroySessionCallbackProxy.DestroySession` (`GameplayStatics.GetPlayerController` 0)
    (:`OnSuccess`
      (`self.DrawDebugLog` "DESTROY")
      (bind _output_get (set `self.MenuPlayerDesc` (struct)))
      (if (`.IsHost?_14_4BCB848D47565AE872CBD7ACBA4F051E` (break `/Game/KoH/Blueprints/MenuBase/Data/STR_MenuPlayerDesc` _output_get))
        (bind _asbp_gm_menu_base (cast `/Game/KoH/Blueprints/MenuBase/GameMode/BP_GM_MenuBase` (`GameplayStatics.GetGameMode`)))
        (`KismetArrayLibrary.Array_Clear` (`/Game/KoH/Blueprints/MenuBase/GameMode/BP_GM_MenuBase.GetPlayersList` _asbp_gm_menu_base)))
      (set `self.MenuPlayerDesc` (make `/Game/KoH/Blueprints/MenuBase/Data/STR_MenuPlayerDesc` (`.PlayerName_16_0AF1807D4D2FB34C017520B53AD48A0D` (break `/Game/KoH/Blueprints/MenuBase/Data/STR_MenuPlayerDesc` (`self.MenuPlayerDesc`)))))
      (`GameplayStatics.OpenLevel` (`self.MainMenuLevelName`) true "listen"))
    (:`OnFailure`
      (`self.DrawDebugLog` "FAIL DESTROY "))))

(event `LocalUpdatePlayerName`
  (params (`Player Name` :type String))
  ;[1 1 1] LocalUpdatePlayerName   (For save from main menu on launch or on change player name in options)
  (`self.SetLocalClientName` `Player Name`))

(fn `DrawDebugLog`
  (params (`Debug Log` :type String))
  (if (`self.DrawDebugLog?`)
    (`KismetSystemLibrary.PrintString` (`KismetStringLibrary.Concat_StrStr` "BASE MENU GI: " `Debug Log`))))

(fn `GetMenuGameDesc`
  (returns (MenuGameDesc :type "/Game/KoH/Blueprints/MenuBase/Data/STR_MenuGameDesc Structure"))
  (return (`self.MenuGameDesc`)))

(fn `GetMenuPlayerDesc`
  (returns (MenuPlayerDesc :type "/Game/KoH/Blueprints/MenuBase/Data/STR_MenuPlayerDesc Structure"))
  (return (`self.MenuPlayerDesc`)))

(fn `ResetHostClientSettings`
  (bind (_playername _ishost_ _isclient_ _teamtype) (break `/Game/KoH/Blueprints/MenuBase/Data/STR_MenuPlayerDesc` (`self.MenuPlayerDesc`)))
  (set `self.MenuPlayerDesc` (make `/Game/KoH/Blueprints/MenuBase/Data/STR_MenuPlayerDesc` _playername false false _teamtype)))

(fn `SetLocalClientAsClient`
  (bind (_playername _ishost_ _isclient_ _teamtype) (break `/Game/KoH/Blueprints/MenuBase/Data/STR_MenuPlayerDesc` (`self.MenuPlayerDesc`)))
  (set `self.MenuPlayerDesc` (make `/Game/KoH/Blueprints/MenuBase/Data/STR_MenuPlayerDesc` _playername _ishost_ true _teamtype)))

(fn `SetLocalClientAsHost`
  (bind (_playername _ishost_ _isclient_ _teamtype) (break `/Game/KoH/Blueprints/MenuBase/Data/STR_MenuPlayerDesc` (`self.MenuPlayerDesc`)))
  (set `self.MenuPlayerDesc` (make `/Game/KoH/Blueprints/MenuBase/Data/STR_MenuPlayerDesc` _playername true _isclient_ _teamtype)))

(fn `SetLocalClientName`
  (params (`Player Name` :type String))
  (bind (_playername _ishost_ _isclient_ _teamtype) (break `/Game/KoH/Blueprints/MenuBase/Data/STR_MenuPlayerDesc` (`self.MenuPlayerDesc`)))
  (set `self.MenuPlayerDesc` (make `/Game/KoH/Blueprints/MenuBase/Data/STR_MenuPlayerDesc` `Player Name` _ishost_ _isclient_ _teamtype)))

(fn `SetMenuGameDesc`
  (params (MenuGameDesc :type "/Game/KoH/Blueprints/MenuBase/Data/STR_MenuGameDesc Structure"))
  (set `self.MenuGameDesc` MenuGameDesc))

(fn `SetMenuPlayerDesc`
  (params (MenuPlayerDesc :type "/Game/KoH/Blueprints/MenuBase/Data/STR_MenuPlayerDesc Structure"))
  (set `self.MenuPlayerDesc` MenuPlayerDesc))