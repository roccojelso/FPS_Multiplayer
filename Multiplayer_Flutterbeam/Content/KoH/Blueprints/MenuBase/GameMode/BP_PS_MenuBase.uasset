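; Menu-base PlayerState that holds a player's MenuPlayerDesc and syncs it between the local game instance and the network.
; On BeginPlay it reads the descriptor from BP_GI_MenuBase and relays it through client and server events into its own variable.
; A server-to-client event pair writes the descriptor back into the game instance, while a separate server event sets it and multicasts it.
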(event `self.ReceiveBeginPlay`
  ;[1 1 1] Event Begin Play
  (bind _asbp_gi_menu_base (cast `/Game/KoH/Blueprints/MenuBase/GameMode/BP_GI_MenuBase` (`GameplayStatics.GetGameInstance`)))
  (`self.ClientUpdateMenuPlayerDesc` (`/Game/KoH/Blueprints/MenuBase/GameMode/BP_GI_MenuBase.GetMenuPlayerDesc` _asbp_gi_menu_base)))

(event `ClientUpdateMenuPlayerDesc`
  (params (MenuPlayerDesc :type "/Game/KoH/Blueprints/MenuBase/Data/STR_MenuPlayerDesc Structure"))
  ;[1 1 1] Initialize Player Properties for all  from game instance (local value)
  ;;[1 1 1] ServerInitializePlayerProperties
  (`self.ServerUpdateMenuPlayerDesc` MenuPlayerDesc))

(event `ServerUpdateMenuPlayerDesc`
  (params (MenuPlayerDecs :type "/Game/KoH/Blueprints/MenuBase/Data/STR_MenuPlayerDesc Structure"))
  ;[1 1 1] Initialize Player Properties for all  from game instance (local value)
  ;;[1 1 1] MulticastInitializePlayerProperties
  (set `self.MenuPlayerDesc` MenuPlayerDecs))

(event `ServerUpdatePlayerPropInGameInstance`
  (`self.ClientUpdatePlayerPropInGameInstance`))

(event `ClientUpdatePlayerPropInGameInstance`
  (bind _asbp_gi_menu_base (cast `/Game/KoH/Blueprints/MenuBase/GameMode/BP_GI_MenuBase` (`GameplayStatics.GetGameInstance`)))
  (`/Game/KoH/Blueprints/MenuBase/GameMode/BP_GI_MenuBase.SetMenuPlayerDesc` _asbp_gi_menu_base (`self.MenuPlayerDesc`)))

(event `ServerInitializeMenuPlayerDesc`
  (params (MenuPlayerDesc :type "/Game/KoH/Blueprints/MenuBase/Data/STR_MenuPlayerDesc Structure"))
  (bind _output_get (set `self.MenuPlayerDesc` MenuPlayerDesc))
  (`self.MulticastInitializeMenuPlayerDesc` _output_get))

(event `MulticastInitializeMenuPlayerDesc`
  (params (MenuPlayerDesc :type "/Game/KoH/Blueprints/MenuBase/Data/STR_MenuPlayerDesc Structure"))
  (set `self.MenuPlayerDesc` MenuPlayerDesc))

(fn `GetMenuPlayerDesc`
  (returns (MenuPlayerDesc :type "/Game/KoH/Blueprints/MenuBase/Data/STR_MenuPlayerDesc Structure"))
  (return (`self.MenuPlayerDesc`)))

(fn `SetMenuPlayerDesc`
  (params (MenuPlayerDesc :type "/Game/KoH/Blueprints/MenuBase/Data/STR_MenuPlayerDesc Structure"))
  (set `self.MenuPlayerDesc` MenuPlayerDesc))

(fn `UserConstructionScript`)