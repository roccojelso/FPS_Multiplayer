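; Menu and lobby player controller that creates the main menu on the local player after a short delay, with UI-only input.
; Server events forward player list, map, game mode, menu lock and countdown changes to Client counterparts, which fire dispatchers or update widgets.
; Client handlers also save the player description to the game instance, destroy sessions, and swap to a loading screen when the countdown reaches one.
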(event `self.ReceiveBeginPlay`
  ;[1 1 1] EVENT BEGIN PLAY
  (if (`self.IsLocalPlayerController`)
    (`KismetSystemLibrary.Delay` 2.0)
    (`WidgetLayoutLibrary.RemoveAllWidgets`)
    (bind _returnvalue (`|CreateWidget` "/Game/KoH/Blueprints/MenuBase/UI/WBP_MainMenu.WBP_MainMenu_C"))
    (bind _output_get (set `self.MenuWidgetRef` _returnvalue))
    (`/Engine/EditorBlueprintResources/StandardMacros.IsValid` _output_get
      (:`Is Valid`
        (`UserWidget.AddToViewport` (`self.MenuWidgetRef`) 0)
        (set `PlayerController.bShowMouseCursor` true (`GameplayStatics.GetPlayerController` 0))
        (`WidgetBlueprintLibrary.SetInputMode_UIOnlyEx` (`GameplayStatics.GetPlayerController` 0) (`self.MenuWidgetRef`))))))

(event `ServerUpdatePlayersList`
  (params (`AreTeamsDivided?` :type Boolean))
  ;[1 1 1] UPDATE PLAYERS LIST
  (`self.ClientUpdatePlayersList` `AreTeamsDivided?`))

(event `ClientUpdatePlayersList`
  (params (`AreTeamsDivided?` :type Boolean))
  ;[1 1 1] UPDATE PLAYERS LIST
  (`self.UpdatePlayersList` `AreTeamsDivided?`)
  (`KismetSystemLibrary.Delay` 1.0)
  (bind _asbp_ps_menu_base (cast `/Game/KoH/Blueprints/MenuBase/GameMode/BP_PS_MenuBase` (`self.PlayerState`)))
  (bind _asbp_gi_menu_base (cast `/Game/KoH/Blueprints/MenuBase/GameMode/BP_GI_MenuBase` (`GameplayStatics.GetGameInstance`)))
  (`/Game/KoH/Blueprints/MenuBase/GameMode/BP_GI_MenuBase.SetMenuPlayerDesc` _asbp_gi_menu_base (`/Game/KoH/Blueprints/MenuBase/GameMode/BP_PS_MenuBase.GetMenuPlayerDesc` _asbp_ps_menu_base)))

(event `ServerHostSetMap`
  ;[1 1 1] MAP UPDATED
  (`self.ClientHostSetMap`))

(event `ClientHostSetMap`
  ;[1 1 1] MAP UPDATED
  (`self.UpdateMapOptions`))

(event `ServerHostSetGamemode`
  ;[1 1 1] GAME MODE UPDATE
  (`self.ClientHostSetGamemode`))

(event `ClientHostSetGamemode`
  ;[1 1 1] GAME MODE UPDATE
  (`self.UpdateGameModeOptions`))

(event `ClientDestroySession`
  ;[1 1 1] CLIENT DESTROY SESSION
  (bind _asbp_gi_menu_base (cast `/Game/KoH/Blueprints/MenuBase/GameMode/BP_GI_MenuBase` (`GameplayStatics.GetGameInstance`)))
  (`/Game/KoH/Blueprints/MenuBase/GameMode/BP_GI_MenuBase.DestroySession` _asbp_gi_menu_base))

(event `ServerHostLockMenu`
  (params (`Host?` :type Boolean))
  ;[1 1 1] LOCK MENU
  (`self.ClientLockMenu` `Host?`))

(event `ClientLockMenu`
  (params (`Host?` :type Boolean))
  (bind _menuwidgetref (`self.MenuWidgetRef`))
  ;[1 1 1] LOCK MENU
  (if `Host?`
    (`Widget.SetIsEnabled` (`/Game/KoH/Blueprints/MenuBase/UI/WBP_MainMenu.ButtonsList_LobbyHostMenu` _menuwidgetref) false)
    (else
      (`Widget.SetIsEnabled` (`/Game/KoH/Blueprints/MenuBase/UI/WBP_MainMenu.ButtonsList_LobbyClientMenu` _menuwidgetref) false))))

(event `ServerTimerUpdate`
  (params (Timer :type Integer))
  ;[1 1 1] TIMER UPDATE
  (`self.ClientTimerUpdate` Timer))

(event `ClientTimerUpdate`
  (params (Timer :type Integer))
  ;[1 1 1] TIMER UPDATE
  (`self.UpdateTimer` Timer)
  (`Widget.SetVisibility` (`/Game/KoH/Blueprints/MenuBase/UI/WBP_LobbyGameDescription.CountdownBlock` (`/Game/KoH/Blueprints/MenuBase/UI/WBP_MainMenu.LobbyGameSettingsDesc` (`self.MenuWidgetRef`))) "Visible")
  (if (== Timer 1)
    (`WidgetLayoutLibrary.RemoveAllWidgets`)
    (bind _returnvalue (`|CreateWidget` "/Game/KoH/Blueprints/MenuBase/UI/WBP_LoadingScreen.WBP_LoadingScreen_C"))
    (`UserWidget.AddToViewport` _returnvalue 0)))

(fn `UserConstructionScript`)