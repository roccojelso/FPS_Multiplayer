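; Lobby game mode for the menu base that tracks joined players and runs the host-driven flow from map and mode selection to match launch.
; Host choices are written to the game state, with player caps read from a data table, and relayed to each player controller.
; A looping countdown splits players into alternating teams, disconnects any overflow, locks menus, then saves the game description to the game instance and server-travels to the map.
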(event `self.K2_PostLogin`
  (params (NewPlayer :type "PlayerController Object Reference"))
  ;[1 1 1] ON POST LOGIN
  (`KismetArrayLibrary.Array_Add` (`self.PlayersList`) NewPlayer)
  (`self.RefreshList`))

(event `HostStartedMatch`
  ;[1 1 1] HOST STARTED MATCH
  (bind _returnvalue (`KismetSystemLibrary.K2_SetTimerDelegate` (delegate `Countdown`) 1.0 true))
  (set `self.TimerHandle` _returnvalue))

(event `Countdown`
  ;[1 1 1] HOST STARTED MATCH
  (bind _result (`/Engine/EditorBlueprintResources/StandardMacros.DecrementInt` (`self.Timer`))
    (:`  `
      (if (== _result 8)
        (`self.DivideOnTeams`)
        (elif (== _result 5)
          (`self.MenuLocker`)
          (`self.TriggerPreLaunchMatch`)
          (elif (== _result 0)
            (`KismetSystemLibrary.K2_PauseTimerHandle` (`self.TimerHandle`))
            (`self.LaunchMatch`))))
      (for _array_element (`self.PlayersList`)
        (bind _asbp_pc_menu_base (cast `/Game/KoH/Blueprints/MenuBase/GameMode/BP_PC_MenuBase` _array_element))
        (`/Game/KoH/Blueprints/MenuBase/GameMode/BP_PC_MenuBase.ServerTimerUpdate` _asbp_pc_menu_base (`self.Timer`))))))

(event `self.K2_OnLogout`
  (params (ExitingController :type "Controller Object Reference"))
  ;[1 1 1] ON LOG OUT
  (for (_array_element _array_index) (`self.PlayersList`)
    (`/Engine/EditorBlueprintResources/StandardMacros.IsValid` _array_element
      (:`Is Valid`
        (if (== (`Controller.PlayerState` _array_element) ExitingController)
          (`KismetArrayLibrary.Array_Remove` (`self.PlayersList`) _array_index)))))
  (`self.RefreshList`))

(event `DivideOnTeams`
  ;[1 1 1] DIVIDE ON TEAMS
  (set `self.Are Team Divided?` true)
  (for (_array_element _array_index) (`self.PlayersList`)
    (if (< (`self.CurrentPlayerCountOnDividing`) (`self.Max Count Player`))
      (`/Engine/EditorBlueprintResources/StandardMacros.IncrementInt` (`self.CurrentPlayerCountOnDividing`)
        (:`  `
          (if (`KismetMathLibrary.Conv_IntToBool` (mod _array_index 2))
            (bind _playerstate (`Controller.PlayerState` _array_element))
            (bind _asbp_ps_menu_base (cast `/Game/KoH/Blueprints/MenuBase/GameMode/BP_PS_MenuBase` _playerstate))
            (bind (_playername _ishost_ _isclient_) (break `/Game/KoH/Blueprints/MenuBase/Data/STR_MenuPlayerDesc` (`/Game/KoH/Blueprints/MenuBase/GameMode/BP_PS_MenuBase.GetMenuPlayerDesc` _asbp_ps_menu_base)))
            (`/Game/KoH/Blueprints/MenuBase/GameMode/BP_PS_MenuBase.ServerInitializeMenuPlayerDesc` _asbp_ps_menu_base (make `/Game/KoH/Blueprints/MenuBase/Data/STR_MenuPlayerDesc` _playername _ishost_ _isclient_ "NewEnumerator0"))
            (else
              (bind _asbp_ps_menu_base_2 (cast `/Game/KoH/Blueprints/MenuBase/GameMode/BP_PS_MenuBase` _playerstate))
              (bind (_playername_2 _ishost__2 _isclient__2) (break `/Game/KoH/Blueprints/MenuBase/Data/STR_MenuPlayerDesc` (`/Game/KoH/Blueprints/MenuBase/GameMode/BP_PS_MenuBase.GetMenuPlayerDesc` _asbp_ps_menu_base_2)))
              (`/Game/KoH/Blueprints/MenuBase/GameMode/BP_PS_MenuBase.ServerInitializeMenuPlayerDesc` _asbp_ps_menu_base_2 (make `/Game/KoH/Blueprints/MenuBase/Data/STR_MenuPlayerDesc` _playername_2 _ishost__2 _isclient__2 "NewEnumerator1"))))
          (`self.RefreshList`)))
      (else
        (bind _asbp_pc_menu_base (cast `/Game/KoH/Blueprints/MenuBase/GameMode/BP_PC_MenuBase` _array_element))
        (`/Game/KoH/Blueprints/MenuBase/GameMode/BP_PC_MenuBase.ClientDestroySession` _asbp_pc_menu_base)
        (`KismetArrayLibrary.Array_RemoveItem` (`self.PlayersList`) _array_element)))))

(event `HostUpdateGameMode`
  (params (`GameMode Index` :type Integer) (`Game Mode Type` :type "/Game/KoH/Blueprints/MenuBase/Data/E_MenuGameModesType Enum" :default "NewEnumerator0"))
  ;[1 1 1] ON HOST UPDATE GAME MODE
  (bind _asbp_gs_menu_base (cast `/Game/KoH/Blueprints/MenuBase/GameMode/BP_GS_MenuBase` (`GameplayStatics.GetGameState`)))
  (`/Game/KoH/Blueprints/MenuBase/GameMode/BP_GS_MenuBase.SetGameModeIndex` _asbp_gs_menu_base `GameMode Index`)
  (bind _asbp_gs_menu_base_2 (cast `/Game/KoH/Blueprints/MenuBase/GameMode/BP_GS_MenuBase` (`GameplayStatics.GetGameState`)))
  (bind _outrownames (`DataTableFunctionLibrary.GetDataTableRowNames` (`/Game/KoH/Blueprints/MenuBase/GameMode/BP_GS_MenuBase.MenuGameModesLibrary` _asbp_gs_menu_base_2)))
  (for _array_element _outrownames
    (bind _asbp_gs_menu_base_3 (cast `/Game/KoH/Blueprints/MenuBase/GameMode/BP_GS_MenuBase` (`GameplayStatics.GetGameState`)))
    (bind _returnvalue (`|GetDataTableRow` (`/Game/KoH/Blueprints/MenuBase/GameMode/BP_GS_MenuBase.MenuGameModesLibrary` _asbp_gs_menu_base_3) _array_element)
      (:`then`
        (bind (_gamemodetype _maxplayercount) (break `/Game/KoH/Blueprints/MenuBase/Data/STR_MenuGameModeLibDesc` _returnvalue))
        (if (`|EnumEquality` _gamemodetype `Game Mode Type`)
          (set `self.Max Count Player` _maxplayercount)
          (bind (_levelname _levelenginename) (break `/Game/KoH/Blueprints/MenuBase/Data/STR_MenuGameDesc` (`/Game/KoH/Blueprints/MenuBase/GameMode/BP_GS_MenuBase.GetMenuGameDesc` _asbp_gs_menu_base)))
          (`/Game/KoH/Blueprints/MenuBase/GameMode/BP_GS_MenuBase.SetMenuGameDesc` _asbp_gs_menu_base (make `/Game/KoH/Blueprints/MenuBase/Data/STR_MenuGameDesc` _levelname _levelenginename `Game Mode Type` (`self.Max Count Player`)))
          (`self.TriggerUpdateGameMode`)
          (for _array_element_2 (`self.PlayersList`)
            (bind _asbp_pc_menu_base (cast `/Game/KoH/Blueprints/MenuBase/GameMode/BP_PC_MenuBase` _array_element_2))
            (`/Game/KoH/Blueprints/MenuBase/GameMode/BP_PC_MenuBase.ServerHostSetGamemode` _asbp_pc_menu_base)))))))

(event `LaunchMatch`
  ;[1 1 1] LAUNCH MATCH
  (bind _asbp_gs_menu_base (cast `/Game/KoH/Blueprints/MenuBase/GameMode/BP_GS_MenuBase` (`GameplayStatics.GetGameState`)))
  (bind _asbp_gi_menu_base (cast `/Game/KoH/Blueprints/MenuBase/GameMode/BP_GI_MenuBase` (`GameplayStatics.GetGameInstance`)))
  (bind _menugamedesc (`/Game/KoH/Blueprints/MenuBase/GameMode/BP_GS_MenuBase.GetMenuGameDesc` _asbp_gs_menu_base))
  (`/Game/KoH/Blueprints/MenuBase/GameMode/BP_GI_MenuBase.SetMenuGameDesc` _asbp_gi_menu_base _menugamedesc)
  (`KismetSystemLibrary.ExecuteConsoleCommand` (`KismetStringLibrary.Concat_StrStr` "servertravel/game/" (`.LevelEngineName_18_2A3AAC8E487D062EDB83E2B85910802F` (break `/Game/KoH/Blueprints/MenuBase/Data/STR_MenuGameDesc` _menugamedesc))) null))

(event `HostUpdateMap`
  (params (`Map Index` :type Integer) (`Level Engine Name` :type String) (`Level Name` :type Name))
  ;[1 1 1] ON HOST UPDATE MAP
  (bind _asbp_gs_menu_base (cast `/Game/KoH/Blueprints/MenuBase/GameMode/BP_GS_MenuBase` (`GameplayStatics.GetGameState`)))
  (`/Game/KoH/Blueprints/MenuBase/GameMode/BP_GS_MenuBase.SetLevelIndex` _asbp_gs_menu_base `Map Index`)
  (bind (_levelname _levelenginename _gamemodetype _maxplayercount) (break `/Game/KoH/Blueprints/MenuBase/Data/STR_MenuGameDesc` (`/Game/KoH/Blueprints/MenuBase/GameMode/BP_GS_MenuBase.GetMenuGameDesc` _asbp_gs_menu_base)))
  (`/Game/KoH/Blueprints/MenuBase/GameMode/BP_GS_MenuBase.SetMenuGameDesc` _asbp_gs_menu_base (make `/Game/KoH/Blueprints/MenuBase/Data/STR_MenuGameDesc` `Level Name` `Level Engine Name` _gamemodetype _maxplayercount))
  (for _array_element (`self.PlayersList`)
    (bind _asbp_pc_menu_base (cast `/Game/KoH/Blueprints/MenuBase/GameMode/BP_PC_MenuBase` _array_element))
    (`/Game/KoH/Blueprints/MenuBase/GameMode/BP_PC_MenuBase.ServerHostSetMap` _asbp_pc_menu_base)))

(event `HostOpenModeRulesMenu`
  ;[1 1 1] OPEN / CLOSE MODE RULES MENU
  (`self.TriggerHostOpenModeRulesMenu`))

(event `HandleHostCloseModeRulesMenu`
  ;[1 1 1] OPEN / CLOSE MODE RULES MENU
  (`self.TriggerHostCloseModeRulesMenu`))

(event `RefreshList`
  ;[1 1 1] REFRESH PLAYER LIST
  (for _array_element (`self.PlayersList`)
    (`/Engine/EditorBlueprintResources/StandardMacros.IsValid` _array_element
      (:`Is Valid`
        (bind _asbp_pc_menu_base (cast `/Game/KoH/Blueprints/MenuBase/GameMode/BP_PC_MenuBase` _array_element))
        (`/Game/KoH/Blueprints/MenuBase/GameMode/BP_PC_MenuBase.ServerUpdatePlayersList` _asbp_pc_menu_base (`self.Are Team Divided?`))))))

(fn `GetPlayersList`
  (returns (PlayersList :type "Array of PlayerController Object Reference"))
  (return (`self.PlayersList`)))

(fn `MenuLocker`
  (for _array_element (`self.PlayersList`)
    (bind _asbp_ps_menu_base (cast `/Game/KoH/Blueprints/MenuBase/GameMode/BP_PS_MenuBase` (`Controller.PlayerState` _array_element)))
    (bind _asbp_pc_menu_base (cast `/Game/KoH/Blueprints/MenuBase/GameMode/BP_PC_MenuBase` _array_element))
    (`/Game/KoH/Blueprints/MenuBase/GameMode/BP_PC_MenuBase.ServerHostLockMenu` _asbp_pc_menu_base (`.IsHost?_14_4BCB848D47565AE872CBD7ACBA4F051E` (break `/Game/KoH/Blueprints/MenuBase/Data/STR_MenuPlayerDesc` (`/Game/KoH/Blueprints/MenuBase/GameMode/BP_PS_MenuBase.GetMenuPlayerDesc` _asbp_ps_menu_base))))))

(fn `RefreshPlayersList`)

(fn `UserConstructionScript`)