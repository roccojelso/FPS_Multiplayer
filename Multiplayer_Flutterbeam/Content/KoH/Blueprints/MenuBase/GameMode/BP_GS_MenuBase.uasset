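; BP_GS_MenuBase is a menu base Blueprint, apparently a game state by its name, that holds menu-side match setup data.
; It stores a menu game description, a game mode index and a level index.
; Each value has a plain getter and setter, with no validation, events or other logic, and the construction script is empty.
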(fn `GetGameModeIndex`
  (returns (GameModeIndex :type Integer))
  (return (`self.GameModeIndex`)))

(fn `GetLevelIndex`
  (returns (LevelIndex :type Integer))
  (return (`self.LevelIndex`)))

(fn `GetMenuGameDesc`
  (returns (MenuGameDesc :type "/Game/KoH/Blueprints/MenuBase/Data/STR_MenuGameDesc Structure"))
  (return (`self.MenuGameDesc`)))

(fn `SetGameModeIndex`
  (params (GameModeIndex :type Integer))
  (set `self.GameModeIndex` GameModeIndex))

(fn `SetLevelIndex`
  (params (LevelIndex :type Integer))
  (set `self.LevelIndex` LevelIndex))

(fn `SetMenuGameDesc`
  (params (MenuGameDesc :type "/Game/KoH/Blueprints/MenuBase/Data/STR_MenuGameDesc Structure"))
  (set `self.MenuGameDesc` MenuGameDesc))

(fn `UserConstructionScript`)