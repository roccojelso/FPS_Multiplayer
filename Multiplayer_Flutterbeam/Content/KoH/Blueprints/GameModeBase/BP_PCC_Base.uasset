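; BP_PCC_Base is a player controller component in KoH that handles spawn facing and scoreboard requests.
; A multicast-named event sets the owning controller's control rotation to the supplied spawn rotation.
; Client-named open and close scoreboard events cast the controller's PlayerState to BP_PS_Base and forward the call to it.
; Every event casts its owner to PlayerController and silently stops if the cast fails.
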(event `MulticastSetControlRotationOnSpawn`
  (params (RotationOnSpawn :type "Rotator Structure"))
  (bind _asplayer_controller (cast `PlayerController` (`self.GetOwner`)))
  (`Controller.SetControlRotation` _asplayer_controller RotationOnSpawn))

(event `ClientOpenScoreBoard`
  (bind _asplayer_controller (cast `PlayerController` (`self.GetOwner`)))
  (bind _asbp_ps_base (cast `/Game/KoH/Blueprints/GameModeBase/BP_PS_Base` (`Controller.PlayerState` _asplayer_controller)))
  (`/Game/KoH/Blueprints/GameModeBase/BP_PS_Base.ClientOpenScoreboard` _asbp_ps_base))

(event `ClientCloseScoreBoard`
  (bind _asplayer_controller (cast `PlayerController` (`self.GetOwner`)))
  (bind _asbp_ps_base (cast `/Game/KoH/Blueprints/GameModeBase/BP_PS_Base` (`Controller.PlayerState` _asplayer_controller)))
  (`/Game/KoH/Blueprints/GameModeBase/BP_PS_Base.ClientCloseScoreboard` _asbp_ps_base))