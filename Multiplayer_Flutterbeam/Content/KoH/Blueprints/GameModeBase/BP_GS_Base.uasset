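; Base GameState for team matches, holding the game and match descriptions, match state, timers, scores, round count and winners.
; The game mode calls Server events, which store each value and mirror it to clients through Multicast events rather than RepNotify.
; Getters expose the state, while UpdateTeamScore clamps scores for counting up or down, with or without rounds.
; Team scores initialize with the match description and reinitialize on the waiting-new-round state, depending on win rules.
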(event `MulticastUpdateWaitingTimer`
  (params (`Current Timer Value` :type Integer))
  ;[1 1 1] UpdateWaitingTimer
  ;;[1 1 1] MulticastUpdateWaitingTimer
  (set `self.CurrentWaitingTimer` `Current Timer Value`))

(event `MulticastInitializeMGSGameDesc`
  (params (MGS_GameDesc :type "/Game/KoH/Blueprints/GameModeBase/Data/STR_BaseGameDesc Structure"))
  ;[1 1 1] INITIALIZE GAME STATE ON START MATCH
  ;;[1 1 1] MulticastInitializeMGSGameDesc
  (set `self.GameDesc` MGS_GameDesc))

(event `ServerInitializeBaseGameDesc`
  (params (MGS_GameDesc :type "/Game/KoH/Blueprints/GameModeBase/Data/STR_BaseGameDesc Structure"))
  ;[1 1 1] INITIALIZE GAME STATE ON START MATCH
  ;;[1 1 1] ServerInitializeMGSGameDesc // Using from game mode on initialize sequence
  (bind _output_get (set `self.GameDesc` MGS_GameDesc))
  (`self.MulticastInitializeMGSGameDesc` _output_get))

(event `ServerUpdateWaitingTimer`
  (params (CurrentWaitingTimer :type Integer))
  ;[1 1 1] UpdateWaitingTimer
  ;;[1 1 1] ServerUpdateWaitingTimer // Using from game mode
  (bind _output_get (set `self.CurrentWaitingTimer` CurrentWaitingTimer))
  (`self.MulticastUpdateWaitingTimer` _output_get)
  (`self.Log` (`KismetStringLibrary.Concat_StrStr` "WAITING: " (`KismetStringLibrary.Conv_IntToString` (`self.CurrentWaitingTimer`)))))

(event `ServerInitializeBaseMatchDesc`
  (params (MGS_MatchBaseDesc :type "/Game/KoH/Blueprints/GameModeBase/Data/STR_BaseMatchDesc Structure"))
  ;[1 1 1] INITIALIZE GAME STATE ON START MATCH
  ;;[1 1 1] ServerInitializeMGSGameDesc  // Using from game mode on initialize sequence
  (bind _output_get (set `self.BaseMatchDesc` MGS_MatchBaseDesc))
  (`self.MulticastInitializeBaseMatchDesc` _output_get)
  (`self.ServerInitializeTeamScore`))

(event `MulticastInitializeBaseMatchDesc`
  (params (MGS_MatchBaseDesc :type "/Game/KoH/Blueprints/GameModeBase/Data/STR_BaseMatchDesc Structure"))
  ;[1 1 1] INITIALIZE GAME STATE ON START MATCH
  ;;[1 1 1] MulticastInitializeMGSMatchBaseDesc
  (set `self.BaseMatchDesc` MGS_MatchBaseDesc))

(event `MulticastUpdateWaitingRoundStartTimer`
  (params (CurrentWaitingStartRoundTimerValue :type Integer))
  ;[1 1 1] UpdateWaitingRoundStartTimer
  ;;[1 1 1] MulticastUpdateWaitingRoundStartTimer
  (set `self.CurrentWaitingStartRoundTimer` CurrentWaitingStartRoundTimerValue))

(event `ServerUpdateWaitingRoundStartTimer`
  (params (CurrentWaitingStartRoundTimer :type Integer))
  ;[1 1 1] UpdateWaitingRoundStartTimer
  ;;[1 1 1] ServerUpdateWaitingRoundStartTimer  // Using from game mode
  (bind _output_get (set `self.CurrentWaitingStartRoundTimer` CurrentWaitingStartRoundTimer))
  (`self.MulticastUpdateWaitingRoundStartTimer` _output_get)
  (`self.Log` (`KismetStringLibrary.Concat_StrStr` "START: " (`KismetStringLibrary.Conv_IntToString` (`self.CurrentWaitingStartRoundTimer`)))))

(event `MulticastInitializeTeamScore`
  (params (CurrentRoundScoreTeam1 :type Integer) (CurrentRoundScoreTeam2 :type Integer))
  ;[1 1 1] INITIALIZE TEAM SCORES
  (set `self.CurrentRoundScoreTeam1` CurrentRoundScoreTeam1)
  (set `self.CurrentRoundScoreTeam2` CurrentRoundScoreTeam2))

(event `ServerInitializeTeamScore`
  (bind _match_score_limit (`self.GetMatchScoreLimit`))
  (bind _round_score_limit (`self.GetRoundScoreLimit`))
  ;[1 1 1] INITIALIZE TEAM SCORES
  (if (`self.GetWinByRoundCount?`)
    (if (`self.GetUseDecreasingMethod`)
      (if (`self.GetUseRoundSystem`)
        (set `self.CurrentRoundScoreTeam1` (`self.GetRoundScoreLimit`))
        (set `self.CurrentRoundScoreTeam2` (`self.GetRoundScoreLimit`))
        (`self.MulticastInitializeTeamScore` _round_score_limit _round_score_limit)
        (else
          (set `self.CurrentRoundScoreTeam1` (`self.GetMatchScoreLimit`))
          (set `self.CurrentRoundScoreTeam2` (`self.GetMatchScoreLimit`))
          (`self.MulticastInitializeTeamScore` _match_score_limit _match_score_limit)))
      (else
        (set `self.CurrentRoundScoreTeam1` 0)
        (set `self.CurrentRoundScoreTeam2` 0)
        (`self.MulticastInitializeTeamScore` 0)))
    (elif (`self.GetUseDecreasingMethod`)
      (`/Engine/EditorBlueprintResources/StandardMacros.DoOnce` false
        (:`Completed`
          (set `self.CurrentRoundScoreTeam1` (`self.GetMatchScoreLimit`))
          (set `self.CurrentRoundScoreTeam2` (`self.GetMatchScoreLimit`))
          (`self.MulticastInitializeTeamScore` (`self.CurrentRoundScoreTeam1`) (`self.CurrentRoundScoreTeam2`)))))))

(event `ServerUpdateMatchTimer`
  (params (CurrentRoundMatchTimer :type Integer))
  ;[1 1 1] UpdateRoundTimer
  ;;[1 1 1] ServerUpdateRoundMatchTimer  // Using from game mode
  (bind _output_get (set `self.CurrentMatchTimer` CurrentRoundMatchTimer))
  (`self.MulticastUpdateMatchTimer` _output_get)
  (`self.Log` (`KismetStringLibrary.Concat_StrStr` "ROUND TIME: " (`KismetStringLibrary.Conv_IntToString` (`self.CurrentMatchTimer`)))))

(event `MulticastUpdateMatchTimer`
  (params (CurrentRoundTimerValue :type Integer))
  ;[1 1 1] UpdateRoundTimer
  ;;[1 1 1] MulticastUpdateRoundTimer
  (set `self.CurrentMatchTimer` CurrentRoundTimerValue))

(event `MulticastUpdateMatchState`
  (params (`Match State` :type "/Game/KoH/Blueprints/GameModeBase/Data/E_MatchState Enum" :default "NewEnumerator0"))
  ;[1 1 1] UpdateMatchState
  ;;[1 1 1] MulticastUpdateMatchState
  (set `self.CurrentMatchState` `Match State`))

(event `ServerUpdateMGSMatchState`
  (params (`Match State` :type "/Game/KoH/Blueprints/GameModeBase/Data/E_MatchState Enum" :default "NewEnumerator0"))
  ;[1 1 1] UpdateMatchState
  ;;[1 1 1] ServerUpdateMGSMatchState  // Using from game mode
  (bind _output_get (set `self.CurrentMatchState` `Match State`))
  (`self.MulticastUpdateMatchState` _output_get)
  (`self.ServerHandleMatchState`)
  (`self.Log` (`KismetStringLibrary.Concat_StrStr` "UPDATE MATCH STATE - " (`|GetEnumeratorNameAsString` (`self.GetMatchState`)))))

(event `MulticastUpdateWaitNewRoundTimer`
  (params (CurrentWaitNewRoundTimerValue :type Integer))
  ;[1 1 1] UpdateWaitNewRoundTimer
  ;;[1 1 1] MulticastUpdateWaitNewRoundTimer
  (set `self.CurrentWaitNewRoundTimer` CurrentWaitNewRoundTimerValue))

(event `ServerUpdateWaitNewRoundTimer`
  (params (CurrentWaitNewRoundTimerValue :type Integer))
  ;[1 1 1] UpdateWaitNewRoundTimer
  ;;[1 1 1] ServerUpdateWaitNewRoundTimer  // Using from game mode
  (bind _output_get (set `self.CurrentWaitNewRoundTimer` CurrentWaitNewRoundTimerValue))
  (`self.MulticastUpdateWaitNewRoundTimer` _output_get)
  (`self.Log` (`KismetStringLibrary.Concat_StrStr` "WAIT NEW ROUND: " (`KismetStringLibrary.Conv_IntToString` (`self.CurrentWaitNewRoundTimer`)))))

(event `MulticastInitializeRoundCount`
  (params (CurrentRoundCount :type Integer))
  ;[1 1 1] InitializeRoundCount
  ;;[1 1 1] MulticastInitializeRoundCount
  (set `self.CurrentRoundCount` CurrentRoundCount))

(event `ServerInitializeRoundCount`
  (params (CurrentRoundCount :type Integer))
  ;[1 1 1] InitializeRoundCount
  ;;[1 1 1] ServerInitializeRoundCount // Using from game mode
  (bind _output_get (set `self.CurrentRoundCount` CurrentRoundCount))
  (`self.MulticastInitializeRoundCount` _output_get)
  (`self.Log` (`KismetStringLibrary.Concat_StrStr` "INCREACE ROUND COUNT: " (`KismetStringLibrary.Conv_IntToString` (`self.CurrentRoundCount`)))))

(event `ServerUpdateWinner`
  (params (CurrentMatchWinner :type "/Game/KoH/Blueprints/GameModeBase/Data/E_TeamWinner Enum" :default "NewEnumerator0"))
  ;[1 1 1] UPDATE WINNER
  (bind _output_get (set `self.CurrentMatchWinner` CurrentMatchWinner))
  (`self.MulticastUpdateWinner` _output_get)
  (`self.Log` (`KismetStringLibrary.Concat_StrStr` "MACTH WINNER: " (`|GetEnumeratorNameAsString` _output_get))))

(event `MulticastUpdateWinner`
  (params (CurrentMatchWinner :type "/Game/KoH/Blueprints/GameModeBase/Data/E_TeamWinner Enum" :default "NewEnumerator0"))
  ;[1 1 1] UPDATE WINNER
  (set `self.CurrentMatchWinner` CurrentMatchWinner))

(event `ServerHandleMatchState`
  ;[1 1 1] HANDLE MATCH STATE
  (switch `/Game/KoH/Blueprints/GameModeBase/Data/E_MatchState` (`self.CurrentMatchState`)
    (:`NewEnumerator4`
      (`self.ServerInitializeTeamScore`))))

(event `ServerUpdateWaitingEndGameTimer`
  (params (CurrentWaitEndGameTimerValue :type Integer))
  ;[1 1 1] UpdateWaitingEndGameTimer
  ;;[1 1 1] ServerUpdateWaitingEndGameTimer // Using from game mode
  (bind _output_get (set `self.CurrentWaitEndGameTimer` CurrentWaitEndGameTimerValue))
  (`self.MulticastUpdateWaitingEndGameTimer` _output_get)
  (`self.Log` (`KismetStringLibrary.Concat_StrStr` "WAIT END GAME: " (`KismetStringLibrary.Conv_IntToString` (`self.CurrentWaitEndGameTimer`)))))

(event `MulticastUpdateWaitingEndGameTimer`
  (params (CurrentWaitEndGameTimerValue :type Integer))
  ;[1 1 1] UpdateWaitingEndGameTimer
  ;;[1 1 1] MulticastUpdateWaitingEndGameTimer
  (set `self.CurrentWaitEndGameTimer` CurrentWaitEndGameTimerValue))

(event `ServerUpdateWinRoundCount`
  (params (`To Team` :type "/Game/KoH/Blueprints/GameModeBase/Data/E_TeamWinner Enum" :default "NewEnumerator0"))
  ;[1 1 1] UPDATE WIN ROUND COUNT
  (bind _output_get (set `self.CurrentRoundWinner` `To Team`))
  (`self.Log` (`|GetEnumeratorNameAsString` _output_get))
  (switch `/Game/KoH/Blueprints/GameModeBase/Data/E_TeamWinner` _output_get
    (:`NewEnumerator0`
      (bind _final_round_count (`self.UpdateWinRoundCountTeam` (`self.CurrentWinRoundCountTeam1`) 1))
      (set `self.CurrentWinRoundCountTeam1` _final_round_count))
    (:`NewEnumerator1`
      (bind _final_round_count_2 (`self.UpdateWinRoundCountTeam` (`self.CurrentWinRoundCountTeam2`) 1))
      (set `self.CurrentWinRoundCountTeam2` _final_round_count_2)))
  (`self.Log` (`KismetStringLibrary.Concat_StrStr` "ROUND WIN COUNT // " "TEAM 1: " (`KismetStringLibrary.Conv_IntToString` (`self.CurrentWinRoundCountTeam1`)) " // " "TEAM 2: " (`KismetStringLibrary.Conv_IntToString` (`self.CurrentWinRoundCountTeam2`))))
  (`self.MulticastUpdateWinRoundCount` (`self.CurrentWinRoundCountTeam1`) (`self.CurrentWinRoundCountTeam2`) (`self.CurrentRoundWinner`)))

(event `MulticastUpdateWinRoundCount`
  (params (CurrentWinRoundCountTeam1 :type Integer) (CurrentWinRoundCountTeam2 :type Integer) (CurrentRoundWinner :type "/Game/KoH/Blueprints/GameModeBase/Data/E_TeamWinner Enum" :default "NewEnumerator0"))
  ;[1 1 1] UPDATE WIN ROUND COUNT
  (set `self.CurrentWinRoundCountTeam1` CurrentWinRoundCountTeam1)
  (set `self.CurrentWinRoundCountTeam2` CurrentWinRoundCountTeam2)
  (set `self.CurrentRoundWinner` CurrentRoundWinner))

(event `ServerUpdateNewRoundState`
  (params (`IsNewRound?` :type Boolean))
  ;[1 1 1] UPDATE NEW ROUND STATE
  (bind _output_get (set `self.IsNewRound?` `IsNewRound?`))
  (`self.MulticastUpdateNewRoundState` _output_get))

(event `MulticastUpdateNewRoundState`
  (params (`IsNewRound?` :type Boolean))
  ;[1 1 1] UPDATE NEW ROUND STATE
  (set `self.IsNewRound?` `IsNewRound?`))

(event `MulticastUpdateTeamMatchScores`
  (params (MatchScoreTeam1 :type Integer) (MatchScoreTeam2 :type Integer))
  ;[1 1 1] Update Team Match Scores
  ;;[1 1 1] MulticastUpdateTeamMatchScores
  (set `self.CurrentRoundScoreTeam1` MatchScoreTeam1)
  (set `self.CurrentRoundScoreTeam2` MatchScoreTeam2))

(event `ServerUpdateTeamMatchScores`
  (params (`For Team` :type "/Game/KoH/Blueprints/GameModeBase/Data/E_ModeTeamType Enum" :default "NewEnumerator0") (Scores :type Integer))
  ;[1 1 1] Update Team Match Scores
  ;;[1 1 1] ServerUpdateTeamMatchScores  // Using from game mode
  (switch `/Game/KoH/Blueprints/GameModeBase/Data/E_ModeTeamType` `For Team`
    (:`NewEnumerator1`
      (bind _updated_team_score (`self.UpdateTeamScore` (`self.CurrentRoundScoreTeam1`) Scores))
      (set `self.CurrentRoundScoreTeam1` _updated_team_score))
    (:`NewEnumerator2`
      (bind _updated_team_score_2 (`self.UpdateTeamScore` (`self.CurrentRoundScoreTeam2`) Scores))
      (set `self.CurrentRoundScoreTeam2` _updated_team_score_2)))
  (`self.MulticastUpdateTeamMatchScores` (`self.CurrentRoundScoreTeam1`) (`self.CurrentRoundScoreTeam2`))
  (`self.Log` (`KismetStringLibrary.Concat_StrStr` "M SCORES TEAM 1: " (`KismetStringLibrary.Conv_IntToString` (`self.CurrentRoundScoreTeam1`)) " // " "M SCORES TEAM 2: " (`KismetStringLibrary.Conv_IntToString` (`self.CurrentRoundScoreTeam2`)))))

(fn `GetAutoSpawn`
  (returns (`AutoSpawn?` :type Boolean))
  (locals (loc_round_score_limit :type Integer :default 0))
  (return (`.AutoSpawn?_28_471834DC4F38F2D4EB040B82B24C34A0` (break `/Game/KoH/Blueprints/GameModeBase/Data/STR_BaseMatchDesc` (`self.BaseMatchDesc`)))))

(fn `GetCurrentMatchScoreTeam1`
  (returns (CurrentMatchScoreTeam1 :type Integer))
  (return (`self.CurrentRoundScoreTeam1`)))

(fn `GetCurrentMatchScoreTeam2`
  (returns (CurrentMatchScoreTeam2 :type Integer))
  (return (`self.CurrentRoundScoreTeam2`)))

(fn `GetCurrentMatchWinner`
  (returns (CurrentMatchWinner :type "/Game/KoH/Blueprints/GameModeBase/Data/E_TeamWinner Enum"))
  (return (`self.CurrentMatchWinner`)))

(fn `GetCurrentRoundCount`
  (returns (CurrentRoundCount :type Integer))
  (return (`self.CurrentRoundCount`)))

(fn `GetCurrentRoundWinner`
  (returns (CurrentRoundWinner :type "/Game/KoH/Blueprints/GameModeBase/Data/E_TeamWinner Enum"))
  (return (`self.CurrentRoundWinner`)))

(fn `GetCurrentWinRoundCountTeam1`
  (returns (CurrentWinRoundCountTeam1 :type Integer))
  (return (`self.CurrentWinRoundCountTeam1`)))

(fn `GetCurrentWinRoundCountTeam2`
  (returns (CurrentWinRoundCountTeam2 :type Integer))
  (return (`self.CurrentWinRoundCountTeam2`)))

(fn `GetEndGameTimer`
  (returns (CurrentWaitEndGameTimer :type Integer))
  (return (`self.CurrentWaitEndGameTimer`)))

(fn `GetGameModeType`
  (returns (`Game Mode Type` :type "/Game/KoH/Blueprints/GameModeBase/Data/E_GameModesType Enum"))
  (return (`.GameModeType_10_5D3971224C3AD9477D1763938254A2EA` (break `/Game/KoH/Blueprints/GameModeBase/Data/STR_BaseGameDesc` (`self.GameDesc`)))))

(fn `GetIsNewRound`
  (returns (`IsNewRound?` :type Boolean))
  (return (`self.IsNewRound?`)))

(fn `GetMatchBeginsTimer`
  (returns (CurrentWaitingStartRoundTimer :type Integer))
  (return (`self.CurrentWaitingStartRoundTimer`)))

(fn `GetMatchRoundTimer`
  (returns (CurrentRoundMatchTimer :type Integer))
  (return (`self.CurrentMatchTimer`)))

(fn `GetMatchScoreLimit`
  (returns (`Match Score Limit` :type Integer))
  (return (`.MatchScoreLimit_10_80D9222ABB4CC19196423292C5ED4E44` (break `/Game/KoH/Blueprints/GameModeBase/Data/STR_BaseMatchDesc` (`self.BaseMatchDesc`)))))

(fn `GetMatchState`
  (returns (`Match State` :type "/Game/KoH/Blueprints/GameModeBase/Data/E_MatchState Enum"))
  (return (`self.CurrentMatchState`)))

(fn `GetMatchTimeLimit`
  (returns (`Match Time Limit` :type Integer))
  (return (`.MatchTimeLimit_6_31243999BF450B68D7D9A2A4FD6B83EF` (break `/Game/KoH/Blueprints/GameModeBase/Data/STR_BaseMatchDesc` (`self.BaseMatchDesc`)))))

(fn `GetMaxRoundsCount`
  (returns (`Max Rounds Count` :type Integer))
  (return (`.MaxRoundsCount_20_BB846466454387DD459F958F375C8169` (break `/Game/KoH/Blueprints/GameModeBase/Data/STR_BaseMatchDesc` (`self.BaseMatchDesc`)))))

(fn `GetNewRoundTimer`
  (returns (CurrentWaitNewRoundTimer :type Integer))
  (return (`self.CurrentWaitNewRoundTimer`)))

(fn `GetRespawnTime`
  (returns (`Respawn Time` :type Integer))
  (return (`.RespawnTime_24_A856E47241BA2BDC63020E8B9DD8811D` (break `/Game/KoH/Blueprints/GameModeBase/Data/STR_BaseMatchDesc` (`self.BaseMatchDesc`)))))

(fn `GetRoundScoreLimit`
  (returns (`Round Score Limit` :type Integer))
  (locals (loc_round_score_limit :type Integer :default 0))
  (bind (_matchtimelimit _matchscorelimit _usemsdecreasingmethod_ _useroundsystem_ _winbyroundcount_ _maxroundscount) (break `/Game/KoH/Blueprints/GameModeBase/Data/STR_BaseMatchDesc` (`self.BaseMatchDesc`)))
  (if _winbyroundcount_
    (set `local.loc_round_score_limit` _matchscorelimit)
    (else
      (set `local.loc_round_score_limit` (/ _matchscorelimit _maxroundscount))))
  (return (`local.loc_round_score_limit`)))

(fn `GetUseDecreasingMethod`
  (returns (`Use Decreasing Method?` :type Boolean))
  (return (`.UseMSDecreasingMethod?_21_1D0FBF0D4C4B969901D0ABB19D694B53` (break `/Game/KoH/Blueprints/GameModeBase/Data/STR_BaseMatchDesc` (`self.BaseMatchDesc`)))))

(fn `GetUseRoundSystem`
  (returns (`Use Round System?` :type Boolean))
  (return (`.UseRoundSystem?_19_FEBC82EC8F4DC171F562EFAC0B9B033C` (break `/Game/KoH/Blueprints/GameModeBase/Data/STR_BaseMatchDesc` (`self.BaseMatchDesc`)))))

(fn `GetWaitingTimer`
  (returns (CurrentWaitingTimer :type Integer))
  (return (`self.CurrentWaitingTimer`)))

(fn `GetWinByRoundCount?`
  (returns (`Win By Round Count?` :type Boolean))
  (return (`.WinByRoundCount?_26_39F44DC5423A70AE347858AEA7467737` (break `/Game/KoH/Blueprints/GameModeBase/Data/STR_BaseMatchDesc` (`self.BaseMatchDesc`)))))

(fn `Log`
  (params (Text :type String))
  (if (`self.Draw Debug Log?`)
    (`KismetSystemLibrary.PrintString` (`KismetStringLibrary.Concat_StrStr` "BASE GS: " Text) true true (struct :`R` 0.371051 :`G` 1.0 :`A` 1.0) 4.0)))

(fn `UpdateTeamScore`
  (params (`Current Team Score` :type Integer) (`Added Score` :type Integer))
  (returns (`Updated Team Score` :type Integer))
  (locals (loc_team_score :type Integer :default 1) (loc_pre_new_value :type Integer :default 0) (loc_added_score :type Integer))
  (set `local.loc_team_score` `Current Team Score`)
  (set `local.loc_added_score` `Added Score`)
  (if (`self.GetUseDecreasingMethod`)
    (set `local.loc_pre_new_value` (- (`local.loc_team_score`) (`local.loc_added_score`)))
    (if (`self.GetUseRoundSystem`)
      (if (`self.GetWinByRoundCount?`)
        (if (>= (`local.loc_pre_new_value`) (`self.GetRoundScoreLimit`))
          (set `local.loc_team_score` 0)
          (else
            (set `local.loc_team_score` (`local.loc_pre_new_value`))))
        (elif (>= (`local.loc_pre_new_value`) (- (`self.GetMaxRoundsCount`) (* (`self.GetRoundScoreLimit`) (`self.CurrentRoundCount`))))
          (set `local.loc_team_score` (`local.loc_pre_new_value`))
          (else
            (set `local.loc_team_score` (- (`self.GetMaxRoundsCount`) (* (`self.GetRoundScoreLimit`) (`self.CurrentRoundCount`)))))))
      (elif (<= (`local.loc_pre_new_value`) 0)
        (set `local.loc_team_score` 0)
        (else
          (set `local.loc_team_score` (`local.loc_pre_new_value`)))))
    (else
      ;[1 1 1] Comment
      (set `local.loc_pre_new_value` (+ (`local.loc_added_score`) (`local.loc_team_score`)))
      (if (`self.GetUseRoundSystem`)
        (if (>= (`local.loc_pre_new_value`) (* (`self.GetRoundScoreLimit`) (`self.CurrentRoundCount`)))
          (set `local.loc_team_score` (* (`self.GetRoundScoreLimit`) (`self.CurrentRoundCount`)))
          (else
            (set `local.loc_team_score` (`local.loc_pre_new_value`))))
        (elif (>= (`local.loc_pre_new_value`) (`self.GetMatchScoreLimit`))
          (set `local.loc_team_score` (`self.GetMatchScoreLimit`))
          (else
            (set `local.loc_team_score` (`local.loc_pre_new_value`)))))))
  (return (`local.loc_team_score`)))

(fn `UpdateWinRoundCountTeam`
  (params (`Current Win Round Count` :type Integer) (`Added Value` :type Integer))
  (returns (`Final Round Count` :type Integer))
  (locals (loc_current :type Integer) (loc_added_value :type Integer))
  (set `local.loc_current` `Current Win Round Count`)
  (set `local.loc_added_value` `Added Value`)
  (bind _output_get (set `local.loc_current` (+ (`local.loc_current`) (`local.loc_added_value`))))
  (return _output_get))

(fn `UserConstructionScript`)