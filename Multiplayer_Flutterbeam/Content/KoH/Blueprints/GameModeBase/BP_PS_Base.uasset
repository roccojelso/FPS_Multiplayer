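; Base multiplayer PlayerState that carries each player's name, team, kill/death/score stats and dead state through match, round and respawn flow.
; Paired Server, Client and Multicast events drive the logic, replicating stats, switching input and swapping match, HUD and end-game widgets.
; Player info comes from the menu GameInstance after fixed startup delays.
; Death starts a server countdown that enables manual or automatic respawn through the GameMode's CommonRespawn.
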(event `self.ReceiveBeginPlay`
  ;[1 1 1] Initialize
  ;;[1 1 1] EVENT BEGIN PLAY
  (`|ExecutionSequence`
    (:`then_0`
      (`KismetSystemLibrary.Delay` 7.1)
      (`/Engine/EditorBlueprintResources/ActorMacros.Switch Has Authority`
        (:`Authority`
          (bind _asbp_gs_base (cast `/Game/KoH/Blueprints/GameModeBase/BP_GS_Base` (`GameplayStatics.GetGameState`)))
          (switch `/Game/KoH/Blueprints/GameModeBase/Data/E_MatchState` (`/Game/KoH/Blueprints/GameModeBase/BP_GS_Base.GetMatchState` _asbp_gs_base)
            (:`NewEnumerator0`
              (`self.ClientOnMatchInitializeState`))))))
    (:`then_1`
      (`KismetSystemLibrary.Delay` 4.0)
      (`/Engine/EditorBlueprintResources/ActorMacros.Switch Has Authority`
        (:`Authority`
          (`self.ClientInitializePlayerProperties`))))))

(event `ServerMatchStart`
  ;[1 1 1] Common Flow
  ;;[1 1 1] ON MATCH START / ON START NEW ROUND
  (`self.ClientMatchStart`))

(event `ClientMatchStart`
  ;[1 1 1] Common Flow
  ;;[1 1 1] ON MATCH START / ON START NEW ROUND
  (`Widget.RemoveFromParent` (`self.WaitingMatchScreenRef`))
  (`/Engine/EditorBlueprintResources/StandardMacros.IsValid` (`self.NewRoundScreenRef`)
    (:`Is Valid`
      (`Widget.RemoveFromParent` (`self.NewRoundScreenRef`)))
    (:`Is Not Valid`
      _))
  (bind _returnvalue (`|CreateWidget` (`self.MatchBeginsScreen`) (`GameplayStatics.GetPlayerController` 0)))
  (bind _output_get (set `self.MatchBeginsScreenRef` _returnvalue))
  (`UserWidget.AddToViewport` _output_get 0)
  (bind _returnvalue_2 (`|CreateWidget` (`self.MainPlayerHUD`) (`GameplayStatics.GetPlayerController` 0)))
  (bind _output_get_2 (set `self.MainPlayerHUDRef` _returnvalue_2))
  (`UserWidget.AddToViewport` _output_get_2 0)
  (`self.ClientCreateAdditionalWidgets`)
  (`self.TriggerClientCreateAdditionalWidgets`)
  (`self.DrawDebugLog` "Match Start"))

(event `ClientCreateAdditionalWidgets`
  ;[1 1 1] Common Flow
  ;;[1 1 1] CREATE & REMOVE ADD WIDGETS
)

(event `ClientRemoveAdditionalWidgets`
  ;[1 1 1] Common Flow
  ;;[1 1 1] CREATE & REMOVE ADD WIDGETS
)

(event `ClientOnMatchInitializeState`
  ;[1 1 1] Initialize
  ;;[1 1 1] CLIENT ON MATCH INITIALIZE STATE
  (bind _returnvalue (`|CreateWidget` (`self.WaitingMatchScreen`) (`GameplayStatics.GetPlayerController` 0)))
  (bind _output_get (set `self.WaitingMatchScreenRef` _returnvalue))
  (`UserWidget.AddToViewport` _output_get 0)
  (`self.DrawDebugLog` "ClientOnMatchInitializeState"))

(event `ClientRoundStart`
  ;[1 1 1] Common Flow
  ;;[1 1 1] ROUND START
  (`Widget.RemoveFromParent` (`self.MatchBeginsScreenRef`))
  (bind _asplayer_controller (cast `PlayerController` (`self.GetOwner`)))
  (`self.EnableInput` (`self.GetOwner`) _asplayer_controller)
  (`self.DrawDebugLog` "Round Start"))

(event `ServerRoundStart`
  ;[1 1 1] Common Flow
  ;;[1 1 1] ROUND START
  (`self.ClientRoundStart`))

(event `ServerInitializePlayerProperties`
  (params (PlayerProperties :type "/Game/KoH/Blueprints/GameModeBase/Data/STR_BasePlayerDesc Structure"))
  ;[1 1 1] Initialize
  ;;[1 1 1] CLIENT INITIALIZE PLAYER PROPERTIES
  ;;;[1 1 1] ServerInitializePlayerProperties
  (bind _output_get (set `self.BasePlayerDesc` PlayerProperties))
  (`self.MulticastInitializePlayerProperties` _output_get))

(event `ClientInitializePlayerProperties`
  ;[1 1 1] Initialize
  ;;[1 1 1] CLIENT INITIALIZE PLAYER PROPERTIES
  ;;;[1 1 1] ClientInitializePlayerProperties
  (`|ExecutionSequence`
    (:`then_0`
      (`self.InitializeFromGameIns`)
      (`self.DrawDebugLog` "Initialize"))
    (:`then_1`
      (bind _asplayer_controller (cast `PlayerController` (`self.GetOwner`)))
      (`self.DisableInput` (`self.GetOwner`) _asplayer_controller)
      (`WidgetBlueprintLibrary.SetInputMode_GameOnly` _asplayer_controller))))

(event `MulticastInitializePlayerProperties`
  (params (PlayerProperties :type "/Game/KoH/Blueprints/GameModeBase/Data/STR_BasePlayerDesc Structure"))
  ;[1 1 1] Initialize
  ;;[1 1 1] CLIENT INITIALIZE PLAYER PROPERTIES
  ;;;[1 1 1] MulticastInitializePlayerProperties
  (set `self.BasePlayerDesc` PlayerProperties))

(event `ServerWaitNewRound`
  ;[1 1 1] Common Flow
  ;;[1 1 1] NEW ROUND
  (`self.ClientWaitNewRound`))

(event `ClientWaitNewRound`
  ;[1 1 1] Common Flow
  ;;[1 1 1] NEW ROUND
  (bind _asplayer_controller (cast `PlayerController` (`self.GetOwner`)))
  (`self.DisableInput` (`self.GetOwner`) _asplayer_controller)
  (`Widget.RemoveFromParent` (`self.MainPlayerHUDRef`))
  (`self.ClientRemoveAdditionalWidgets`)
  (`self.TriggerClientRemoveAdditionalWidgets`)
  (bind _returnvalue (`|CreateWidget` (`self.NewRoundScreen`) (`GameplayStatics.GetPlayerController` 0)))
  (bind _output_get (set `self.NewRoundScreenRef` _returnvalue))
  (`UserWidget.AddToViewport` _output_get 0)
  (`self.DrawDebugLog` "Wait New Round"))

(event `ServerWaitEndMatch`
  ;[1 1 1] Common Flow
  ;;[1 1 1] END GAME
  (`self.ClientWaitEndMatch`))

(event `ClientWaitEndMatch`
  ;[1 1 1] Common Flow
  ;;[1 1 1] END GAME
  (bind _asplayer_controller (cast `PlayerController` (`self.GetOwner`)))
  (`self.DisableInput` (`self.GetOwner`) _asplayer_controller)
  (`Widget.RemoveFromParent` (`self.MainPlayerHUDRef`))
  (`self.ClientRemoveAdditionalWidgets`)
  (`self.TriggerClientRemoveAdditionalWidgets`)
  (bind _returnvalue (`|CreateWidget` (`self.EndGameScreen`) (`GameplayStatics.GetPlayerController` 0)))
  (bind _output_get (set `self.EndGameScreenRef` _returnvalue))
  (`UserWidget.AddToViewport` _output_get 0)
  (`self.DrawDebugLog` "Wait End Match"))

(event `ServerSetTeamForPlayer`
  (params (Team :type "/Game/KoH/Blueprints/GameModeBase/Data/E_ModeTeamType Enum" :default "NewEnumerator0"))
  ;[1 1 1] Misc
  ;;[1 1 1] FOR DICRECT LAUNCH
  (`self.SetTeam` Team)
  (`self.MulticastSetTeamForPlayer` Team))

(event `MulticastSetTeamForPlayer`
  (params (Team :type "/Game/KoH/Blueprints/GameModeBase/Data/E_ModeTeamType Enum" :default "NewEnumerator0"))
  ;[1 1 1] Misc
  ;;[1 1 1] FOR DICRECT LAUNCH
  (`self.SetTeam` Team))

(event `ServerPlayerLogin`
  (params (`MP Player State` :type "/Game/KoH/Blueprints/GameModeBase/BP_PS_Base Object Reference"))
  ;[1 1 1] Misc
  ;;[1 1 1] Other Player Login
  (`self.DrawDebugLog` (`KismetSystemLibrary.GetDisplayName` `MP Player State`))
  (`self.ClientPlayerLogin` `MP Player State`))

(event `ClientPlayerLogin`
  (params (`MP Player State` :type "/Game/KoH/Blueprints/GameModeBase/BP_PS_Base Object Reference"))
  ;[1 1 1] Misc
  ;;[1 1 1] Other Player Login
  (`self.DrawDebugLog` (`KismetStringLibrary.Concat_StrStr` "Player Join to Game: " (`KismetSystemLibrary.GetDisplayName` `MP Player State`))))

(event `ServerPlayerDead`
  ;[1 1 1] Dead & Kill
  ;;[1 1 1] PLAYER DEAD
  (`self.ServerUpdateDeadState` true)
  (`self.ServerUpdateDeathCount` 1)
  (bind _asplayer_controller (cast `PlayerController` (`self.GetOwner`)))
  (`self.DisableInput` (`self.GetOwner`) _asplayer_controller)
  (`|ExecutionSequence`
    (:`then_0`
      (`KismetSystemLibrary.Delay` (`self.DelayBeforeRespawnScreen`))
      (`self.ClientPlayerDead`))
    (:`then_1`
      (`self.ServerStartSelfRespawnTimer`))
    (:`then_2`
      (`/Engine/EditorBlueprintResources/StandardMacros.IsValid` (`self.MainPlayerHUDRef`)
        (:`Is Valid`
          (`Widget.RemoveFromParent` (`self.MainPlayerHUDRef`))
          (`self.ClientRemoveAdditionalWidgets`))))))

(event `ClientPlayerDead`
  ;[1 1 1] Dead & Kill
  ;;[1 1 1] PLAYER DEAD
  (`|ExecutionSequence`
    (:`then_0`
      (`self.TriggerClientOpenRespawnScreen`)
      (`self.DrawDebugLog` "ClientPlayerDead"))
    (:`then_1`
      (bind _asbp_gs_base (cast `/Game/KoH/Blueprints/GameModeBase/BP_GS_Base` (`GameplayStatics.GetGameState`)))
      (if (not (`/Game/KoH/Blueprints/GameModeBase/BP_GS_Base.GetAutoSpawn` _asbp_gs_base))
        (bind _asplayer_controller (cast `PlayerController` (`self.GetOwner`)))
        (`WidgetBlueprintLibrary.SetInputMode_UIOnlyEx` _asplayer_controller null)
        (set `PlayerController.bShowMouseCursor` true _asplayer_controller)))
    (:`then_2`
      (`self.TriggerClientRemoveAdditionalWidgets`))))

(event `ServerPlayerCanRespawn`
  ;[1 1 1] Dead & Kill
  ;;[1 1 1] CAN RESPAWN
  (bind _output_get (set `self.Can Respawn` true))
  (`self.ClientPlayerCanRespawn` _output_get))

(event `ClientCommonPlayerDead`
  (params (`Dead Player State` :type "/Game/KoH/Blueprints/GameModeBase/BP_PS_Base Object Reference") (`Causer Player State` :type "/Game/KoH/Blueprints/GameModeBase/BP_PS_Base Object Reference") (`Kill Info` :type "/Game/KoH/Blueprints/GameModeBase/Data/STR_KIllInfo Structure"))
  ;[1 1 1] Dead & Kill
  ;;[1 1 1] CommonPlayerDead
  (`self.ClientAddKillFragListEvent` `Causer Player State` `Dead Player State`)
  (`self.DrawDebugLog` "CommonPlayerDead"))

(event `ServerCommonPlayerDead`
  (params (`Dead Player State` :type "/Game/KoH/Blueprints/GameModeBase/BP_PS_Base Object Reference") (`Causer Player State` :type "/Game/KoH/Blueprints/GameModeBase/BP_PS_Base Object Reference") (`Kill Info` :type "/Game/KoH/Blueprints/GameModeBase/Data/STR_KIllInfo Structure"))
  ;[1 1 1] Dead & Kill
  ;;[1 1 1] CommonPlayerDead
  (`self.ClientCommonPlayerDead` `Dead Player State` `Causer Player State` `Kill Info`))

(event `ClientPlayerCanRespawn`
  (params (`Can Respawn` :type Boolean))
  ;[1 1 1] Dead & Kill
  ;;[1 1 1] CAN RESPAWN
)

(event `ServerPlayerLogout`
  (params (`MP Player State` :type "/Game/KoH/Blueprints/GameModeBase/BP_PS_Base Object Reference"))
  ;[1 1 1] Misc
  ;;[1 1 1] Other Player Logout
  (`self.ClientPlayerLogout` `MP Player State`))

(event `ClientPlayerLogout`
  (params (`MP Player State` :type "/Game/KoH/Blueprints/GameModeBase/BP_PS_Base Object Reference"))
  ;[1 1 1] Misc
  ;;[1 1 1] Other Player Logout
  (`self.DrawDebugLog` (`KismetStringLibrary.Concat_StrStr` "Player Logout from Game: " (`KismetSystemLibrary.GetDisplayName` `MP Player State`))))

(event `ServerUpdateDeadState`
  (params (IsDead :type Boolean))
  ;[1 1 1] Dead & Kill
  ;;[1 1 1] UPDATE DEAD STATE
  (bind _output_get (set `self.IsDead` IsDead))
  (`self.ClientUpdateDeadState` _output_get))

(event `ClientUpdateDeadState`
  (params (IsDead :type Boolean))
  ;[1 1 1] Dead & Kill
  ;;[1 1 1] UPDATE DEAD STATE
  (set `self.IsDead` IsDead))

(event `ServerTerminatePawn`
  ;[1 1 1] Dead & Kill
  ;;[1 1 1] ServerTerminatePawn
  (`self.TriggerTerminatePawn`))

(event `ClientOpenScoreboard`
  ;[1 1 1] Misc
  ;;[1 1 1] SCOREBOARD
  (`Widget.SetVisibility` (`self.MainPlayerHUDRef`) "Hidden")
  (`Widget.SetVisibility` (`self.MatchBeginsScreenRef`) "Hidden")
  (`self.TriggerClientOpenScoreboard`))

(event `ClientCloseScoreboard`
  ;[1 1 1] Misc
  ;;[1 1 1] SCOREBOARD
  (`Widget.SetVisibility` (`self.MainPlayerHUDRef`) "Visible")
  (`Widget.SetVisibility` (`self.MatchBeginsScreenRef`) "Visible")
  (`self.TriggerClientCloseScoreboard`))

(event `ServerStartSelfRespawnTimer`
  ;[1 1 1] Dead & Kill
  ;;[1 1 1] RESPAWN SELF TIMER
  (bind _asbp_gs_base (cast `/Game/KoH/Blueprints/GameModeBase/BP_GS_Base` (`GameplayStatics.GetGameState`)))
  (set `self.RespawnTimerValue` (`/Game/KoH/Blueprints/GameModeBase/BP_GS_Base.GetRespawnTime` _asbp_gs_base))
  (if (== (`self.RespawnTimerValue`) 0)
    (`self.ServerPlayerCanRespawn`)
    (else
      (bind _returnvalue (`KismetSystemLibrary.K2_SetTimerDelegate` (delegate `ServerRespawnTimer`) 1.0 true))
      (set `self.SelfRespawnTimer` _returnvalue))))

(event `ClientRespawnTimer`
  (params (RespawnTimerValue :type Integer))
  ;[1 1 1] Dead & Kill
  ;;[1 1 1] RESPAWN SELF TIMER
  (set `self.RespawnTimerValue` RespawnTimerValue))

(event `ServerRespawnTimer`
  ;[1 1 1] Dead & Kill
  ;;[1 1 1] RESPAWN SELF TIMER
  (bind _result (`/Engine/EditorBlueprintResources/StandardMacros.DecrementInt` (`self.RespawnTimerValue`))
    (:`  `
      (`self.ClientRespawnTimer` _result)
      (if (== (`self.RespawnTimerValue`) 0)
        (`KismetSystemLibrary.K2_PauseTimerHandle` (`self.SelfRespawnTimer`))
        (`self.ServerPlayerCanRespawn`)
        (bind _asbp_gs_base (cast `/Game/KoH/Blueprints/GameModeBase/BP_GS_Base` (`GameplayStatics.GetGameState`)))
        (if (`/Game/KoH/Blueprints/GameModeBase/BP_GS_Base.GetAutoSpawn` _asbp_gs_base)
          (`|ExecutionSequence`
            (:`then_0`
              (`self.ClientCloseRespawnScreen`)
              (set `self.Can Respawn` false))
            (:`then_1`
              (`self.ServerTriggerRespawn`))))))))

(event `ClientCloseRespawnScreen`
  ;[1 1 1] Dead & Kill
  ;;[1 1 1] CLOSE RESPAWN SCREEN
  (`self.TriggerClientCloseRespawnScreen`)
  (bind _asplayer_controller (cast `PlayerController` (`self.GetOwner`)))
  (`WidgetBlueprintLibrary.SetInputMode_GameOnly` _asplayer_controller)
  (set `PlayerController.bShowMouseCursor` false _asplayer_controller))

(event `ClientAddScoreEventOnHUD`
  (params (Scores :type Integer) (`Desc Text` :type Text))
  ;[1 1 1] Misc
  ;;[1 1 1] SCORE EVENT
  (bind _aswbp_main_player_hud (cast `/Game/KoH/Blueprints/UIBase/WBP_MainPlayerHUD` (`self.MainPlayerHUDRef`)))
  (`/Game/KoH/Blueprints/UIBase/WBP_MainPlayerHUD.AddScoreEvent` _aswbp_main_player_hud Scores `Desc Text`))

(event `ServerPlayerKilledOtherPlayer`
  ;[1 1 1] Dead & Kill
  ;;[1 1 1] PLAYER KILLED ENEMY
  (`self.ClientPlayerKilledOtherPlayer`)
  (`self.ServerUpdateKillCount` 1)
  (`self.ServerUpdateScores` 100))

(event `ClientPlayerKilledOtherPlayer`
  ;[1 1 1] Dead & Kill
  ;;[1 1 1] PLAYER KILLED ENEMY
  (`self.ClientAddScoreEventOnHUD` 100 "Kill Enemy")
  (`self.DrawDebugLog` "Player Killed Other Player"))

(event `ServerTriggerRespawn`
  ;[1 1 1] Dead & Kill
  ;;[1 1 1] TRIGGER RESPAWN
  (bind _asplayer_controller (cast `PlayerController` (`self.GetOwner`)))
  (`self.EnableInput` (`self.GetOwner`) _asplayer_controller)
  (`self.ServerUpdateDeadState` false)
  (set `self.Can Respawn` false)
  (`|ExecutionSequence`
    (:`then_0`
      (bind _asbp_gs_base (cast `/Game/KoH/Blueprints/GameModeBase/BP_GS_Base` (`GameplayStatics.GetGameState`)))
      (switch `/Game/KoH/Blueprints/GameModeBase/Data/E_MatchState` (`/Game/KoH/Blueprints/GameModeBase/BP_GS_Base.GetMatchState` _asbp_gs_base)
        (:`NewEnumerator2`
          (bind _asbp_gm_base (cast `/Game/KoH/Blueprints/GameModeBase/BP_GM_Base` (`GameplayStatics.GetGameMode`)))
          (`/Game/KoH/Blueprints/GameModeBase/BP_GM_Base.CommonRespawn` _asbp_gm_base self))))
    (:`then_1`
      (bind _asbp_gs_base_2 (cast `/Game/KoH/Blueprints/GameModeBase/BP_GS_Base` (`GameplayStatics.GetGameState`)))
      (if (`/Game/KoH/Blueprints/GameModeBase/BP_GS_Base.GetAutoSpawn` _asbp_gs_base_2)
        (`self.ClientHACKForAutoSpawn`)))))

(event `ClientTriggerRespawn`
  ;[1 1 1] Dead & Kill
  ;;[1 1 1] TRIGGER RESPAWN
  (`self.ServerTriggerRespawn`)
  (`self.ClientCloseRespawnScreen`)
  (set `self.Can Respawn` false)
  (bind _returnvalue (`|CreateWidget` (`self.MainPlayerHUD`) (`GameplayStatics.GetPlayerController` 0)))
  (bind _output_get (set `self.MainPlayerHUDRef` _returnvalue))
  (`UserWidget.AddToViewport` _output_get 0)
  (`self.ClientCreateAdditionalWidgets`)
  (`self.TriggerClientCreateAdditionalWidgets`))

(event `ClientAddKillFragListEvent`
  (params (KillerBasePS :type "/Game/KoH/Blueprints/GameModeBase/BP_PS_Base Object Reference") (VictimBasePS :type "/Game/KoH/Blueprints/GameModeBase/BP_PS_Base Object Reference"))
  ;[1 1 1] Misc
  ;;[1 1 1] FRAG LIST EVENT
  (bind _aswbp_main_player_hud (cast `/Game/KoH/Blueprints/UIBase/WBP_MainPlayerHUD` (`self.MainPlayerHUDRef`)))
  (`/Game/KoH/Blueprints/UIBase/WBP_MainPlayerHUD.AddKillFragListEvent` _aswbp_main_player_hud KillerBasePS VictimBasePS))

(event `ClientHACKForAutoSpawn`
  ;[1 1 1] Dead & Kill
  ;;[1 1 1] TRIGGER RESPAWN
  (`self.TriggerClientCreateAdditionalWidgets`))

(event `ServerUpdateKillCount`
  (params (`Added Value` :type Integer :default 1))
  ;[1 1 1] Dead & Kill
  ;;[1 1 1] UpdateKillCount
  (bind _updated_player_status (`self.UpdateKillCount` `Added Value`))
  (`self.MulticastUpdateKillCount` _updated_player_status))

(event `MulticastUpdateKillCount`
  (params (PlayerStatus :type "/Game/KoH/Blueprints/GameModeBase/Data/STR_BasePlayerStat Structure"))
  ;[1 1 1] Dead & Kill
  ;;[1 1 1] UpdateKillCount
  (set `self.BasePlayerStat` PlayerStatus))

(event `ServerReturnToLobby`
  ;[1 1 1] Misc
  ;;[1 1 1] RETURN TO LOBBY
  (`self.ClientReturnToLobby`))

(event `ClientReturnToLobby`
  ;[1 1 1] Misc
  ;;[1 1 1] RETURN TO LOBBY
  (bind _returnvalue (`|CreateWidget` (`self.ReturnLoadintScreen`) (`GameplayStatics.GetPlayerController` 0)))
  (`UserWidget.AddToViewport` _returnvalue 0))

(event `ServerUpdateDeathCount`
  (params (`Added Value` :type Integer :default 1))
  ;[1 1 1] Dead & Kill
  ;;[1 1 1] UpdateDeathCount
  (bind _updated_player_status (`self.UpdateDeathCount` `Added Value`))
  (`self.MulticastUpdateDeathCount` _updated_player_status))

(event `MulticastUpdateDeathCount`
  (params (PlayerStatus :type "/Game/KoH/Blueprints/GameModeBase/Data/STR_BasePlayerStat Structure"))
  ;[1 1 1] Dead & Kill
  ;;[1 1 1] UpdateDeathCount
  (set `self.BasePlayerStat` PlayerStatus))

(event `ServerUpdateScores`
  (params (`Added Value` :type Integer))
  ;[1 1 1] Dead & Kill
  ;;[1 1 1] UpdateScores
  (bind _updated_player_status (`self.UpdateScores` `Added Value`))
  (`self.MulticastUpdateScores` _updated_player_status))

(event `MulticastUpdateScores`
  (params (BasePlayerStat :type "/Game/KoH/Blueprints/GameModeBase/Data/STR_BasePlayerStat Structure"))
  ;[1 1 1] Dead & Kill
  ;;[1 1 1] UpdateScores
  (set `self.BasePlayerStat` BasePlayerStat))

(fn `DrawDebugLog`
  (params (DebugLog :type String))
  (bind _drawdebuglogs_ (`self.DrawDebugLogs?`))
  (`KismetSystemLibrary.PrintString` (`KismetStringLibrary.Concat_StrStr` "PLAYER STATE: " DebugLog) _drawdebuglogs_ _drawdebuglogs_ (struct :`R` 1.0 :`B` 0.113781 :`A` 1.0) 4.0))

(fn `GetCanRespawn`
  (returns (`Can Respawn` :type Boolean))
  (return (`self.Can Respawn`)))

(fn `GetDeathCount`
  (returns (`Death Count` :type Integer))
  (return (`.DeathCount_17_0A3567444E14CF89FE60D2911EE46723` (break `/Game/KoH/Blueprints/GameModeBase/Data/STR_BasePlayerStat` (`self.BasePlayerStat`)))))

(fn `GetIsDead`
  (returns (IsDead :type Boolean))
  (return (`self.IsDead`)))

(fn `GetKillCount`
  (returns (`Kill Count` :type Integer))
  (return (`.KillCount_15_A41E95194DD802157B780AAEC507FA17` (break `/Game/KoH/Blueprints/GameModeBase/Data/STR_BasePlayerStat` (`self.BasePlayerStat`)))))

(fn `GetPlayerNameDesv`
  (returns (PlayerName :type String))
  (return (`.PlayerName_5_359B60F64217DC73F81AD288A34B835D` (break `/Game/KoH/Blueprints/GameModeBase/Data/STR_BasePlayerDesc` (`self.BasePlayerDesc`)))))

(fn `GetRatio`
  (returns (Ratio :type "Float (double-precision)"))
  (locals (loc_ratio :type "Float (double-precision)" :default 0.0))
  (bind (_killcount _deathcount) (break `/Game/KoH/Blueprints/GameModeBase/Data/STR_BasePlayerStat` (`self.BasePlayerStat`)))
  (if (== 0 (`.DeathCount_17_0A3567444E14CF89FE60D2911EE46723` (break `/Game/KoH/Blueprints/GameModeBase/Data/STR_BasePlayerStat` (`self.BasePlayerStat`))))
    (set `local.loc_ratio` (/ (`KismetMathLibrary.Conv_IntToDouble` (`.KillCount_15_A41E95194DD802157B780AAEC507FA17` (break `/Game/KoH/Blueprints/GameModeBase/Data/STR_BasePlayerStat` (`self.BasePlayerStat`)))) 1.0))
    (else
      (set `local.loc_ratio` (/ (`KismetMathLibrary.Conv_IntToDouble` _killcount) (`KismetMathLibrary.Conv_IntToDouble` _deathcount)))))
  (return (`local.loc_ratio`)))

(fn `GetRespawnTimerValue`
  (returns (RespawnTimerValue :type Integer))
  (return (`self.RespawnTimerValue`)))

(fn `GetScores`
  (returns (Scores :type Integer))
  (return (`.Scores_20_D9704656415BB30849F982B837C9EB9A` (break `/Game/KoH/Blueprints/GameModeBase/Data/STR_BasePlayerStat` (`self.BasePlayerStat`)))))

(fn `GetTeam`
  (returns (Team :type "/Game/KoH/Blueprints/GameModeBase/Data/E_ModeTeamType Enum"))
  (return (`.TeamType_13_A41E95194DD802157B780AAEC507FA17` (break `/Game/KoH/Blueprints/GameModeBase/Data/STR_BasePlayerDesc` (`self.BasePlayerDesc`)))))

(fn `InitializeFromGameIns`
  (locals (loc_team_type :type "/Game/KoH/Blueprints/GameModeBase/Data/E_ModeTeamType Enum" :default "NewEnumerator0"))
  (`/Engine/EditorBlueprintResources/StandardMacros.IsValid` (`GameplayStatics.GetGameInstance`)
    (:`Is Valid`
      (bind _asbp_gi_menu_base (cast `/Game/KoH/Blueprints/MenuBase/GameMode/BP_GI_MenuBase` (`GameplayStatics.GetGameInstance`)))
      (bind (_playername _ishost_ _isclient_ _teamtype) (break `/Game/KoH/Blueprints/MenuBase/Data/STR_MenuPlayerDesc` (`/Game/KoH/Blueprints/MenuBase/GameMode/BP_GI_MenuBase.GetMenuPlayerDesc` _asbp_gi_menu_base)))
      (switch `/Game/KoH/Blueprints/MenuBase/Data/E_TeamType` _teamtype
        (:`NewEnumerator2`
          (set `local.loc_team_type` "NewEnumerator0"))
        (:`NewEnumerator0`
          (set `local.loc_team_type` "NewEnumerator1"))
        (:`NewEnumerator1`
          (set `local.loc_team_type` "NewEnumerator2")))
      (`self.ServerInitializePlayerProperties` (make `/Game/KoH/Blueprints/GameModeBase/Data/STR_BasePlayerDesc` _playername _ishost_ _isclient_ (`local.loc_team_type`))))))

(fn `SetTeam`
  (params (Team :type "/Game/KoH/Blueprints/GameModeBase/Data/E_ModeTeamType Enum" :default "NewEnumerator0"))
  (bind (_playername _ishost_ _isclient_) (break `/Game/KoH/Blueprints/GameModeBase/Data/STR_BasePlayerDesc` (`self.BasePlayerDesc`)))
  (set `self.BasePlayerDesc` (make `/Game/KoH/Blueprints/GameModeBase/Data/STR_BasePlayerDesc` _playername _ishost_ _isclient_ Team)))

(fn `UpdateDeathCount`
  (params (`Added Value` :type Integer))
  (returns (`Updated Player Status` :type "/Game/KoH/Blueprints/GameModeBase/Data/STR_BasePlayerStat Structure"))
  (bind (_killcount _deathcount _scores) (break `/Game/KoH/Blueprints/GameModeBase/Data/STR_BasePlayerStat` (`self.BasePlayerStat`)))
  (bind _output_get (set `self.BasePlayerStat` (make `/Game/KoH/Blueprints/GameModeBase/Data/STR_BasePlayerStat` _killcount (+ `Added Value` _deathcount) _scores)))
  (return _output_get))

(fn `UpdateKillCount`
  (params (`Added Value` :type Integer))
  (returns (`Updated Player Status` :type "/Game/KoH/Blueprints/GameModeBase/Data/STR_BasePlayerStat Structure"))
  (bind (_killcount _deathcount _scores) (break `/Game/KoH/Blueprints/GameModeBase/Data/STR_BasePlayerStat` (`self.BasePlayerStat`)))
  (bind _output_get (set `self.BasePlayerStat` (make `/Game/KoH/Blueprints/GameModeBase/Data/STR_BasePlayerStat` (+ `Added Value` _killcount) _deathcount _scores)))
  (return _output_get))

(fn `UpdateScores`
  (params (`Added Value` :type Integer))
  (returns (`Updated Player Status` :type "/Game/KoH/Blueprints/GameModeBase/Data/STR_BasePlayerStat Structure"))
  (bind (_killcount _deathcount _scores) (break `/Game/KoH/Blueprints/GameModeBase/Data/STR_BasePlayerStat` (`self.BasePlayerStat`)))
  (bind _output_get (set `self.BasePlayerStat` (make `/Game/KoH/Blueprints/GameModeBase/Data/STR_BasePlayerStat` _killcount _deathcount (+ `Added Value` _scores))))
  (return _output_get))

(fn `UserConstructionScript`)