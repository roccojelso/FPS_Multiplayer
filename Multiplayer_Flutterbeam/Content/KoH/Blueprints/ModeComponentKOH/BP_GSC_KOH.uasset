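; BP_GSC_KOH is a King of the Hill component, apparently for the GameState, that holds the current point's state and lifetime.
; Server update events set each value locally, then pass it to a matching multicast event that sets it again, judging by names to sync clients.
; Two getter functions expose the stored values to other code.
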(event `ServerUpdateCurrentPointState`
  (params (CurrentPointState :type "/Game/KoH/Blueprints/CapturePointBase/Data/E_PointState Enum" :default "NewEnumerator0"))
  ;[1 1 1] Current Point State
  (bind _output_get (set `self.CurrentPointState` CurrentPointState))
  (`self.MulticastUpdateCurrentPointState` _output_get))

(event `MulticastUpdateCurrentPointState`
  (params (CurrentPointState :type "/Game/KoH/Blueprints/CapturePointBase/Data/E_PointState Enum" :default "NewEnumerator0"))
  ;[1 1 1] Current Point State
  (set `self.CurrentPointState` CurrentPointState))

(event `ServerUpdateCurrentPointLifeTime`
  (params (CurrentPointLifeTime :type Integer))
  ;[1 1 1] Current Point Life Time
  (bind _output_get (set `self.CurrentPointLifeTime` CurrentPointLifeTime))
  (`self.MulticastUpdateCurrentPointLifeTime` _output_get))

(event `MulticastUpdateCurrentPointLifeTime`
  (params (CurrentPointLifeTime :type Integer))
  ;[1 1 1] Current Point Life Time
  (set `self.CurrentPointLifeTime` CurrentPointLifeTime))

(fn `GetCurrentPointLifeTime`
  (returns (CurrentPointLifeTime :type Integer))
  (return (`self.CurrentPointLifeTime`)))

(fn `GetCurrentPointState`
  (returns (CurrentPointState :type "/Game/KoH/Blueprints/CapturePointBase/Data/E_PointState Enum"))
  (return (`self.CurrentPointState`)))