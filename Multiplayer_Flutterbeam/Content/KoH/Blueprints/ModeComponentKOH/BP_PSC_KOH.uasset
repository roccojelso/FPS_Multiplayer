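; Player state component for King of the Hill that manages each player's HUD, scoreboard and capture point indicators.
; After a startup delay on server or standalone, it checks the game mode, caches the owner's team and calls client initialization to gather capture points.
; BP_PS_Base triggers drive HUD and scoreboard creation and removal.
; Server events forward to Client counterparts that update team-relative point indication and toggle HUD point icons.
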(event `HandleTriggerClientOpenScoreboard`
  ;[1 1 1] EVENT BEGIN PLAY
  (`self.ClientOpenDOMScoreboard`))

(event `HandleTriggerClientCloseScoreboard`
  ;[1 1 1] EVENT BEGIN PLAY
  (`self.ClientCloseDOMScoreboard`))

(event `self.ReceiveBeginPlay`
  ;[1 1 1] EVENT BEGIN PLAY
  (`|ExecutionSequence`
    (:`then_0`
      (if (`KismetSystemLibrary.IsStandalone`)
        (`KismetSystemLibrary.Delay` 7.0 :!label _label)
        (`KismetSystemLibrary.Delay` 1.0)
        (bind _asbp_gs_base (cast `/Game/KoH/Blueprints/GameModeBase/BP_GS_Base` (`GameplayStatics.GetGameState`)))
        (if (`|EnumEquality` (`/Game/KoH/Blueprints/GameModeBase/BP_GS_Base.GetGameModeType` _asbp_gs_base) "NewEnumerator4")
          (`|ExecutionSequence`
            (:`then_0`
              (bind _asbp_ps_base (cast `/Game/KoH/Blueprints/GameModeBase/BP_PS_Base` (`self.GetOwner`)))
              (set `self.OwnerTeam` (`/Game/KoH/Blueprints/GameModeBase/BP_PS_Base.GetTeam` _asbp_ps_base))
              (`self.ClientInitializePSComponent`))))
        (elif (`KismetSystemLibrary.IsServer`)
          (goto _label))))
    (:`then_1`
      (bind _asbp_ps_base_2 (cast `/Game/KoH/Blueprints/GameModeBase/BP_PS_Base` (`self.GetOwner`)))
      (add `/Game/KoH/Blueprints/GameModeBase/BP_PS_Base.TriggerClientOpenScoreboard` _asbp_ps_base_2 (delegate `HandleTriggerClientOpenScoreboard`))
      (add `/Game/KoH/Blueprints/GameModeBase/BP_PS_Base.TriggerClientCloseScoreboard` _asbp_ps_base_2 (delegate `HandleTriggerClientCloseScoreboard`)))))

(event `ClientInitializePSComponent`
  ;[1 1 1] CLIENT INITIALIZE PS COMPONENT
  (`self.DrawDebugLog` "ClientInitializePSComponent")
  (bind _outactors (`GameplayStatics.GetAllActorsOfClass` "/Game/KoH/Blueprints/CapturePointBase/BP_CP_BaseCapturePoint.BP_CP_BaseCapturePoint_C"))
  (for _array_element _outactors
    (if (`|EnumEquality` (`/Game/KoH/Blueprints/CapturePointBase/BP_CP_BaseCapturePoint.CapturePointType` _array_element) "NewEnumerator1")
      (`KismetArrayLibrary.Array_Add` (`self.AllDominationPoint`) _array_element)))
  (bind _asbp_ps_base (cast `/Game/KoH/Blueprints/GameModeBase/BP_PS_Base` (`self.GetOwner`)))
  (add `/Game/KoH/Blueprints/GameModeBase/BP_PS_Base.TriggerClientCreateAdditionalWidgets` _asbp_ps_base (delegate `ServerHandleCreateAdditionalWidgets`))
  (bind _asbp_ps_base_2 (cast `/Game/KoH/Blueprints/GameModeBase/BP_PS_Base` (`self.GetOwner`)))
  (add `/Game/KoH/Blueprints/GameModeBase/BP_PS_Base.TriggerClientRemoveAdditionalWidgets` _asbp_ps_base_2 (delegate `HandleTriggerClientRemoveAdditionalWidgets`)))

(event `ServerHandleCreateAdditionalWidgets`
  ;[1 1 1] CLIENT INITIALIZE PS COMPONENT
  (`KismetSystemLibrary.Delay` 0.5)
  (`self.ClientHandleCreateAdditionalWidgets` (`self.AllDominationPoint`)))

(event `HandleTriggerClientRemoveAdditionalWidgets`
  ;[1 1 1] CLIENT INITIALIZE PS COMPONENT
  (`Widget.RemoveFromParent` (`self.KingOfTheHillHUD`)))

(event `ClientHandleCreateAdditionalWidgets`
  (params (CapturePoints :type "Array of /Game/KoH/Blueprints/CapturePointBase/BP_CP_BaseCapturePoint Object Reference (by ref)"))
  ;[1 1 1] CLIENT HANDLE CREATE ADDITIONAL WIDGETS
  (bind _returnvalue (`|CreateWidget` "/Game/KoH/Blueprints/UIKOH/WBP_KingOfTheHillHUD.WBP_KingOfTheHillHUD_C" (`GameplayStatics.GetPlayerController` 0)))
  (bind _output_get (set `self.KingOfTheHillHUD` _returnvalue))
  (`UserWidget.AddToViewport` _output_get 0)
  (bind _asplayer_state (cast `PlayerState` (`self.GetOwner`)))
  (bind _asplayer_controller (cast `PlayerController` (`Actor.GetOwner` _asplayer_state)))
  (bind _asbp_ps_base (cast `/Game/KoH/Blueprints/GameModeBase/BP_PS_Base` _asplayer_state))
  (`/Game/KoH/Blueprints/UIKOH/WBP_KingOfTheHillHUD.InitializeKOHHUD` (`self.KingOfTheHillHUD`) CapturePoints (`Controller.K2_GetPawn` _asplayer_controller) _asbp_ps_base)
  (`self.DrawDebugLog` "Create Additional Widgets"))

(event `ServerHandlePointCaptured`
  (params (Point :type "/Game/KoH/Blueprints/CapturePointBase/BP_CP_BaseCapturePoint Object Reference") (`New State` :type "/Game/KoH/Blueprints/CapturePointBase/Data/E_PointState Enum" :default "NewEnumerator0"))
  ;[1 1 1] HANDLE POINT CAPTURED
  (`self.ClientHandlePointCaptured` Point `New State`))

(event `ClientHandlePointCaptured`
  (params (Point :type "/Game/KoH/Blueprints/CapturePointBase/BP_CP_BaseCapturePoint Object Reference") (`New State` :type "/Game/KoH/Blueprints/CapturePointBase/Data/E_PointState Enum" :default "NewEnumerator0"))
  ;[1 1 1] HANDLE POINT CAPTURED
  (switch `/Game/KoH/Blueprints/GameModeBase/Data/E_ModeTeamType` (`self.OwnerTeam`)
    (:`NewEnumerator1`
      (`/Game/KoH/Blueprints/CapturePointBase/BP_CP_BaseCapturePoint.ClientUpdateFormIndication` Point `New State` "NewEnumerator0"))
    (:`NewEnumerator2`
      (`/Game/KoH/Blueprints/CapturePointBase/BP_CP_BaseCapturePoint.ClientUpdateFormIndication` Point `New State` "NewEnumerator1"))))

(event `ClientOpenDOMScoreboard`
  ;[1 1 1] Scoreboard
  (bind _returnvalue (`|CreateWidget` (`self.KOHScoreboardClass`) (`GameplayStatics.GetPlayerController` 0)))
  (bind _output_get (set `self.KOHScoreboardClassRef` _returnvalue))
  (`UserWidget.AddToViewport` _output_get 5)
  (bind _aswbp_score_board_koh (cast `/Game/KoH/Blueprints/UIKOH/WBP_ScoreBoardKOH` (`self.KOHScoreboardClassRef`)))
  (bind _asbp_ps_base (cast `/Game/KoH/Blueprints/GameModeBase/BP_PS_Base` (`self.GetOwner`)))
  (`/Game/KoH/Blueprints/UIKOH/WBP_ScoreBoardKOH.InitializeScoreBoard` _aswbp_score_board_koh _asbp_ps_base))

(event `ClientCloseDOMScoreboard`
  ;[1 1 1] Scoreboard
  (`/Engine/EditorBlueprintResources/StandardMacros.IsValid` (`self.KOHScoreboardClassRef`)
    (:`Is Valid`
      (`Widget.RemoveFromParent` (`self.KOHScoreboardClassRef`)))))

(event `ServerKOHPointTurnON`
  (params (PointName :type "/Game/KoH/Blueprints/CapturePointBase/Data/E_CapturePointName Enum" :default "NewEnumerator0"))
  ;[1 1 1] KOHPointTurnON
  (`self.ClientKOHPointTurnON` PointName))

(event `ClientKOHPointTurnON`
  (params (PointName :type "/Game/KoH/Blueprints/CapturePointBase/Data/E_CapturePointName Enum" :default "NewEnumerator0"))
  ;[1 1 1] KOHPointTurnON
  (`/Engine/EditorBlueprintResources/StandardMacros.IsValid` (`self.KingOfTheHillHUD`)
    (:`Is Valid`
      (`/Game/KoH/Blueprints/UIKOH/WBP_KingOfTheHillHUD.TurnONPointIcon` (`self.KingOfTheHillHUD`) PointName))))

(event `ServerKOHPointTurnOFF`
  (params (PointName :type "/Game/KoH/Blueprints/CapturePointBase/Data/E_CapturePointName Enum" :default "NewEnumerator0"))
  ;[1 1 1] KOHPointTurnOFF
  (`self.ClientKOHPointTurnOFF` PointName))

(event `ClientKOHPointTurnOFF`
  (params (PointName :type "/Game/KoH/Blueprints/CapturePointBase/Data/E_CapturePointName Enum" :default "NewEnumerator0"))
  ;[1 1 1] KOHPointTurnOFF
  (`/Engine/EditorBlueprintResources/StandardMacros.IsValid` (`self.KingOfTheHillHUD`)
    (:`Is Valid`
      (`/Game/KoH/Blueprints/UIKOH/WBP_KingOfTheHillHUD.TurnOFFPointIcon` (`self.KingOfTheHillHUD`) PointName))))

(fn `DrawDebugLog`
  (params (DebugLog :type String))
  (if (`self.DrawDebugLogs?`)
    (`KismetSystemLibrary.PrintString` (`KismetStringLibrary.Concat_StrStr` "DOM PS COMP: " DebugLog))))