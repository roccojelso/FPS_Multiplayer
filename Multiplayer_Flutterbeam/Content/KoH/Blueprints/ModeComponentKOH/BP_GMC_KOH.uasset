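; Game mode component that runs King of the Hill on the server, setting match rules from the scoring type.
; It gathers the level's hill points and binds to their capture events and game mode round events.
; Looping timers score held points and rotate the active hill through shuffled unused points, returning to the first when all are used.
; Point state, lifetime and on/off changes are pushed to KOH GameState and PlayerState components.
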(event `InitializeCKOHDesc`
  ;[1 1 1] INITIALIZE CKOH DESC
  (set `self.KOHMatchDesc` (struct))
  (`self.DrawDebugLog` "Laucnh from Main Menu / Initialize Base Setting")
  (`self.InitializeBaseSettings`))

(event `self.ReceiveBeginPlay`
  ;[1 1 1] EVENT BEGIN PLAY
  (`self.DrawDebugLog` "KING OF THE HILL IS HERE")
  (if (`KismetSystemLibrary.IsStandalone`)
    (`KismetSystemLibrary.Delay` 7.2 :!label _label)
    (bind _asbp_gs_base (cast `/Game/KoH/Blueprints/GameModeBase/BP_GS_Base` (`GameplayStatics.GetGameState`)))
    (if (`|EnumEquality` (`/Game/KoH/Blueprints/GameModeBase/BP_GS_Base.GetGameModeType` _asbp_gs_base) "NewEnumerator4")
      (bind _asbp_gm_base (cast `/Game/KoH/Blueprints/GameModeBase/BP_GM_Base` (`self.GetOwner`)))
      (if (`/Game/KoH/Blueprints/GameModeBase/BP_GM_Base.Use Direct Launch?` _asbp_gm_base)
        (`self.DrawDebugLog` "Use direct Launch / Initialize Base Setting")
        (`self.InitializeBaseSettings`))
      (`KismetSystemLibrary.Delay` 1.0)
      (`self.DrawDebugLog` "Using GameType == CKOH. Initialize CKOH")
      (`self.InitializeCKOH`))
    (elif (`KismetSystemLibrary.IsServer`)
      (goto _label))))

(event `InitializeCKOH`
  ;[1 1 1] INITIALIZE CKOH
  (bind _asbp_gs_base (cast `/Game/KoH/Blueprints/GameModeBase/BP_GS_Base` (`GameplayStatics.GetGameState`)))
  (set `self.GameStateRef` _asbp_gs_base)
  (`self.InitializeCapturePoints`)
  (`self.InitializeKingOfTheHill`))

(event `StartPointRotationTimer`
  ;[1 1 1] KOH
  (bind _returnvalue (`KismetSystemLibrary.K2_SetTimerDelegate` (delegate `HandleKOHPointSpawn`) (`KismetMathLibrary.Conv_IntToDouble` (`self.PointLifeTime`)) true))
  (set `self.PointRotationTimer` _returnvalue))

(event `HandleKOHPointSpawn`
  ;[1 1 1] KOH
  (`self.KOHPointRemove`)
  (`KismetSystemLibrary.Delay` 0.2)
  (`KismetArrayLibrary.Array_Shuffle` (`self.KOHPoints`))
  (set `self.IsNewPointFounded?` false)
  (`KismetSystemLibrary.K2_ClearAndInvalidateTimerHandle` (`self.PointLifeTimeTimer`))
  (`self.StartPointLifeTimeTimer`)
  (for _array_element (`self.KOHPoints`)
    (bind _capturepointname (`/Game/KoH/Blueprints/CapturePointBase/BP_CP_BaseCapturePoint.CapturePointName` _array_element))
    (if (not (`KismetArrayLibrary.Array_Contains` (`self.KOHUsedPointArray`) _capturepointname))
      (`/Engine/EditorBlueprintResources/StandardMacros.DoOnce` false :!label _label_2
        (:`Completed`
          (`self.KOHPointSpawn` _array_element _capturepointname)
          (set `self.IsNewPointFounded?` true)))))
  (if (`self.IsNewPointFounded?`)
    (goto _label_2 :!via `Reset`)
    (else
      (`KismetArrayLibrary.Array_Clear` (`self.KOHUsedPointArray`))
      (`self.SpawnFirstPoint`)
      (goto _label_2 :!via `Reset`))))

(event `StartPointLifeTimeTimer`
  ;[1 1 1] KOH
  (set `self.PointLifeTimeValue` (`self.PointLifeTime`))
  (bind _returnvalue (`KismetSystemLibrary.K2_SetTimerDelegate` (delegate `HandlePointLifeTimeTimer`) 1.0 true))
  (set `self.PointLifeTimeTimer` _returnvalue))

(event `HandlePointLifeTimeTimer`
  ;[1 1 1] KOH
  (`/Engine/EditorBlueprintResources/StandardMacros.DecrementInt` (`self.PointLifeTimeValue`)
    (:`  `
      (bind _asbp_gs_base (cast `/Game/KoH/Blueprints/GameModeBase/BP_GS_Base` (`GameplayStatics.GetGameState`)))
      (`/Game/KoH/Blueprints/ModeComponentKOH/BP_GSC_KOH.ServerUpdateCurrentPointLifeTime` (`Actor.GetComponentByClass` _asbp_gs_base "/Game/KoH/Blueprints/ModeComponentKOH/BP_GSC_KOH.BP_GSC_KOH_C") (`self.PointLifeTimeValue`)))))

(event `InitializeCapturePoints`
  ;[1 1 1] INITIALIZE CAPTURE POINTS
  (bind _outactors (`GameplayStatics.GetAllActorsOfClass` "/Game/KoH/Blueprints/CapturePointBase/BP_CP_BaseCapturePoint.BP_CP_BaseCapturePoint_C"))
  (bind _output_get (set `self.AllPoint` _outactors))
  (for _array_element _output_get
    (if (`|EnumEquality` (`/Game/KoH/Blueprints/CapturePointBase/BP_CP_BaseCapturePoint.CapturePointType` _array_element) "NewEnumerator1")
      (`KismetArrayLibrary.Array_Add` (`self.KOHPoints`) _array_element)))
  (bind _asbp_gm_base (cast `/Game/KoH/Blueprints/GameModeBase/BP_GM_Base` (`self.GetOwner`)))
  (add `/Game/KoH/Blueprints/GameModeBase/BP_GM_Base.TriggerEndRound` _asbp_gm_base (delegate `HandleTriggerEndRound`))
  (for _array_element_2 (`self.AllPoint`)
    (add `/Game/KoH/Blueprints/CapturePointBase/BP_CP_BaseCapturePoint.PointCaptured` _array_element_2 (delegate `HandlePointCaptured`))))

(event `HandlePointCaptured`
  (params (Point :type "/Game/KoH/Blueprints/CapturePointBase/BP_CP_BaseCapturePoint Object Reference") (NewPointState :type "/Game/KoH/Blueprints/CapturePointBase/Data/E_PointState Enum" :default "NewEnumerator0"))
  ;[1 1 1] INITIALIZE CAPTURE POINTS
  (`self.PointCaptured` Point NewPointState))

(event `HandleTriggerEndRound`
  ;[1 1 1] INITIALIZE CAPTURE POINTS
  (`KismetSystemLibrary.K2_PauseTimerHandle` (`self.PointRotationTimer`))
  (`KismetSystemLibrary.K2_PauseTimerHandle` (`self.PointLifeTimeTimer`))
  (for _array_element (`self.KOHPoints`)
    (`/Game/KoH/Blueprints/CapturePointBase/BP_CP_BaseCapturePoint.ServerPointReset` _array_element)
    (`/Game/KoH/Blueprints/CapturePointBase/BP_CP_BaseCapturePoint.ServerTurnOffKOHPoint` _array_element))
  (set `self.Team1PointsCount` 0)
  (set `self.Team2PointsCount` 0))

(event `StartPointRotation`
  ;[1 1 1] KOH
  (`KismetSystemLibrary.K2_ClearAndInvalidateTimerHandle` (`self.PointRotationTimer`))
  (`KismetSystemLibrary.K2_ClearAndInvalidateTimerHandle` (`self.PointLifeTimeTimer`))
  (`self.StartPointLifeTimeTimer`)
  (`self.StartPointRotationTimer`))

(event `HandleRoundMatchStarted`
  ;[1 1 1] INITIALIZE KING OF THE HILL
  (bind _returnvalue (`KismetSystemLibrary.K2_SetTimer` self "UpdateTeamScores" (`self.UpdateScoreTime`) true))
  (set `self.UpdateTeamsScoresTimer` _returnvalue)
  (`self.StartPointRotation`))

(event `HandleTriggerInitialSpawn`
  ;[1 1 1] INITIALIZE KING OF THE HILL
  (`self.SpawnFirstPoint`))

(event `InitializeKingOfTheHill`
  ;[1 1 1] INITIALIZE KING OF THE HILL
  (bind _asbp_gm_base (cast `/Game/KoH/Blueprints/GameModeBase/BP_GM_Base` (`self.GetOwner`)))
  (add `/Game/KoH/Blueprints/GameModeBase/BP_GM_Base.TriggerRoundMatchStarted` _asbp_gm_base (delegate `HandleRoundMatchStarted`))
  (add `/Game/KoH/Blueprints/GameModeBase/BP_GM_Base.TriggerInitialSpawn` _asbp_gm_base (delegate `HandleTriggerInitialSpawn`)))

(event `KOHPointSpawn`
  (params (KOHPoint :type "/Game/KoH/Blueprints/CapturePointBase/BP_CP_BaseCapturePoint Object Reference") (PointName :type "/Game/KoH/Blueprints/CapturePointBase/Data/E_CapturePointName Enum (by ref)"))
  ;[1 1 1] KOH
  (bind _output_get (set `self.CurrentKOHPoint` KOHPoint))
  (`KismetArrayLibrary.Array_Add` (`self.KOHUsedPointArray`) PointName)
  (`/Game/KoH/Blueprints/CapturePointBase/BP_CP_BaseCapturePoint.ServerPointReset` _output_get)
  (`/Game/KoH/Blueprints/CapturePointBase/BP_CP_BaseCapturePoint.ServerInitializeCapturePoint` KOHPoint (`self.BaseTimeToCapture`) (`self.ResetDominationStatusSpeed`) (`self.TeamMemberEcnounter`))
  (`/Game/KoH/Blueprints/CapturePointBase/BP_CP_BaseCapturePoint.ServerInitializeKOHPoint` KOHPoint)
  (bind _asbp_gs_base (cast `/Game/KoH/Blueprints/GameModeBase/BP_GS_Base` (`GameplayStatics.GetGameState`)))
  (`/Game/KoH/Blueprints/ModeComponentKOH/BP_GSC_KOH.ServerUpdateCurrentPointState` (`Actor.GetComponentByClass` _asbp_gs_base "/Game/KoH/Blueprints/ModeComponentKOH/BP_GSC_KOH.BP_GSC_KOH_C") "NewEnumerator0")
  (for _array_element (`GameStateBase.PlayerArray` (`self.GameStateRef`))
    (bind _asbp_ps_base (cast `/Game/KoH/Blueprints/GameModeBase/BP_PS_Base` _array_element))
    (`/Game/KoH/Blueprints/ModeComponentKOH/BP_PSC_KOH.ServerKOHPointTurnON` (`Actor.GetComponentByClass` _asbp_ps_base "/Game/KoH/Blueprints/ModeComponentKOH/BP_PSC_KOH.BP_PSC_KOH_C") (`/Game/KoH/Blueprints/CapturePointBase/BP_CP_BaseCapturePoint.CapturePointName` KOHPoint))))

(event `KOHPointRemove`
  (bind _currentkohpoint (`self.CurrentKOHPoint`))
  ;[1 1 1] KOH
  (`/Game/KoH/Blueprints/CapturePointBase/BP_CP_BaseCapturePoint.ServerTurnOffKOHPoint` _currentkohpoint)
  (`/Game/KoH/Blueprints/CapturePointBase/BP_CP_BaseCapturePoint.ServerPointReset` _currentkohpoint)
  (set `self.Team1PointsCount` 0)
  (set `self.Team2PointsCount` 0)
  (for _array_element (`GameStateBase.PlayerArray` (`self.GameStateRef`))
    (bind _asbp_ps_base (cast `/Game/KoH/Blueprints/GameModeBase/BP_PS_Base` _array_element))
    (`/Game/KoH/Blueprints/ModeComponentKOH/BP_PSC_KOH.ServerKOHPointTurnOFF` (`Actor.GetComponentByClass` _asbp_ps_base "/Game/KoH/Blueprints/ModeComponentKOH/BP_PSC_KOH.BP_PSC_KOH_C") (`/Game/KoH/Blueprints/CapturePointBase/BP_CP_BaseCapturePoint.CapturePointName` _currentkohpoint))))

(event `PointCaptured`
  (params (Point :type "/Game/KoH/Blueprints/CapturePointBase/BP_CP_BaseCapturePoint Object Reference") (`New Point State` :type "/Game/KoH/Blueprints/CapturePointBase/Data/E_PointState Enum" :default "NewEnumerator0"))
  ;[1 1 1] POINT CAPTURED
  (`self.DrawDebugLog` (`KismetStringLibrary.Concat_StrStr` "POINT CAPTURED BY: " (`|GetEnumeratorNameAsString` `New Point State`)))
  (`self.UpdateTeamsPointsCount`)
  (`|ExecutionSequence`
    (:`then_0`
      (bind _asbp_gs_base (cast `/Game/KoH/Blueprints/GameModeBase/BP_GS_Base` (`GameplayStatics.GetGameState`)))
      (`/Game/KoH/Blueprints/ModeComponentKOH/BP_GSC_KOH.ServerUpdateCurrentPointState` (`Actor.GetComponentByClass` _asbp_gs_base "/Game/KoH/Blueprints/ModeComponentKOH/BP_GSC_KOH.BP_GSC_KOH_C") `New Point State`))
    (:`then_1`
      (for _array_element (`GameStateBase.PlayerArray` (`self.GameStateRef`))
        (bind _asbp_ps_base (cast `/Game/KoH/Blueprints/GameModeBase/BP_PS_Base` _array_element))
        (`/Game/KoH/Blueprints/ModeComponentKOH/BP_PSC_KOH.ServerHandlePointCaptured` (`Actor.GetComponentByClass` _asbp_ps_base "/Game/KoH/Blueprints/ModeComponentKOH/BP_PSC_KOH.BP_PSC_KOH_C") Point `New Point State`)))))

(event `SpawnFirstPoint`
  (bind _firstcapturepoint (`self.FirstCapturePoint`))
  ;[1 1 1] KOH
  (`KismetSystemLibrary.Delay` 1.0)
  (`KismetArrayLibrary.Array_Clear` (`self.KOHUsedPointArray`))
  (for _array_element (`self.KOHPoints`)
    (if (`|EnumEquality` _firstcapturepoint (`/Game/KoH/Blueprints/CapturePointBase/BP_CP_BaseCapturePoint.CapturePointName` _array_element))
      (`self.KOHPointSpawn` _array_element _firstcapturepoint))))

(fn `DrawDebugLog`
  (params (DebugLog :type String))
  (if (`self.DrawDebugLogs?`)
    (`KismetSystemLibrary.PrintString` (`KismetStringLibrary.Concat_StrStr` "CKOH_GMC: " DebugLog))))

(fn `GetBaseTimeToCapture`
  (returns (BaseTimeToCapture :type "Float (double-precision)"))
  (return (`self.BaseTimeToCapture`)))

(fn `GetResetDominationStatusSpeed`
  (returns (ResetDominationStatusSpeed :type "Float (double-precision)"))
  (return (`self.ResetDominationStatusSpeed`)))

(fn `GetScorePerTime`
  (returns (`Score per Time` :type Integer))
  (return (`self.ScoreperTime`)))

(fn `GetTeamMemberEcnounter`
  (returns (TeamMemberEcnounter :type "Float (double-precision)"))
  (return (`self.TeamMemberEcnounter`)))

(fn `GetUpdateScoreTime`
  (returns (`Update Score Time` :type "Float (double-precision)"))
  (return (`self.UpdateScoreTime`)))

(fn `InitializeBaseSettings`
  (bind (_matchtimelimit _matchscorelimit _baserespawntime _autospawn_) (break `/Game/KoH/Blueprints/GameModeBase/Data/STR_BaseSingleRoundMatchDesc` (`self.BaseSingleRoundMatchDesc`)))
  (bind (_matchtimelimit_2 _matchscorelimit_2 _baserespawntime_2 _autospawn__2) (break `/Game/KoH/Blueprints/GameModeBase/Data/STR_BaseSingleRoundMatchDesc` (`self.BaseSingleRoundMatchDesc`)))
  (bind (_matchtimelimit_3 _matchscorelimit_3 _roundscount _baserespawntime_3 _autospawn__3) (break `/Game/KoH/Blueprints/GameModeBase/Data/STR_BaseCommonRoundedMatchDesc` (`self.BaseCommonRoundedMatchDesc`)))
  (bind (_matchtimelimit_4 _matchscorelimit_4 _roundscount_2 _baserespawntime_4 _autospawn__4) (break `/Game/KoH/Blueprints/GameModeBase/Data/STR_BaseCommonRoundedMatchDesc` (`self.BaseCommonRoundedMatchDesc`)))
  (bind (_roundtimelimit _roundscorelimit _roundwinlimit _baserespawntime_5 _autospawn__5) (break `/Game/KoH/Blueprints/GameModeBase/Data/STR_BaseRoundedMatchDesc` (`self.BaseRoundedMatchDesc`)))
  (bind (_roundtimelimit_2 _roundscorelimit_2 _roundwinlimit_2 _baserespawntime_6 _autospawn__6) (break `/Game/KoH/Blueprints/GameModeBase/Data/STR_BaseRoundedMatchDesc` (`self.BaseRoundedMatchDesc`)))
  (switch `/Game/KoH/Blueprints/GameModeBase/Data/E_ScoringType` (`self.ScoringType`)
    (:`NewEnumerator0`
      ;[1 1 1] Defaul Single Round
      (bind _asbp_gm_base (cast `/Game/KoH/Blueprints/GameModeBase/BP_GM_Base` (`self.GetOwner`)))
      (`/Game/KoH/Blueprints/GameModeBase/BP_GM_Base.InitializeBaseMatchDesc` _asbp_gm_base (make `/Game/KoH/Blueprints/GameModeBase/Data/STR_BaseMatchDesc` _matchtimelimit_2 _matchscorelimit_2 false false false 1 _autospawn__2 false _baserespawntime_2)))
    (:`NewEnumerator1`
      ;[1 1 1] Reverse Single Round
      (bind _asbp_gm_base_2 (cast `/Game/KoH/Blueprints/GameModeBase/BP_GM_Base` (`self.GetOwner`)))
      (`/Game/KoH/Blueprints/GameModeBase/BP_GM_Base.InitializeBaseMatchDesc` _asbp_gm_base_2 (make `/Game/KoH/Blueprints/GameModeBase/Data/STR_BaseMatchDesc` _matchtimelimit _matchscorelimit true false false 1 _autospawn_ false _baserespawntime)))
    (:`NewEnumerator2`
      ;[1 1 1] Defaul Common Rounded
      (bind _asbp_gm_base_3 (cast `/Game/KoH/Blueprints/GameModeBase/BP_GM_Base` (`self.GetOwner`)))
      (`/Game/KoH/Blueprints/GameModeBase/BP_GM_Base.InitializeBaseMatchDesc` _asbp_gm_base_3 (make `/Game/KoH/Blueprints/GameModeBase/Data/STR_BaseMatchDesc` _matchtimelimit_3 _matchscorelimit_3 false true false _roundscount _autospawn__3 false _baserespawntime_3)))
    (:`NewEnumerator3`
      ;[1 1 1] Reverse Common Rounded
      (bind _asbp_gm_base_4 (cast `/Game/KoH/Blueprints/GameModeBase/BP_GM_Base` (`self.GetOwner`)))
      (`/Game/KoH/Blueprints/GameModeBase/BP_GM_Base.InitializeBaseMatchDesc` _asbp_gm_base_4 (make `/Game/KoH/Blueprints/GameModeBase/Data/STR_BaseMatchDesc` _matchtimelimit_4 _matchscorelimit_4 true true false _roundscount_2 _autospawn__4 false _baserespawntime_4)))
    (:`NewEnumerator4`
      ;[1 1 1] Defaul Rounded
      (bind _asbp_gm_base_5 (cast `/Game/KoH/Blueprints/GameModeBase/BP_GM_Base` (`self.GetOwner`)))
      (`/Game/KoH/Blueprints/GameModeBase/BP_GM_Base.InitializeBaseMatchDesc` _asbp_gm_base_5 (make `/Game/KoH/Blueprints/GameModeBase/Data/STR_BaseMatchDesc` _roundtimelimit_2 _roundscorelimit_2 false true true _roundwinlimit_2 _autospawn__6 false _baserespawntime_6)))
    (:`NewEnumerator5`
      ;[1 1 1] Reverse Rounded
      (bind _asbp_gm_base_6 (cast `/Game/KoH/Blueprints/GameModeBase/BP_GM_Base` (`self.GetOwner`)))
      (`/Game/KoH/Blueprints/GameModeBase/BP_GM_Base.InitializeBaseMatchDesc` _asbp_gm_base_6 (make `/Game/KoH/Blueprints/GameModeBase/Data/STR_BaseMatchDesc` _roundtimelimit _roundscorelimit true true true _roundwinlimit _autospawn__5 false _baserespawntime_5)))))

(fn `PointRotation`
  (locals (loc_koh_point_step :type "/Game/KoH/Blueprints/CapturePointBase/BP_CP_BaseCapturePoint Object Reference"))
  (`KismetSystemLibrary.PrintString` "PointRotation"))

(fn `UpdateTeamScores`
  (`|ExecutionSequence`
    (:`then_0`
      ;[1 1 1] Comment
      (if (not (== (`self.Team1PointsCount`) 0))
        ;[1 1 1] Comment
        (bind _asbp_gm_base (cast `/Game/KoH/Blueprints/GameModeBase/BP_GM_Base` (`self.GetOwner`)))
        (`/Game/KoH/Blueprints/GameModeBase/BP_GM_Base.UpdateTeamMatchScore` _asbp_gm_base "NewEnumerator1" (* (`self.Team1PointsCount`) (`self.GetScorePerTime`)))))
    (:`then_1`
      ;[1 1 1] Comment
      (if (not (== (`self.Team2PointsCount`) 0))
        ;[1 1 1] Comment
        (bind _asbp_gm_base_2 (cast `/Game/KoH/Blueprints/GameModeBase/BP_GM_Base` (`self.GetOwner`)))
        (`/Game/KoH/Blueprints/GameModeBase/BP_GM_Base.UpdateTeamMatchScore` _asbp_gm_base_2 "NewEnumerator2" (* (`self.Team2PointsCount`) (`self.GetScorePerTime`)))))))

(fn `UpdateTeamsPointsCount`
  (set `self.Team1PointsCount` 0)
  (set `self.Team2PointsCount` 0)
  (for _array_element (`self.AllPoint`)
    (bind _pointstate (`/Game/KoH/Blueprints/CapturePointBase/BP_CP_BaseCapturePoint.PointState` _array_element))
    (if (`|EnumEquality` _pointstate "NewEnumerator1")
      (`/Engine/EditorBlueprintResources/StandardMacros.IncrementInt` (`self.Team1PointsCount`))
      (elif (`|EnumEquality` _pointstate "NewEnumerator2")
        (`/Engine/EditorBlueprintResources/StandardMacros.IncrementInt` (`self.Team2PointsCount`)))))
  ;[1 1 1] Comment
  (`self.DrawDebugLog` (`KismetStringLibrary.Concat_StrStr` "Update Points Countes // " "Team1: " (`KismetStringLibrary.Conv_IntToString` (`self.Team1PointsCount`)) " // " "Team2: " (`KismetStringLibrary.Conv_IntToString` (`self.Team2PointsCount`))))
  (return))