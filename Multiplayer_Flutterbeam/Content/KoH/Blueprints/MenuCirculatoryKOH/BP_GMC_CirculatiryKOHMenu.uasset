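; Game mode component for the Circulatiry King of the Hill menu that hands match settings over to the game instance before launch.
; On BeginPlay it binds to the owning BP_GM_MenuBase's pre-launch, mode-update and rules-menu-open triggers.
; Pre-launch copies the match description from the game state's menu component into BP_GI_MenuCirculatiryKOH.
; Closing the rules menu calls back into the game mode; update and open handlers are effectively empty, with leftover unwired DOM initialization calls.
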(event `HandleTriggerPreLaunchMatch`
  ;[1 1 1] EVENT BEGIN PLAY
  (`self.ComponentTriggerPreLaunchMatch`))

(event `HandleTriggerUpdateGameMode`
  ;[1 1 1] EVENT BEGIN PLAY
  (`self.ComponentTriggerUpdateGameMode`))

(event `HandleTriggerHostOpenModeRulesMenu`
  ;[1 1 1] EVENT BEGIN PLAY
  (`self.ComponentTriggerHostOpenModeRulesMenu`))

(event `self.ReceiveBeginPlay`
  ;[1 1 1] EVENT BEGIN PLAY
  (bind _asbp_gm_menu_base (cast `/Game/KoH/Blueprints/MenuBase/GameMode/BP_GM_MenuBase` (`self.GetOwner`)))
  (add `/Game/KoH/Blueprints/MenuBase/GameMode/BP_GM_MenuBase.TriggerPreLaunchMatch` _asbp_gm_menu_base (delegate `HandleTriggerPreLaunchMatch`))
  (add `/Game/KoH/Blueprints/MenuBase/GameMode/BP_GM_MenuBase.TriggerUpdateGameMode` _asbp_gm_menu_base (delegate `HandleTriggerUpdateGameMode`))
  (add `/Game/KoH/Blueprints/MenuBase/GameMode/BP_GM_MenuBase.TriggerHostOpenModeRulesMenu` _asbp_gm_menu_base (delegate `HandleTriggerHostOpenModeRulesMenu`)))

(event `ComponentTriggerPreLaunchMatch`
  ;[1 1 1] COMPONENT TRIGGER PRE LAUNCH MATCH
  (bind _asbp_gs_menu_base (cast `/Game/KoH/Blueprints/MenuBase/GameMode/BP_GS_MenuBase` (`GameplayStatics.GetGameState`)))
  (bind _asbp_gi_menu_circulatiry_koh (cast `/Game/KoH/Blueprints/MenuCirculatoryKOH/GameMode/BP_GI_MenuCirculatiryKOH` (`GameplayStatics.GetGameInstance`)))
  (set `/Game/KoH/Blueprints/MenuCirculatoryKOH/GameMode/BP_GI_MenuCirculatiryKOH.CirculatiryKOHMatchDesc` (`/Game/KoH/Blueprints/MenuCirculatoryKOH/BP_GSC_CirculatiryKOHMenu.GetCirculatiryKOHMatchDesc` (`Actor.GetComponentByClass` _asbp_gs_menu_base "/Game/KoH/Blueprints/MenuCirculatoryKOH/BP_GSC_CirculatiryKOHMenu.BP_GSC_CirculatiryKOHMenu_C")) _asbp_gi_menu_circulatiry_koh))

(event `ComponentTriggerUpdateGameMode`
  ;[1 1 1] COMPONENT TRIGGER UPDATE GAME MODE
)

(event `ComponentTriggerHostOpenModeRulesMenu`
  ;[1 1 1] COMPONENT TRIGGER HOST OPEN MODE RULES MENU
)

(event `ComponentTriggerHostCloseModeRulesMenu`
  ;[1 1 1] COMPONENT TRIGGER HOST CLOSE MODE RULES MENU
  (bind _asbp_gm_menu_base (cast `/Game/KoH/Blueprints/MenuBase/GameMode/BP_GM_MenuBase` (`self.GetOwner`)))
  (`/Game/KoH/Blueprints/MenuBase/GameMode/BP_GM_MenuBase.HandleHostCloseModeRulesMenu` _asbp_gm_menu_base))

(event `ComponentTriggerUpdateGameModeRules`
  ;[1 1 1] COMPONENT TRIGGER UPDATE GAME MODE RULES
)