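; Assault class character Blueprint that specializes a parent class, throwing a small ammo box as its item through the server MedKit spawn call.
; It plays the current weapon's first-person equip montage, showing the weapon after a short timer to avoid a one-frame misplacement and clearing the performing-action flag on completion.
; Unequipping plays its montage at double speed and hides the weapon on blend out.
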(event `/Game/FPS/Blueprints/Interfaces/iPawnActions.ThrowItem`
  (`self.Server_SpawnMedKit` "/Game/FPS/Blueprints/AmmoBox/BP_SmallAmmoBox.BP_SmallAmmoBox_C"))

(fn `UserConstructionScript`
  (`parent.UserConstructionScript`))