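; BP_LobbyPC is the lobby player controller that shows the lobby menu and relays each player's map vote and ready state.
; Client events open WB_NewLobby with cursor and UI-only input, or clear all widgets.
; Server events allow one vote via a CanVote flag, passed to BP_Lobby_GM for tallying.
; Ready changes go to the PlayerState, and readying up asks BP_Lobby_GS to start the countdown.
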(event `Client_OpenLobbyMenu`
  ;[1 1 1] Open Lobby Menu
  (set `self.bShowMouseCursor` true)
  (bind _returnvalue (`|CreateWidget` "/Game/FB_UI/UI/WB_NewLobby.WB_NewLobby_C" self))
  (`UserWidget.AddToViewport` _returnvalue 0)
  (`WidgetBlueprintLibrary.SetInputMode_UIOnlyEx` self null))

(event `Server_VoteMap`
  (params (Map :type Integer))
  ;[1 1 1] Vote Map
  (if (`self.bCanVote`)
    (set `self.bCanVote` false)
    (bind _asbp_lobby_gm (cast `/Game/FPS/Blueprints/GameModes/Lobby/BP_Lobby_GM` (`GameplayStatics.GetGameMode`)))
    (`/Game/FPS/Blueprints/GameModes/Lobby/BP_Lobby_GM.Server_IncreaseMapVotes` _asbp_lobby_gm Map)))

(event `Client_RemoveWidget`
  ;[1 1 1] Remove Widget
  (`WidgetLayoutLibrary.RemoveAllWidgets`))

(event `Server_SetPlayerReady`
  (params (bReady :type Boolean))
  ;[1 1 1] Server SetPlayerReady
  (message `/Game/FPS/Blueprints/Interfaces/iPlayerState.SetIsPlayerReady` (`self.PlayerState`) bReady)
  (if bReady
    (bind _asbp_lobby_gs (cast `/Game/FPS/Blueprints/GameModes/Lobby/BP_Lobby_GS` (`GameplayStatics.GetGameState`)))
    (`/Game/FPS/Blueprints/GameModes/Lobby/BP_Lobby_GS.Server_StartCountDown` _asbp_lobby_gs)))

(fn `UserConstructionScript`)